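; Boss paddle in a reversed brick-breaker that launches enemy bouncing balls among player bricks and slides along Y.
; A Tick-driven Status machine switches between random repositioning, spawning balls and chasing the lowest-X eligible ball, using DoOnce/DoN gates.
; Running out of balls during a chase costs health, triggering death or a faster phase with more balls and a new brick layout.
; Balls overlapping its Box die, and timer functions build each brick layout.
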(event `self.ReceiveBeginPlay`
  (bind _asui_life_bar (cast `/Game/UI_LifeBar` (`WidgetComponent.GetWidget` (`self.Widget`))))
  (set `/Game/UI_LifeBar.BounceBoard` self _asui_life_bar)
  (`KismetSystemLibrary.Delay` 1.0)
  (set `self.Status` 2)
  (bind _returnvalue (`KismetSystemLibrary.K2_SetTimer` null "BrickSpawn" 0.001 true))
  (set `self.SpawnHandle` _returnvalue))

(event `Choose Random Location`
  (bind _movingrange (`self.MovingRange`))
  (bind _returnvalue (`KismetMathLibrary.MakeVector` -500.0 (`KismetMathLibrary.RandomFloatInRange` (* _movingrange -1.0) _movingrange)))
  (`/Engine/EditorBlueprintResources/StandardMacros.DoOnce` false :!label _label
    (:`Completed`
      (`KismetSystemLibrary.Delay` 0.01 :!label _label_2)
      (if (>= (`KismetMathLibrary.Vector_Distance` (`self.NewLocation`) _returnvalue) 300.0)
        (set `self.NewLocation` _returnvalue)
        (`KismetSystemLibrary.Delay` 1.0)
        (goto _label :!via `Reset`)
        (else
          (goto _label_2))))))

(event `self.ReceiveTick`
  (params (DeltaSeconds :type "Float (single-precision)"))
  (bind _returnvalue (`self.K2_GetActorLocation`))
  (bind _newlocation (`self.NewLocation`))
  (bind (_returnvalue_x _returnvalue_y) (`KismetMathLibrary.BreakVector` (* (`KismetMathLibrary.GetDirectionUnitVector` _returnvalue _newlocation) (`KismetMathLibrary.Lerp` 1.0 (`self.MoveSpeed`) (/ (`KismetMathLibrary.Vector_Distance` _returnvalue _newlocation) 50.0)))))
  (`self.K2_AddActorWorldOffset` (`KismetMathLibrary.MakeVector` 0.0 _returnvalue_y))
  (switch `int` (`self.Status`)
    (:`0`
      (`self.Choose Random Location`))
    (:`1`
      (`self.ChaseClosestBall`))
    (:`2`
      (`self.SpawnNewBall`))))

(event `ChaseClosestBall`
  (bind _returnvalue_location (`KismetMathLibrary.BreakTransform` (`self.GetTransform`)))
  (bind _phase (`self.Phase`))
  (bind (_returnvalue_x _returnvalue_y) (`KismetMathLibrary.BreakVector` (`self.K2_GetActorLocation` (`self.BallTracing`))))
  (`|ExecutionSequence`
    (:`then_0`
      (`/Engine/EditorBlueprintResources/StandardMacros.DoOnce` false :!label _label_3
        (:`Completed`
          (bind _counter (`/Engine/EditorBlueprintResources/StandardMacros.Do N` (`self.Intervals`) :!label _label_4)
            (:`Exit`
              (`self.BallTrace`)
              (`KismetSystemLibrary.Delay` 0.1)
              (if (>= _counter (`self.Intervals`))
                (`|ExecutionSequence`
                  (:`then_0`
                    (bind _outactors (`GameplayStatics.GetAllActorsOfClass` "/Game/BP/Nova/BP_Enemy_BouncingBall.BP_Enemy_BouncingBall_C"))
                    (if (> (`KismetArrayLibrary.Array_Length` _outactors) 0)
                      (set `self.Status` 2)))
                  (:`then_1`
                    (`self.ResetChaseBall`))
                  (:`then_2`
                    (`self.ResetChaseBallAll`)))
                (else
                  (`self.ResetChaseBall`))))))))
    (:`then_1`
      (`self.BallTracing`
        (:`then`
          (set `self.NewLocation` (`KismetMathLibrary.MakeVector` -500.0 (`KismetMathLibrary.FClamp` _returnvalue_y -1050.0 1050.0))))
        (:`else`
          (bind _outactors_2 (`GameplayStatics.GetAllActorsOfClass` "/Game/BP/Nova/BP_Enemy_BouncingBall.BP_Enemy_BouncingBall_C"))
          (if (not (> (`KismetArrayLibrary.Array_Length` _outactors_2) 0))
            (`/Engine/EditorBlueprintResources/StandardMacros.DoOnce` false :!label _label_5
              (:`Completed`
                (`|SpawnActorFromClass` "/Game/BP/Nova/BP_Shockwave.BP_Shockwave_C" (`KismetMathLibrary.MakeTransform` _returnvalue_location) "AlwaysSpawn" "MultiplyWithRoot" null null)
                (bind _output_get (set `self.Health` (- (`self.Health`) 0.34)))
                (if (<= _output_get 0.0)
                  (`self.Death`)
                  (else
                    (`KismetSystemLibrary.Delay` 2.0)
                    (set `self.Status` 0)
                    (`|ExecutionSequence`
                      (:`then_0`
                        (`self.ResetChaseBallAll`))
                      (:`then_1`
                        (`/Engine/EditorBlueprintResources/StandardMacros.IncrementInt` (`self.Phase`)
                          (:`  `
                            (`/Engine/EditorBlueprintResources/StandardMacros.IncrementInt` (`self.SpawnCounter`)))))
                      (:`then_2`
                        (`self.ResetChaseBall`))
                      (:`then_4`
                        (set `self.Intervals` (- (`self.Intervals`) 5))
                        (set `self.MoveSpeed` (+ (`self.MoveSpeed`) 3.0))
                        (bind _returnvalue (`KismetSystemLibrary.K2_SetTimer` null (select `int` (`self.Phase`) :`0` "BrickSpawn" :`1` "BrickSpawn2" :`2` "BrickSpawn3") 0.001 true))
                        (set `self.SpawnHandle` _returnvalue)
                        (`KismetSystemLibrary.Delay` 0.2)
                        (`self.BurstSpawn` (select `int` _phase :`0` 0 :`1` 15 :`2` 30))
                        (`KismetSystemLibrary.Delay` (select `int` _phase :`0` 1.0 :`1` 3.0 :`2` 4.0))
                        (set `self.Status` 2)
                        (`self.ResetHurt`)))))))))))))

(event `ResetChaseBall`
  (goto _label_3 :!via `Reset`))

(event `self.Box.OnComponentBeginOverlap`
  (params (OverlappedComponent :type "PrimitiveComponent Object Reference") (OtherActor :type "Actor Object Reference") (OtherComp :type "PrimitiveComponent Object Reference") (OtherBodyIndex :type Integer) (bFromSweep :type Boolean) (SweepResult :type "HitResult Structure (by ref)"))
  (bind _asbp_enemy_bouncing_ball (cast `/Game/BP/Nova/BP_Enemy_BouncingBall` OtherActor))
  (`/Game/BP/Nova/BP_EnemyMaster.Death` _asbp_enemy_bouncing_ball))

(event `ResetChaseBallAll`
  (goto _label_4 :!via `Reset`))

(event `ResetHurt`
  (goto _label_5 :!via `Reset`))

(event `BurstSpawn`
  (params (n :type Integer))
  (bind _returnvalue (`SceneComponent.K2_GetComponentToWorld` (`self.Arrow`)))
  (`NiagaraFunctionLibrary.SpawnSystemAttached` "/Game/VFX/BlinkAndDashVFX/VFX_Niagara/NS_Blink_FireSmall.NS_Blink_FireSmall" (`self.Arrow`) "None" (0.0 0.0 0.0) (struct) "KeepRelativeOffset")
  (bind _counter (`/Engine/EditorBlueprintResources/StandardMacros.Do N` n :!label _label_6)
    (:`Exit`
      (bind _returnvalue_2 (`|SpawnActorFromClass` "/Game/BP/Nova/BP_Enemy_BouncingBall.BP_Enemy_BouncingBall_C" (`KismetMathLibrary.MakeTransform` (`KismetMathLibrary.MakeVector` (.x (.location _returnvalue)) (+ (.y (.location _returnvalue)) (`KismetMathLibrary.RandomFloatInRange` -50.0 50.0)) (.z (.location _returnvalue))) (`KismetMathLibrary.MakeRotator` (.roll (.rotation _returnvalue)) (.pitch (.rotation _returnvalue)) (+ (.yaw (.rotation _returnvalue)) (`KismetMathLibrary.RandomFloatInRange` -35.0 35.0))) (0.2 0.2 0.2)) "Undefined" "MultiplyWithRoot" null null))
      (set `/Game/BP/Nova/BP_Enemy_BouncingBall.BounceTimes` 3 _returnvalue_2)
      (if (> _counter n)
        (goto _label_6 :!via `Reset`)
        (else
          (`KismetSystemLibrary.Delay` 0.05)
          (goto _label_6))))))

(event `SpawnNewBall`
  (bind _arrow (`self.Arrow`))
  (bind _spawncounter (`self.SpawnCounter`))
  (bind (_returnvalue_roll _returnvalue_pitch _returnvalue_yaw) (`KismetMathLibrary.BreakRotator` (`SceneComponent.K2_GetComponentRotation` _arrow)))
  (`/Engine/EditorBlueprintResources/StandardMacros.DoOnce` false :!label _label_7
    (:`Completed`
      (`NiagaraFunctionLibrary.SpawnSystemAttached` "/Game/VFX/BlinkAndDashVFX/VFX_Niagara/NS_Blink_FireSmall.NS_Blink_FireSmall" (`self.Arrow`) "None" (0.0 0.0 0.0) (struct) "KeepRelativeOffset")
      (bind _outactors (`GameplayStatics.GetAllActorsOfClass` "/Game/BP/Nova/BP_Enemy_BouncingBall.BP_Enemy_BouncingBall_C"))
      (if (not (> (`KismetArrayLibrary.Array_Length` _outactors) (select `int` (`self.Phase`) :`0` 5 :`1` 8 :`2` 12)))
        (bind _counter (`/Engine/EditorBlueprintResources/StandardMacros.Do N` _spawncounter :!label _label_8)
          (:`Exit`
            (`|SpawnActorFromClass` "/Game/BP/Nova/BP_Enemy_BouncingBall.BP_Enemy_BouncingBall_C" (`KismetMathLibrary.MakeTransform` (`SceneComponent.K2_GetComponentLocation` _arrow) (`KismetMathLibrary.MakeRotator` _returnvalue_roll _returnvalue_pitch (+ _returnvalue_yaw (`KismetMathLibrary.RandomFloatInRange` -35.0 35.0))) (0.5 0.5 0.5)) "Undefined" "MultiplyWithRoot" null null)
            (if (>= _counter _spawncounter)
              (`KismetSystemLibrary.Delay` 0.2)
              (else
                (`KismetSystemLibrary.Delay` 0.1)
                (goto _label_8))))))
      (set `self.Status` 1)
      (`self.ResetSpawn`))))

(event `ResetSpawn`
  (`|ExecutionSequence`
    (:`then_0`
      (goto _label_7 :!via `Reset`))
    (:`then_1`
      (goto _label_8 :!via `Reset`))))

(event `Death`
  (`/Engine/EditorBlueprintResources/StandardMacros.DoOnce` false
    (:`Completed`
      (`self.SetActorEnableCollision` false)
      (`NiagaraFunctionLibrary.SpawnSystemAtLocation` "/Game/VFX/BlinkAndDashVFX/VFX_Niagara/NS_Blink_Fire.NS_Blink_Fire" (`self.K2_GetActorLocation`))
      (bind (_direction `_新建轨道_0`) (`Timeline|时间轴` :!via `PlayFromStart`)
        (:`Update`
          (`self.SetActorScale3D` (`KismetMathLibrary.VLerp` (1.0 1.0 1.0) (3.0 3.0 3.0) `_新建轨道_0`))
          (`MeshComponent.SetScalarParameterValueOnMaterials` (`self.Cube`) "Opacity" `_新建轨道_0`)
          (`self.K2_DestroyActor`))))))

(fn `BallTrace`
  (bind _outactors (`GameplayStatics.GetAllActorsOfClass` "/Game/BP/Nova/BP_Enemy_BouncingBall.BP_Enemy_BouncingBall_C"))
  (if (> (`KismetArrayLibrary.Array_Length` _outactors) 0)
    (set `self.MinimumDistance` 10000.0)
    (set `self.BallTracing` null)
    (for _array_element _outactors
      (bind _x (.x (`self.K2_GetActorLocation` _array_element)))
      (if (and (> (`/Game/BP/Nova/BP_Enemy_BouncingBall.BounceTimes` _array_element) 5) (< _x (`self.MinimumDistance`)))
        (set `self.MinimumDistance` _x)
        (set `self.BallTracing` _array_element)))
    (`/Engine/EditorBlueprintResources/StandardMacros.IsValid` (`self.BallTracing`)
      (:`Is Valid`
        (set `self.Status` 1)))))

(fn `BrickSpawn`
  (locals (Location :type "Vector Structure" :default (0.0 120.0 0.0)) (Tooclose :type Boolean))
  (bind _outactors (`GameplayStatics.GetAllActorsOfClass` "/Game/BP/Nova/BP_Bricks_Player.BP_Bricks_Player_C"))
  (bind _returnvalue (`KismetArrayLibrary.Array_Length` _outactors))
  (bind (_remainder _returnvalue_2) (`KismetMathLibrary.FMod` (`KismetMathLibrary.Conv_IntToDouble` _returnvalue) 30.0))
  (set `local.Location` (`KismetMathLibrary.MakeVector` (`KismetMathLibrary.Conv_IntToDouble` (* _returnvalue_2 60)) (+ (* _remainder 60.0) -900.0)))
  (if (>= _returnvalue 240)
    (`KismetSystemLibrary.K2_ClearAndInvalidateTimerHandle` (`self.SpawnHandle`))
    (else
      (`|SpawnActorFromClass` "/Game/BP/Nova/BP_Bricks_Player.BP_Bricks_Player_C" (`KismetMathLibrary.MakeTransform` (`local.Location`)) "Undefined" "MultiplyWithRoot" null null))))

(fn `BrickSpawn2`
  (locals (Location :type "Vector Structure" :default (0.0 120.0 0.0)) (Tooclose :type Boolean))
  (bind _outactors (`GameplayStatics.GetAllActorsOfClass` "/Game/BP/Nova/BP_Bricks_Player.BP_Bricks_Player_C"))
  (bind _returnvalue (`KismetArrayLibrary.Array_Length` _outactors))
  (bind (_remainder _returnvalue_2) (`KismetMathLibrary.FMod` (`KismetMathLibrary.Conv_IntToDouble` _returnvalue) 10.0))
  (bind _returnvalue_3 (>= _returnvalue 100))
  (set `local.Location` (`KismetMathLibrary.MakeVector` (- (`KismetMathLibrary.Conv_IntToDouble` (* _returnvalue_2 60)) (`KismetMathLibrary.SelectFloat` 700.0 100.0 _returnvalue_3)) (+ (* _remainder 60.0) (`KismetMathLibrary.SelectFloat` 360.0 -900.0 _returnvalue_3))))
  (if (>= _returnvalue 200)
    (`KismetSystemLibrary.K2_ClearAndInvalidateTimerHandle` (`self.SpawnHandle`))
    (else
      (`|SpawnActorFromClass` "/Game/BP/Nova/BP_Bricks_Player.BP_Bricks_Player_C" (`KismetMathLibrary.MakeTransform` (`local.Location`)) "Undefined" "MultiplyWithRoot" null null))))

(fn `BrickSpawn3`
  (locals (Location :type "Vector Structure" :default (0.0 120.0 0.0)) (Tooclose :type Boolean))
  (bind _outactors (`GameplayStatics.GetAllActorsOfClass` "/Game/BP/Nova/BP_Bricks_Player.BP_Bricks_Player_C"))
  (bind _returnvalue (`KismetArrayLibrary.Array_Length` _outactors))
  (bind (_remainder _returnvalue_2) (`KismetMathLibrary.FMod` (`KismetMathLibrary.Conv_IntToDouble` _returnvalue) 10.0))
  (set `local.Location` (`KismetMathLibrary.MakeVector` (- (`KismetMathLibrary.Conv_IntToDouble` (* _returnvalue_2 60)) 200.0) (+ (* _remainder 60.0) (* (`KismetMathLibrary.RandomIntegerInRange` -17 12) 60))))
  (if (>= _returnvalue 120)
    (`KismetSystemLibrary.K2_ClearAndInvalidateTimerHandle` (`self.SpawnHandle`))
    (else
      (`|SpawnActorFromClass` "/Game/BP/Nova/BP_Bricks_Player.BP_Bricks_Player_C" (`KismetMathLibrary.MakeTransform` (`local.Location`)) "Undefined" "MultiplyWithRoot" null null))))

(fn `UserConstructionScript`)