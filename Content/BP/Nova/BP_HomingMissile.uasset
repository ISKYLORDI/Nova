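; BP_HomingMissile is a missile that homes in on the player character and deals damage on contact.
; While attached, it copies its parent's rotation each tick, and a BeginPlay timeline slides the cone from an offset into place.
; Initialize detaches and launches it forward, enabling homing on the player after a short delay.
; It bursts with a Niagara effect on timeout, or once launched, on overlapping BP_PLayer1 or a BP_Projectile.
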(event `self.ReceiveBeginPlay`
  (bind _initial_location (`self.Initial Location`))
  (set `self.Initial Location` (`SceneComponent.RelativeLocation` (`self.Cone`)))
  (bind (_direction `_新建轨道_0`) (`Timeline|时间轴`)
    (:`Update`
      (`SceneComponent.K2_SetRelativeLocation` (`self.Cone`) (`KismetMathLibrary.VLerp` (+ _initial_location (-60.0 0.0 0.0)) _initial_location `_新建轨道_0`) false false))))

(event `self.ReceiveTick`
  (params (DeltaSeconds :type "Float (single-precision)"))
  (bind _returnvalue (`SceneComponent.GetAttachParent` (`self.DefaultSceneRoot`)))
  (`/Engine/EditorBlueprintResources/StandardMacros.IsValid` _returnvalue
    (:`Is Valid`
      (`self.K2_SetActorRotation` (`SceneComponent.K2_GetComponentRotation` _returnvalue)))))

(event `Initialize`
  (bind _projectilemovement (`self.ProjectileMovement`))
  (set `ProjectileMovementComponent.bIsHomingProjectile` true _projectilemovement)
  (set `MovementComponent.Velocity` (* (`SceneComponent.GetForwardVector` (`self.DefaultSceneRoot`)) 200.0) (`self.ProjectileMovement`))
  (`self.K2_DetachFromActor` "KeepWorld" "KeepWorld" "KeepWorld")
  (`KismetSystemLibrary.Delay` 0.2)
  (set `ProjectileMovementComponent.HomingTargetComponent` (`Actor.RootComponent` (`GameplayStatics.GetPlayerCharacter` 0)) _projectilemovement)
  (`KismetSystemLibrary.Delay` 2.4)
  (`NiagaraFunctionLibrary.SpawnSystemAtLocation` "/Game/VFX/BlinkAndDashVFX/VFX_Niagara/NS_Blink_FireSmall.NS_Blink_FireSmall" (`self.K2_GetActorLocation`) (struct) (0.2 0.2 0.2) :!label _label)
  (`self.K2_DestroyActor`))

(event `self.ReceiveActorBeginOverlap`
  (params (OtherActor :type "Actor Object Reference"))
  (if (`ProjectileMovementComponent.bIsHomingProjectile` (`self.ProjectileMovement`))
    (bind _asbp_player_1 (cast `/Game/BP/Nova/BP_PLayer1` OtherActor)
      (:`then`
        (`GameplayStatics.ApplyDamage` _asbp_player_1 0.2 null self)
        (goto _label))
      (:`CastFailed`
        (cast `/Game/BP/Nova/BP_Projectile` OtherActor)
        (goto _label)))))

(fn `UserConstructionScript`)