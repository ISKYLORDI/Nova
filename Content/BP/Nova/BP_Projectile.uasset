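; BP_Projectile is a short-lived projectile that damages enemies, bricks and bounce boards.
; After a brief delay, a timeline shrinks it to zero scale and destroys it, with a lifespan also set on spawn.
; Box overlap casts by target type to apply damage, pushing enemies back by their own KnockBackScale.
; Hits and the ProjectileHit event share one exit that spawns a Niagara impact effect and destroys the projectile.
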(event `self.ReceiveBeginPlay`
  (`self.SetLifeSpan` 1.0)
  (set `self.Scale` (`self.GetActorScale3D`))
  (`KismetSystemLibrary.Delay` 0.25)
  (bind (_direction `_新建轨道_0`) (`Timeline|时间轴` :!via `PlayFromStart`)
    (:`Update`
      (`self.SetActorScale3D` (`KismetMathLibrary.VLerp` (`self.Scale`) (0.0 0.0 0.0) `_新建轨道_0`)))
    (:`Finished`
      (`self.K2_DestroyActor`))))

(event `self.Box.OnComponentBeginOverlap`
  (params (OverlappedComponent :type "PrimitiveComponent Object Reference") (OtherActor :type "Actor Object Reference") (OtherComp :type "PrimitiveComponent Object Reference") (OtherBodyIndex :type Integer) (bFromSweep :type Boolean) (SweepResult :type "HitResult Structure (by ref)"))
  (bind _returnvalue (`SceneComponent.K2_GetComponentLocation` (`self.Sphere`)))
  (`|ExecutionSequence`
    (:`then_0`
      (bind _asbp_enemy_master (cast `/Game/BP/Nova/BP_EnemyMaster` OtherActor))
      (`GameplayStatics.ApplyDamage` OtherActor 0.1 null self)
      (bind _knockbackscale (`/Game/BP/Nova/BP_EnemyMaster.KnockBackScale` _asbp_enemy_master))
      (if (> _knockbackscale 0.0)
        (`/Game/BP/Nova/BP_EnemyMaster.StartPush` _asbp_enemy_master (`KismetMathLibrary.GetDirectionUnitVector` (`self.K2_GetActorLocation`) (`self.K2_GetActorLocation` _asbp_enemy_master)) (* _knockbackscale 1.0))))
    (:`then_1`
      (cast `/Game/BP/Nova/BP_Bricks` OtherActor)
      (`GameplayStatics.ApplyDamage` OtherActor 0.1 null self :!label _label))
    (:`then_2`
      (cast `/Game/BP/Nova/BP_BounceBoard` OtherActor)
      (goto _label)))
  (`NiagaraFunctionLibrary.SpawnSystemAtLocation` "/Game/NS_ProjectileHit.NS_ProjectileHit" _returnvalue (`KismetMathLibrary.FindLookAtRotation` (`self.K2_GetActorLocation` OtherActor) _returnvalue) :!label _label_2)
  (`self.K2_DestroyActor`))

(event `ProjectileHit`
  (goto _label_2))

(fn `UserConstructionScript`)