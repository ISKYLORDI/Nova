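; BP_Bricks is a brick actor that plays a scale-up, fade-out effect when its Destroyed event fires.
; BeginPlay caches the actor's scale, and Destroyed disables collision and starts a timeline.
; The timeline doubles that scale while driving the cube's material parameters to fade opacity and boost intensity, then destroys the actor.
; A Niagara blink spawn is left disconnected and never runs.
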(event `self.ReceiveBeginPlay`
  (set `self.Scale` (`self.GetActorScale3D`)))

(event `Destroyed`
  (bind _cube (`self.Cube`))
  (bind _scale (`self.Scale`))
  (`self.SetActorEnableCollision` false)
  (bind (_direction `_新建轨道_0`) (`Timeline|时间轴`)
    (:`Update`
      (`self.SetActorScale3D` (`KismetMathLibrary.VLerp` _scale (* _scale 2.0) `_新建轨道_0`))
      (`MeshComponent.SetScalarParameterValueOnMaterials` _cube "Opacity" (`KismetMathLibrary.Lerp` 1.0 0.0 `_新建轨道_0`))
      (`MeshComponent.SetScalarParameterValueOnMaterials` _cube "Intensity" (`KismetMathLibrary.Lerp` 1.0 20.0 `_新建轨道_0`)))
    (:`Finished`
      (`self.K2_DestroyActor`))))

(fn `UserConstructionScript`)