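; Free-moving camera actor that becomes the player's view target and enables its own input on BeginPlay.
; Holding right mouse hides the cursor and rotates the spring arm (local pitch, world yaw), re-centering the cursor in the viewport.
; Movement axes shift the spring arm along the camera's forward and right XY components or world Z at half strength, while the wheel moves it along the full view direction.
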(event `InputAxisKey|MouseY`
  (params (AxisValue :type "Float (single-precision)"))
  (bind (_returnvalue_x _returnvalue_y) (`KismetMathLibrary.BreakVector2D` (`WidgetLayoutLibrary.GetViewportSize`)))
  (if (`self.Pressed`)
    (`SceneComponent.K2_AddLocalRotation` (`self.SpringArm`) (`KismetMathLibrary.MakeRotator` 0.0 (* AxisValue 2.0)) false false)
    (`PlayerController.SetMouseLocation` (`GameplayStatics.GetPlayerController` 0) (`KismetMathLibrary.FTrunc` (/ _returnvalue_x 2.0)) (`KismetMathLibrary.FTrunc` (/ _returnvalue_y 2.0)) :!label _label)))

(event `InputAxisKey|MouseX`
  (params (AxisValue :type "Float (single-precision)"))
  (if (`self.Pressed`)
    (`SceneComponent.K2_AddWorldRotation` (`self.SpringArm`) (`KismetMathLibrary.MakeRotator` 0.0 0.0 (* AxisValue 2.0)) false false)
    (goto _label)))

(event `Key|MouseScrollUp`
  (params (Key :type "Key Structure"))
  (:`Pressed`
    (`SceneComponent.K2_AddWorldOffset` (`self.SpringArm`) (* (`SceneComponent.GetForwardVector` (`self.Camera`)) (`self.MovementStrength`)) false false)))

(event `Key|RightMouseButton`
  (params (Key :type "Key Structure"))
  (bind _returnvalue (`GameplayStatics.GetPlayerController` 0))
  (:`Pressed`
    (set `self.Pressed` true)
    (set `PlayerController.bShowMouseCursor` false _returnvalue))
  (:`Released`
    (set `self.Pressed` false)
    (set `PlayerController.bShowMouseCursor` true _returnvalue)))

(event `Key|MouseScrollDown`
  (params (Key :type "Key Structure"))
  (:`Pressed`
    (`SceneComponent.K2_AddWorldOffset` (`self.SpringArm`) (* (`SceneComponent.GetForwardVector` (`self.Camera`)) (`self.MovementStrength`) -1.0) false false)))

(event `InputAxis|MovementForward`
  (params (AxisValue :type "Float (single-precision)"))
  (bind (_returnvalue_x _returnvalue_y) (`KismetMathLibrary.BreakVector` (* (`SceneComponent.GetForwardVector` (`self.Camera`)) (* AxisValue (`self.MovementStrength`)))))
  (`SceneComponent.K2_AddWorldOffset` (`self.SpringArm`) (`KismetMathLibrary.MakeVector` _returnvalue_x _returnvalue_y) false false))

(event `InputAxis|MovementSide`
  (params (AxisValue :type "Float (single-precision)"))
  (bind (_returnvalue_x _returnvalue_y) (`KismetMathLibrary.BreakVector` (* (`SceneComponent.GetRightVector` (`self.Camera`)) (* AxisValue (`self.MovementStrength`)))))
  (`SceneComponent.K2_AddWorldOffset` (`self.SpringArm`) (`KismetMathLibrary.MakeVector` _returnvalue_x _returnvalue_y) false false))

(event `InputAxis|MovementUp`
  (params (AxisValue :type "Float (single-precision)"))
  (`SceneComponent.K2_AddWorldOffset` (`self.SpringArm`) (`KismetMathLibrary.MakeVector` 0.0 0.0 (* AxisValue (* (`self.MovementStrength`) 0.5))) false false))

(event `self.ReceiveBeginPlay`
  (`PlayerController.SetViewTargetWithBlend` (`GameplayStatics.GetPlayerController` 0) self 0.0 "VTBlend_Linear" 0.0 false)
  (`self.EnableInput` (`GameplayStatics.GetPlayerController` 0)))

(fn `UserConstructionScript`)