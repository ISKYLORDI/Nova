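; Body segment of the snake enemy, which trails the head or preceding segment, fires projectiles and can be revived.
; A looping 0.01s timer lerps it to its Target's attach point, turning it with the Target, or toward the player while shooting.
; Shooting ramps up body glow before firing.
; Death runs once until reset, bursting and fading the core and calling PhaseShift on the first snake found; Revive reverses this fade.
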(event `self.Death`
  (`parent.Death`)
  (`/Engine/EditorBlueprintResources/StandardMacros.DoOnce` false :!label _label
    (:`Completed`
      (`NiagaraFunctionLibrary.SpawnSystemAtLocation` "/Game/VFX/BlinkAndDashVFX/VFX_Niagara/NS_Blink_Fire.NS_Blink_Fire" (`self.K2_GetActorLocation`) (struct) (0.5 0.5 0.5))
      (`|ExecutionSequence`
        (:`then_0`
          (bind (_direction `_新建轨道_0`) (`Timeline|时间轴_2` :!via `PlayFromStart` :!label _label_2)
            (:`Update`
              (`SceneComponent.SetRelativeScale3D` (`self.Core`) (`KismetMathLibrary.VLerp` (`KismetMathLibrary.Conv_DoubleToVector` 0.026897) (`KismetMathLibrary.Conv_DoubleToVector` 0.1) `_新建轨道_0`))
              (`MeshComponent.SetScalarParameterValueOnMaterials` (`self.Core`) "Opacity" (`KismetMathLibrary.Lerp` 1.0 0.0 `_新建轨道_0`)))))
        (:`then_1`
          (set `self.Dead` true))
        (:`then_2`
          (bind _outactors (`GameplayStatics.GetAllActorsOfClass` "/Game/BP/Nova/BP_Enemy_Snake.BP_Enemy_Snake_C"))
          (`/Game/BP/Nova/BP_Enemy_Snake.PhaseShift` (`|GetArrayItem` _outactors)))))))

(event `Reset Death`
  (goto _label :!via `Reset`))

(event `Revive`
  (set `self.Dead` false)
  (set `self.HP` 1.6)
  (`self.Reset Death`)
  (goto _label_2 :!via `ReverseFromEnd`))

(event `self.ReceiveBeginPlay`
  (`parent.ReceiveBeginPlay`)
  (bind _returnvalue (`KismetSystemLibrary.K2_SetTimer` null "UpdatingLocation" 0.01 true))
  (set `self.UpdateHandle` _returnvalue)
  (set `self.UpdateLocation` (`SceneComponent.K2_GetComponentLocation` (`self.AttachPoint`)))
  (`self.SetActorEnableCollision` false)
  (bind (_direction `_新建轨道_0`) (`Timeline|时间轴_0` :!via `PlayFromStart`)
    (:`Update`
      (`MeshComponent.SetScalarParameterValueOnMaterials` (`self.Body`) "Opacity" (`KismetMathLibrary.Lerp` 0.0 1.0 `_新建轨道_0`))
      (`MeshComponent.SetScalarParameterValueOnMaterials` (`self.Core`) "Opacity" (`KismetMathLibrary.Lerp` 0.0 1.0 `_新建轨道_0`))
      (`self.SetActorScale3D` (`KismetMathLibrary.VLerp` (0.0 0.0 0.0) (`self.Scale`) `_新建轨道_0`)))
    (:`Finished`
      (`self.SetActorEnableCollision` true))))

(event `self.ReceiveTick`
  (params (DeltaSeconds :type "Float (single-precision)"))
  (`parent.ReceiveTick` DeltaSeconds))

(event `Shooting`
  (bind (_returnvalue_location _returnvalue_rotation) (`KismetMathLibrary.BreakTransform` (`SceneComponent.K2_GetComponentToWorld` (`self.Arrow1`))))
  (if (not (`self.Dead`))
    (set `self.Status` 1)
    (`KismetSystemLibrary.Delay` 0.2)
    (`|ExecutionSequence`
      (:`then_0`
        (bind (_direction `_新建轨道_0`) (`Timeline|时间轴_3` :!via `PlayFromStart`)
          (:`Update`
            (`MeshComponent.SetScalarParameterValueOnMaterials` (`self.Body`) "Intensity" (`KismetMathLibrary.Lerp` 10.0 100.0 `_新建轨道_0`)))))
      (:`then_1`
        (`KismetSystemLibrary.Delay` 0.75)
        (`|SpawnActorFromClass` "/Game/BP/Nova/BP_ProjectileEnemy.BP_ProjectileEnemy_C" (`KismetMathLibrary.MakeTransform` _returnvalue_location _returnvalue_rotation) "AlwaysSpawn" "MultiplyWithRoot" null null)
        (`KismetSystemLibrary.Delay` 1.0)
        (set `self.Status` 0)))))

(fn `UpdatingLocation`
  (bind (_returnvalue_roll _returnvalue_pitch _returnvalue_yaw) (`KismetMathLibrary.BreakRotator` (`self.K2_GetActorRotation`)))
  (bind _returnvalue (`self.K2_GetActorLocation`))
  (bind _target (`self.Target`))
  (bind _returnvalue_2 (`SceneComponent.K2_GetComponentLocation` (`self.AttachPoint`)))
  (bind (_returnvalue_roll_2 _returnvalue_pitch_2 _returnvalue_yaw_2) (`KismetMathLibrary.BreakRotator` (`KismetMathLibrary.NormalizedDeltaRotator` (`self.K2_GetActorRotation` _target) (`self.K2_GetActorRotation`))))
  (bind (_returnvalue_roll_3 _returnvalue_pitch_3 _returnvalue_yaw_3) (`KismetMathLibrary.BreakRotator` (`KismetMathLibrary.FindLookAtRotation` (`self.K2_GetActorLocation`) (`self.K2_GetActorLocation` (`GameplayStatics.GetPlayerCharacter` 0)))))
  (`|ExecutionSequence`
    (:`then_0`
      (if (> (`KismetMathLibrary.Vector_Distance` _returnvalue_2 (`self.UpdateLocation`)) 5.0)
        (set `self.UpdateLocation` _returnvalue_2)))
    (:`then_1`
      (`/Engine/EditorBlueprintResources/StandardMacros.IsValid` _target
        (:`Is Valid`
          (bind _asbp_enemy_snake_body (cast `/Game/BP/Nova/BP_Enemy_SnakeBody` _target)
            (:`then`
              (`self.K2_SetActorLocation` (`KismetMathLibrary.VLerp` _returnvalue (`SceneComponent.K2_GetComponentLocation` (`/Game/BP/Nova/BP_Enemy_SnakeBody.AttachPoint` _asbp_enemy_snake_body)) 0.05)))
            (:`CastFailed`
              (bind _asbp_enemy_snake (cast `/Game/BP/Nova/BP_Enemy_Snake` _target))
              (`self.K2_SetActorLocation` (`KismetMathLibrary.VLerp` _returnvalue (`SceneComponent.K2_GetComponentLocation` (`/Game/BP/Nova/BP_Enemy_Snake.AttachPoint` _asbp_enemy_snake)) 0.05))))
          (switch `int` (`self.Status`)
            (:`0`
              (`self.K2_AddActorWorldRotation` (`KismetMathLibrary.MakeRotator` 0.0 0.0 (`KismetMathLibrary.Lerp` 0.0 (* (`self.RotationSpeed`) (`KismetMathLibrary.SignOfFloat` _returnvalue_yaw_2)) (/ (`KismetMathLibrary.Abs` _returnvalue_yaw_2) 10.0)))))
            (:`1`
              (`self.K2_SetActorRotation` (`KismetMathLibrary.RLerp` (`KismetMathLibrary.MakeRotator` 0.0 0.0 _returnvalue_yaw) (`KismetMathLibrary.MakeRotator` 0.0 0.0 _returnvalue_yaw_3) 0.1 true)))))))))

(fn `UserConstructionScript`
  (`parent.UserConstructionScript`))