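; BP_Shockwave is an expanding shockwave actor that destroys BP_Bricks actors its sphere overlaps.
; On BeginPlay a timeline scales the actor up, flatter in Z, while fading the sphere material's Opacity, then destroys the actor.
; In parallel, after a short delay, it triggers a brief hit-stop through global time dilation if HitEnemy is set, though this graph never sets that flag.
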(event `self.ReceiveBeginPlay`
  (`|ExecutionSequence`
    (:`then_0`
      (bind (_direction `_新建轨道_0`) (`Timeline|时间轴` :!via `PlayFromStart`)
        (:`Update`
          (`self.SetActorScale3D` (`KismetMathLibrary.VLerp` (0.0 0.0 0.0) (10.0 10.0 5.0) `_新建轨道_0`))
          (`MeshComponent.SetScalarParameterValueOnMaterials` (`self.Sphere`) "Opacity" (`KismetMathLibrary.Lerp` 0.3 0.0 `_新建轨道_0`)))
        (:`Finished`
          (`self.K2_DestroyActor`))))
    (:`then_1`
      (`KismetSystemLibrary.Delay` 0.25)
      (if (`self.HitEnemy`)
        (`GameplayStatics.SetGlobalTimeDilation` 0.1)
        (`KismetSystemLibrary.Delay` 0.05)
        (`GameplayStatics.SetGlobalTimeDilation` 1.0)))))

(event `self.Sphere.OnComponentBeginOverlap`
  (params (OverlappedComponent :type "PrimitiveComponent Object Reference") (OtherActor :type "Actor Object Reference") (OtherComp :type "PrimitiveComponent Object Reference") (OtherBodyIndex :type Integer) (bFromSweep :type Boolean) (SweepResult :type "HitResult Structure (by ref)"))
  (bind _asbp_bricks (cast `/Game/BP/Nova/BP_Bricks` OtherActor))
  (`/Game/BP/Nova/BP_Bricks.Destroyed` _asbp_bricks))

(fn `UserConstructionScript`)