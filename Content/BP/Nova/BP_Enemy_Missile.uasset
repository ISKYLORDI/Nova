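; Enemy that enters through a BP_Portal found by random traces around the player and fires volleys of homing missiles.
; A looping timer turns it toward the player and triggers DoOnce-gated volleys, attached at four launch points before delayed launch.
; It roams by repeatedly moving a homing target to trace-validated random points away from the player.
; Death drops a collectible, then scales up and fades it with unlaunched missiles.
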(event `self.ReceiveBeginPlay`
  (set `self.Scale` (`self.GetActorScale3D`)))

(event `self.Death`
  (bind _scale (`self.Scale`))
  (`parent.Death`)
  (`self.SpawnCollectible`)
  (`self.SetActorEnableCollision` false)
  (`NiagaraFunctionLibrary.SpawnSystemAtLocation` "/Game/VFX/BlinkAndDashVFX/VFX_Niagara/NS_Blink_Fire.NS_Blink_Fire" (`self.K2_GetActorLocation`) (struct) (0.5 0.5 0.5))
  (bind (_direction `_新建轨道_0`) (`Timeline|时间轴_0`)
    (:`Update`
      (`self.SetActorScale3D` (`KismetMathLibrary.VLerp` _scale (* _scale 3.0) `_新建轨道_0`))
      (for _array_element (`self.Missiles`)
        (`self.K2_DetachFromActor` _array_element "KeepWorld" "KeepWorld" "KeepWorld")
        (`MeshComponent.SetScalarParameterValueOnMaterials` (`self.Sphere`) "Opacity" (`KismetMathLibrary.Lerp` 1.0 0.0 `_新建轨道_0`))
        (`MeshComponent.SetScalarParameterValueOnMaterials` (`/Game/BP/Nova/BP_HomingMissile.Cone` _array_element) "Opacity" (`KismetMathLibrary.Lerp` 1.0 0.0 `_新建轨道_0`))
        (`MeshComponent.SetScalarParameterValueOnMaterials` (`self.Sphere1`) "Opacity" (`KismetMathLibrary.Lerp` 1.0 0.0 `_新建轨道_0`))))
    (:`Finished`
      (for _array_element_2 (`self.Missiles`)
        (`self.K2_DestroyActor` _array_element_2))
      (`self.K2_DestroyActor`))))

(event `self.SpawnIn`
  (bind (_returnvalue_roll _returnvalue_pitch _returnvalue_yaw) (`KismetMathLibrary.BreakRotator` (`KismetMathLibrary.RandomRotator` false)))
  (bind _returnvalue (`self.K2_GetActorLocation` (`GameplayStatics.GetPlayerCharacter` 0)))
  (bind _returnvalue_2 (+ (`self.SpawnHitLocation`) (* (`KismetMathLibrary.GetForwardVector` (`self.SpawnRotation`)) 100.0)))
  (set `self.SpawnRotation` (`KismetMathLibrary.MakeRotator` 0.0 0.0 _returnvalue_yaw) :!label _label)
  (bind _outhit (`KismetSystemLibrary.LineTraceSingleForObjects` _returnvalue (+ _returnvalue (* (`KismetMathLibrary.GetForwardVector` (`self.SpawnRotation`)) 3000.0)) (`|MakeArray` "ObjectTypeQuery5" :!type "EObjectTypeQuery Enum") true (`|MakeArray` self :!type "Actor Object Reference")))
  (bind (_bblockinghit _binitialoverlap _time _distance _location _impactpoint _normal _impactnormal _physmat _hitactor) (`GameplayStatics.BreakHitResult` _outhit))
  (cast `/Game/BP/Nova/BP_Portal` _hitactor)
  (if (<= _distance 1000.0)
    (goto _label)
    (else
      (set `self.SpawnHitLocation` _location)
      (`self.K2_SetActorLocation` _returnvalue_2)
      (`self.K2_SetActorRotation` (`KismetMathLibrary.FindLookAtRotation` _returnvalue_2 (`self.K2_GetActorLocation` (`GameplayStatics.GetPlayerCharacter` 0))))
      (`self.StartPush` (`KismetMathLibrary.GetDirectionUnitVector` _returnvalue_2 (`self.SpawnHitLocation`)) 10.0)
      (`|ExecutionSequence`
        (:`then_0`
          (`KismetSystemLibrary.Delay` 1.0)
          (bind _returnvalue_3 (`KismetSystemLibrary.K2_SetTimer` null "RotationtoPlayer" 0.01 true :!label _label_2))
          (set `self.RotationHandle` _returnvalue_3)
          (`/Engine/EditorBlueprintResources/StandardMacros.Gate` false :!label _label_3
            (:`Exit`
              (`self.StartPush` (0.0 0.0 0.0) 0.0))))
        (:`then_1`
          (goto _label_3 :!via `Close`))))))

(event `StartRotation`
  (goto _label_2))

(event `SpawnMissile`
  (`/Engine/EditorBlueprintResources/StandardMacros.DoOnce` false :!label _label_4
    (:`Completed`
      (for _array_element (`|MakeArray` (`self.LaunchPoint1`) (`self.LaunchPoint2`) (`self.LaunchPoint4`) (`self.LaunchPoint3`))
        (bind _returnvalue (`|SpawnActorFromClass` "/Game/BP/Nova/BP_HomingMissile.BP_HomingMissile_C" (`SceneComponent.K2_GetComponentToWorld` _array_element) "AlwaysSpawn" "MultiplyWithRoot" null null))
        (`KismetArrayLibrary.Array_AddUnique` (`self.Missiles`) _returnvalue)
        (`self.K2_AttachToComponent` _returnvalue _array_element "None" "KeepWorld" "SnapToTarget" "KeepWorld" true))
      (`KismetSystemLibrary.Delay` (`KismetMathLibrary.RandomFloatInRange` 1.0 3.0))
      (for _array_element_2 (`self.Missiles`)
        (`/Game/BP/Nova/BP_HomingMissile.Initialize` _array_element_2))
      (`KismetArrayLibrary.Array_Clear` (`self.Missiles`))
      (`KismetSystemLibrary.Delay` 1.5)
      (`self.ResetMissile`))))

(event `ResetMissile`
  (goto _label_4 :!via `Reset`))

(event `self.StartPush`
  (params (PushDirection :type "Vector Structure") (`Push Force` :type "Float (double-precision)"))
  (bind (_returnvalue_x _returnvalue_y _returnvalue_z) (`KismetMathLibrary.BreakVector` (`self.K2_GetActorLocation`)))
  (bind _array (`|MakeArray` "ObjectTypeQuery5" :!type "EObjectTypeQuery Enum"))
  (bind _homingtarget (`self.HomingTarget`))
  (bind _x (.x (`self.RandomPoint`)))
  (bind _y (.y (`self.RandomPoint`)))
  (`parent.StartPush` PushDirection `Push Force`)
  (`KismetSystemLibrary.RetriggerableDelay` 2.0 :!label _label_5)
  (set `ProjectileMovementComponent.bSimulationEnabled` true (`self.ProjectileMovement`) :!label _label_6)
  (bind _output_get (set `self.RandomPoint` (`KismetMathLibrary.RandomPointInBoundingBox` (`self.K2_GetActorLocation`) (`KismetMathLibrary.MakeVector` 5000.0 5000.0))))
  (if (>= (`KismetMathLibrary.Vector_Distance` _output_get (`self.K2_GetActorLocation` (`GameplayStatics.GetPlayerCharacter` 0))) 500.0)
    (bind (_outhit _returnvalue) (`KismetSystemLibrary.SphereTraceSingleForObjects` :`Start` _output_get :`End` _output_get :`Radius` 300.0 :`ObjectTypes` _array :`bTraceComplex` true :`DrawTime` 1.0))
    (bind (_outhit_2 _returnvalue_2) (`KismetSystemLibrary.LineTraceSingleForObjects` (`self.K2_GetActorLocation` (`GameplayStatics.GetPlayerCharacter` 0)) (`self.RandomPoint`) _array true))
    (if (or _returnvalue_2 _returnvalue)
      (goto _label_6)
      (else
        (`/Engine/EditorBlueprintResources/StandardMacros.IsValid` _homingtarget
          (:`Is Valid`
            (`self.K2_SetActorLocation` _homingtarget (`KismetMathLibrary.MakeVector` _x _y _returnvalue_z) false false))
          (:`Is Not Valid`
            (bind _returnvalue_3 (`|SpawnActorFromClass` "/Game/BP/Nova/BP_HomingTarget.BP_HomingTarget_C" (`KismetMathLibrary.MakeTransform` (`KismetMathLibrary.MakeVector` _x _y (.z (`self.RandomPoint`)))) "Undefined" "MultiplyWithRoot" null null))
            (bind _output_get_2 (set `self.HomingTarget` _returnvalue_3))))
        (set `ProjectileMovementComponent.HomingTargetComponent` (`/Game/BP/Nova/BP_HomingTarget.Sphere` _output_get_2) (`self.ProjectileMovement`))
        (goto _label_5)))
    (else
      (goto _label_6))))

(fn `RotationtoPlayer`
  (bind _returnvalue (`self.K2_GetActorRotation`))
  (bind _rotationspeed (`self.RotationSpeed`))
  (bind _returnvalue_2 (`KismetMathLibrary.FindLookAtRotation` (`self.K2_GetActorLocation`) (`self.K2_GetActorLocation` (`GameplayStatics.GetPlayerCharacter` 0))))
  (bind _yaw (.yaw (`KismetMathLibrary.NormalizedDeltaRotator` _returnvalue _returnvalue_2)))
  (bind (_returnvalue_roll _returnvalue_pitch _returnvalue_yaw) (`KismetMathLibrary.BreakRotator` (`KismetMathLibrary.SelectRotator` _returnvalue (`KismetMathLibrary.MakeRotator` (.roll _returnvalue) (.pitch _returnvalue) (+ (.yaw _returnvalue) (* (`KismetMathLibrary.Lerp` (* _rotationspeed 0.2) _rotationspeed (/ (`KismetMathLibrary.Abs` _yaw) 90.0)) (* (`KismetMathLibrary.SignOfFloat` _yaw) -1.0)))) (== _returnvalue _returnvalue_2 :`ErrorTolerance` 0.5))))
  (`self.K2_SetActorRotation` (`KismetMathLibrary.MakeRotator` 0.0 0.0 _returnvalue_yaw))
  (`self.SpawnMissile`))

(fn `UserConstructionScript`
  (`parent.UserConstructionScript`))