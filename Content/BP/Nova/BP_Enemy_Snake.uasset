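; Snake boss enemy that slides into the arena, hunts collectables it periodically spawns, and grows a chain of follower body segments.
; Homing ProjectileMovement steers it via a movable target actor toward the nearest collectable, or a trace-validated random point.
; Segments shoot at random intervals; once all are dead, PhaseShift emits a shockwave, revives them and advances the phase, which sets the body-length cap for resource spawning.
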(event `SpawnBody`
  (params (n :type Integer))
  (bind _body (`self.Body`))
  (bind _returnvalue (`KismetArrayLibrary.Array_Length` _body))
  (`|ExecutionSequence`
    (:`then_0`
      (goto _label :!via `Reset`))
    (:`then_1`
      (`/Engine/EditorBlueprintResources/StandardMacros.Do N` n :!label _label
        (:`Exit`
          (bind _returnvalue_2 (`|SpawnActorFromClass` "/Game/BP/Nova/BP_Enemy_SnakeBody.BP_Enemy_SnakeBody_C" (`KismetMathLibrary.MakeTransform` (`self.K2_GetActorLocation`)) "AlwaysSpawn" "MultiplyWithRoot" null null))
          (if (> _returnvalue 0)
            (set `/Game/BP/Nova/BP_Enemy_SnakeBody.Target` (`|GetArrayItem` _body (- _returnvalue 1)) _returnvalue_2)
            (set `/Game/BP/Nova/BP_Enemy_SnakeBody.Index` (+ _returnvalue 1) _returnvalue_2)
            (else
              (set `/Game/BP/Nova/BP_Enemy_SnakeBody.Target` self _returnvalue_2)
              (set `/Game/BP/Nova/BP_Enemy_SnakeBody.Index` 1 _returnvalue_2)))
          (`KismetArrayLibrary.Array_AddUnique` (`self.Body`) _returnvalue_2)
          (`KismetSystemLibrary.Delay` 0.1)
          (goto _label))))))

(event `self.ReceiveBeginPlay`
  (`parent.ReceiveBeginPlay`)
  (bind _returnvalue (`KismetSystemLibrary.K2_SetTimer` null "UpdatingLocation" 0.01 true))
  (set `self.UpdateHandle` _returnvalue)
  (`self.K2_SetActorLocation` (0.0 -2000.0 0.0))
  (`self.K2_SetActorRotation` (struct :`Yaw` 90.0))
  (bind (_direction `_新建轨道_0`) (`Timeline|时间轴_0` :!via `PlayFromStart`)
    (:`Update`
      (`self.K2_SetActorLocation` (`KismetMathLibrary.VLerp` (0.0 -2000.0 0.0) (0.0 -500.0 0.0) `_新建轨道_0`)))
    (:`Finished`
      (`|ExecutionSequence`
        (:`then_0`
          (`/Engine/EditorBlueprintResources/StandardMacros.Do N` 5 :!label _label_2
            (:`Exit`
              (`self.SpawnResource`)
              (goto _label_2))))
        (:`then_1`
          (`KismetSystemLibrary.Delay` 0.2)
          (`self.LookforRandomTarget`)
          (bind _returnvalue_2 (`KismetSystemLibrary.K2_SetTimer` null "SpawnResource" 5.0 true))
          (set `self.ResourceHandle` _returnvalue_2)
          (`KismetSystemLibrary.Delay` (`KismetMathLibrary.RandomFloatInRange` 3.0 8.0) :!label _label_3)
          (`self.ShootMode`)
          (goto _label_3))))))

(event `self.ReceiveTick`
  (params (DeltaSeconds :type "Float (single-precision)"))
  (`parent.ReceiveTick` DeltaSeconds))

(event `LookforRandomTarget`
  (bind _returnvalue (`self.K2_GetActorLocation`))
  (bind _array (`|MakeArray` "ObjectTypeQuery5" :!type "EObjectTypeQuery Enum"))
  (bind _homingtarget (`self.HomingTarget`))
  (bind _x (.x (`self.RandomPoint`)))
  (bind _y (.y (`self.RandomPoint`)))
  (bind _z (.z (`self.RandomPoint`)))
  (set `ProjectileMovementComponent.bSimulationEnabled` true (`self.ProjectileMovement`))
  (bind _valid (`self.ResourceSpotted` :!label _label_4))
  (if (not _valid)
    (bind _output_get (set `self.RandomPoint` (`KismetMathLibrary.RandomPointInBoundingBox` _returnvalue (`KismetMathLibrary.MakeVector` 5000.0 5000.0))))
    (if (<= (`KismetMathLibrary.Vector_Distance` _output_get _returnvalue) 300.0)
      (goto _label_4)
      (else
        (bind (_outhit _returnvalue_2) (`KismetSystemLibrary.SphereTraceSingleForObjects` :`Start` _output_get :`End` _output_get :`Radius` 500.0 :`ObjectTypes` _array :`DrawTime` 1.0))
        (bind (_outhit_2 _returnvalue_3) (`KismetSystemLibrary.LineTraceSingleForObjects` (`self.K2_GetActorLocation` (`GameplayStatics.GetPlayerCharacter` 0)) (`self.RandomPoint`) _array true))
        (if (or _returnvalue_3 _returnvalue_2)
          (goto _label_4)
          (else
            _)))))
  (`/Engine/EditorBlueprintResources/StandardMacros.IsValid` _homingtarget
    (:`Is Valid`
      (`self.K2_SetActorLocation` _homingtarget (`KismetMathLibrary.MakeVector` _x _y _z) false false))
    (:`Is Not Valid`
      (bind _returnvalue_4 (`|SpawnActorFromClass` "/Game/BP/Nova/BP_HomingTarget.BP_HomingTarget_C" (`KismetMathLibrary.MakeTransform` (`KismetMathLibrary.MakeVector` _x _y _z)) "Undefined" "MultiplyWithRoot" null null))
      (bind _output_get_2 (set `self.HomingTarget` _returnvalue_4))))
  (set `ProjectileMovementComponent.HomingTargetComponent` (`/Game/BP/Nova/BP_HomingTarget.Sphere` _output_get_2) (`self.ProjectileMovement`))
  (`KismetSystemLibrary.RetriggerableDelay` 1.0)
  (goto _label_4))

(event `PhaseShift`
  (`|ExecutionSequence`
    (:`then_0`
      (goto _label_5 :!via `Open`))
    (:`then_1`
      (for _array_element (`self.Body`)
        (if (not (`/Game/BP/Nova/BP_Enemy_SnakeBody.Dead` _array_element))
          (goto _label_5 :!via `Close`)))
      (`/Engine/EditorBlueprintResources/StandardMacros.Gate` false :!label _label_5
        (:`Exit`
          (set `ProjectileMovementComponent.bSimulationEnabled` false (`self.ProjectileMovement`))
          (`/Engine/EditorBlueprintResources/StandardMacros.IncrementInt` (`self.Phase`)
            (:`  `
              (`|SpawnActorFromClass` "/Game/BP/Nova/BP_Shockwave.BP_Shockwave_C" (`KismetMathLibrary.MakeTransform` (`self.K2_GetActorLocation`)) "Undefined" "MultiplyWithRoot" null null)
              (`KismetSystemLibrary.Delay` 2.0)
              (for _array_element_2 (`self.Body`)
                (`/Game/BP/Nova/BP_Enemy_SnakeBody.Revive` _array_element_2))
              (`KismetSystemLibrary.Delay` 1.0)
              (`self.LookforRandomTarget`))))))))

(fn `ResourceSpotted`
  (returns (Valid :type Boolean))
  (set `self.MinimumDistance` 10000.0)
  (bind _outactors (`GameplayStatics.GetAllActorsOfClass` "/Game/BP/Nova/BP_Collectables_Snake.BP_Collectables_Snake_C"))
  (`/Engine/EditorBlueprintResources/StandardMacros.IsValid` (`|GetArrayItem` _outactors)
    (:`Is Valid`
      (for _array_element _outactors
        (bind _returnvalue (`self.K2_GetActorLocation` _array_element))
        (bind _returnvalue_2 (`KismetMathLibrary.Vector_Distance` _returnvalue (`self.K2_GetActorLocation`)))
        (if (< _returnvalue_2 (`self.MinimumDistance`))
          (set `self.MinimumDistance` _returnvalue_2)
          (set `self.RandomPoint` _returnvalue)))
      (return true))
    (:`Is Not Valid`
      (return false))))

(fn `ShootMode`
  (if (`ProjectileMovementComponent.bSimulationEnabled` (`self.ProjectileMovement`))
    (for _array_element (`self.Body`)
      (`/Game/BP/Nova/BP_Enemy_SnakeBody.Shooting` _array_element))))

(fn `SpawnResource`
  (locals (RandomPoint :type "Vector Structure" :default (0.0 0.0 0.0)))
  (if (not (>= (`KismetArrayLibrary.Array_Length` (`self.Body`)) (select `int` (`self.Phase`) :`0` 8 :`1` 15 :`2` 20)))
    (bind _output_get (set `local.RandomPoint` (`KismetMathLibrary.RandomPointInBoundingBox` (0.0 0.0 0.0) (450.0 900.0 0.0))))
    (if (< (`KismetMathLibrary.Vector_Distance` _output_get (`self.K2_GetActorLocation`)) 500.0)
      (`self.SpawnResource`)
      (else
        (bind _returnvalue (`|SpawnActorFromClass` "/Game/BP/Nova/BP_Collectables_Snake.BP_Collectables_Snake_C" (`KismetMathLibrary.MakeTransform` _output_get) "Undefined" "MultiplyWithRoot" null null))
        (set `/Game/BP/Nova/BP_Collectables.Target` self _returnvalue)))))

(fn `UpdatingLocation`
  (bind _returnvalue (`SceneComponent.K2_GetComponentLocation` (`self.AttachPoint`)))
  (if (> (`KismetMathLibrary.Vector_Distance` _returnvalue (`self.UpdateLocation`)) 50.0)
    (set `self.UpdateLocation` _returnvalue)))

(fn `UserConstructionScript`
  (`parent.UserConstructionScript`))