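; A snake collectable that grows a BP_Enemy_Snake by one body segment when collected, and can be shot away by projectiles.
; On spawn, a timeline shrinks it from triple size while driving Sphere opacity, enabling collision when finished.
; Projectile overlaps reduce its health until it triggers Destroyed.
; Hit and Destroyed share a reversed timeline exit that disables collision, then calls the parent Hit.
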(event `self.ReceiveBeginPlay`
  (bind _initialscale (`self.InitialScale`))
  (`parent.ReceiveBeginPlay`)
  (set `self.InitialScale` (`self.GetActorScale3D`))
  (`self.SetActorEnableCollision` false)
  (bind (_direction `_新建轨道_0`) (`Timeline|时间轴_0` :!via `PlayFromStart`)
    (:`Update`
      (`self.SetActorScale3D` (`KismetMathLibrary.VLerp` (* _initialscale 3.0) _initialscale `_新建轨道_0`))
      (`MeshComponent.SetScalarParameterValueOnMaterials` (`self.Sphere`) "Opacity" `_新建轨道_0`))
    (:`Finished`
      (`self.SetActorEnableCollision` true))))

(event `self.ReceiveActorBeginOverlap`
  (params (OtherActor :type "Actor Object Reference"))
  (`parent.ReceiveActorBeginOverlap` OtherActor)
  (bind _asbp_projectile (cast `/Game/BP/Nova/BP_Projectile` OtherActor))
  (`/Game/BP/Nova/BP_Projectile.ProjectileHit` _asbp_projectile)
  (bind _output_get (set `self.Health` (- (`self.Health`) 0.2)))
  (if (<= _output_get 0.0)
    (`self.Destroyed`)))

(event `self.Hit`
  (bind _initialscale (`self.InitialScale`))
  (bind _asbp_enemy_snake (cast `/Game/BP/Nova/BP_Enemy_Snake` (`self.Target`)))
  (`/Game/BP/Nova/BP_Enemy_Snake.SpawnBody` _asbp_enemy_snake 1)
  (`self.SetActorEnableCollision` false :!label _label)
  (bind (_direction `_新建轨道_0`) (`Timeline|时间轴_1` :!via `ReverseFromEnd`)
    (:`Update`
      (`self.SetActorScale3D` (`KismetMathLibrary.VLerp` (* _initialscale 3.0) _initialscale `_新建轨道_0`))
      (`MeshComponent.SetScalarParameterValueOnMaterials` (`self.Sphere`) "Opacity" `_新建轨道_0`))
    (:`Finished`
      (`parent.Hit`))))

(event `Destroyed`
  (goto _label))

(fn `UserConstructionScript`
  (`parent.UserConstructionScript`))