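; BP_Bricks_Enemy is an enemy Blueprint, named for bricks, that tracks health and reacts to damage.
; Its AnyDamage event subtracts incoming damage from Health and, at zero or below, calls Destroyed through a DoOnce so it fires only once.
; BeginPlay, overlap and Tick are disabled placeholders, and the construction script only calls its parent.
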(event `self.ReceiveAnyDamage`
  (params (Damage :type "Float (single-precision)") (DamageType :type "DamageType Object Reference") (InstigatedBy :type "Controller Object Reference") (DamageCauser :type "Actor Object Reference"))
  (bind _output_get (set `self.Health` (- (`self.Health`) Damage)))
  (if (<= _output_get 0.0)
    (`/Engine/EditorBlueprintResources/StandardMacros.DoOnce` false
      (:`Completed`
        (`self.Destroyed`)))))

(fn `UserConstructionScript`
  (`parent.UserConstructionScript`))