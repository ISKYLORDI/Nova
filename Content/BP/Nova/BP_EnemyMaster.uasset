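; Base enemy Blueprint that handles health, player-collision knockback and pickup drops, with empty SpawnIn and Death events.
; Damage lowers HP; at zero it destroys any HomingTarget and calls Death.
; Player hits start knockback scaled by player speed, applied as decaying horizontal offsets by a looping Push timer; its wall-bounce logic is disconnected.
; SpawnCollectible, not called here, has a random chance to spawn a bullet collectible targeting the player.
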(event `self.ReceiveBeginPlay`
  (set `self.Scale` (`self.GetActorScale3D`)))

(event `self.ReceiveAnyDamage`
  (params (Damage :type "Float (single-precision)") (DamageType :type "DamageType Object Reference") (InstigatedBy :type "Controller Object Reference") (DamageCauser :type "Actor Object Reference"))
  (bind _homingtarget (`self.HomingTarget`))
  (bind _output_get (set `self.HP` (- (`self.HP`) Damage)))
  (if (<= _output_get 0.0)
    (`/Engine/EditorBlueprintResources/StandardMacros.IsValid` _homingtarget
      (:`Is Valid`
        (`self.K2_DestroyActor` _homingtarget))
      (:`Is Not Valid`
        _))
    (`self.Death`)))

(event `SpawnIn`)

(event `Death`)

(event `StartPush`
  (params (PushDirection :type "Vector Structure") (`Push Force` :type "Float (double-precision)" :default 3.0))
  (set `self.PushDirection` PushDirection)
  (set `self.Push Force` `Push Force`)
  (bind _returnvalue (`KismetSystemLibrary.K2_SetTimer` null "Push" 0.01 true))
  (set `self.PushHandle` _returnvalue))

(event `self.CapsuleComponent.OnComponentHit`
  (params (HitComponent :type "PrimitiveComponent Object Reference") (OtherActor :type "Actor Object Reference") (OtherComp :type "PrimitiveComponent Object Reference") (NormalImpulse :type "Vector Structure") (Hit :type "HitResult Structure (by ref)"))
  (bind _knockbackscale (`self.KnockBackScale`))
  (cast `/Game/BP/Nova/BP_PLayer1` OtherActor)
  (if (> _knockbackscale 0.0)
    (`self.StartPush` (`KismetMathLibrary.GetDirectionUnitVector` (`self.K2_GetActorLocation` OtherActor) (`self.K2_GetActorLocation`)) (* (`KismetMathLibrary.Lerp` 1.0 10.0 (/ (`KismetMathLibrary.VSize` (`self.GetVelocity` OtherActor)) 800.0)) _knockbackscale))))

(event `self.CapsuleComponent.OnComponentBeginOverlap`
  (params (OverlappedComponent :type "PrimitiveComponent Object Reference") (OtherActor :type "Actor Object Reference") (OtherComp :type "PrimitiveComponent Object Reference") (OtherBodyIndex :type Integer) (bFromSweep :type Boolean) (SweepResult :type "HitResult Structure (by ref)")))

(event `SpawnCollectible`
  (if (>= (`KismetMathLibrary.RandomFloat`) 0.8)
    (bind _returnvalue (`|SpawnActorFromClass` "/Game/BP/Nova/BP_Collectables_Bullets.BP_Collectables_Bullets_C" (`KismetMathLibrary.MakeTransform` (`self.K2_GetActorLocation`)) "Undefined" "MultiplyWithRoot" null null))
    (set `/Game/BP/Nova/BP_Collectables.Target` (`GameplayStatics.GetPlayerPawn` 0) _returnvalue)))

(event `self.ReceiveTick`
  (params (DeltaSeconds :type "Float (single-precision)")))

(fn `Push`
  (bind _returnvalue (`self.K2_GetActorLocation`))
  (bind (_returnvalue_x _returnvalue_y) (`KismetMathLibrary.BreakVector` (* (`self.PushDirection`) (`self.Push Force`))))
  (bind (_outhit _returnvalue_2) (`KismetSystemLibrary.SphereTraceSingleForObjects` _returnvalue (+ _returnvalue (* (`self.PushDirection`) 1.0)) (`CapsuleComponent.CapsuleRadius` (`self.CapsuleComponent`)) (`|MakeArray` "ObjectTypeQuery3" "ObjectTypeQuery6" :!type "EObjectTypeQuery Enum") true (`|MakeArray` self :!type "Actor Object Reference") "None" true (struct :`R` 1.0 :`A` 1.0) (struct :`G` 1.0 :`A` 1.0) 1.0))
  (`self.K2_AddActorWorldOffset` (`KismetMathLibrary.MakeVector` _returnvalue_x _returnvalue_y))
  (bind _output_get (set `self.Push Force` (- (`self.Push Force`) (`KismetMathLibrary.Lerp` 0.01 0.05 (/ (`self.Push Force`) 5.0)))))
  (if (<= _output_get 0.01)
    (`KismetSystemLibrary.K2_ClearAndInvalidateTimerHandle` (`self.PushHandle`))))

(fn `UserConstructionScript`)