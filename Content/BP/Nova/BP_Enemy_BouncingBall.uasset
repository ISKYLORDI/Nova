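; BP_Enemy_BouncingBall is a ball enemy that ricochets in the yaw plane and scales up on spawn.
; Each tick, a sphere trace triggers gated reflections off bricks, the player and portals, spending limited bounces and destroying player bricks.
; Bounce boards reflect it at quadruple speed, with excess speed gradually damped.
; Exhausted bounces or distance from the player trigger death: collectible drop, Niagara burst, expanding fade-out, destruction.
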(event `self.ReceiveBeginPlay`
  (`parent.ReceiveBeginPlay`)
  (bind (_direction `_新建轨道_0`) (`Timeline|时间轴_0`)
    (:`Update`
      (`self.SetActorScale3D` (`KismetMathLibrary.VLerp` (0.0 0.0 0.0) (`self.Scale`) `_新建轨道_0`)))))

(event `self.Death`
  (bind _scale (`self.Scale`))
  (`parent.Death`)
  (`self.SpawnCollectible`)
  (`self.SetActorEnableCollision` false)
  (`NiagaraFunctionLibrary.SpawnSystemAtLocation` "/Game/VFX/BlinkAndDashVFX/VFX_Niagara/NS_Blink_Fire.NS_Blink_Fire" (`self.K2_GetActorLocation`) (struct) (0.5 0.5 0.5))
  (bind (_direction `_新建轨道_0`) (`Timeline|时间轴_1`)
    (:`Update`
      (`self.SetActorScale3D` (`KismetMathLibrary.VLerp` _scale (* _scale 3.0) `_新建轨道_0`))
      (`MeshComponent.SetScalarParameterValueOnMaterials` (`self.Sphere`) "Opacity" (`KismetMathLibrary.Lerp` 1.0 0.0 `_新建轨道_0`)))
    (:`Finished`
      (`self.K2_DestroyActor`))))

(event `self.StartPush`
  (params (PushDirection :type "Vector Structure") (`Push Force` :type "Float (double-precision)")))

(event `self.ReceiveTick`
  (params (DeltaSeconds :type "Float (single-precision)"))
  (bind _returnvalue (`self.K2_GetActorLocation`))
  (bind _returnvalue_2 (`KismetMathLibrary.MakeVector` 0.0))
  (bind (_returnvalue_x _returnvalue_y _returnvalue_z) (`KismetMathLibrary.BreakVector` (`self.GetActorScale3D`)))
  (bind _projectilemovement (`self.ProjectileMovement`))
  (bind _projectilemovement_2 (`self.ProjectileMovement`))
  (bind _velocity (`MovementComponent.Velocity` _projectilemovement_2))
  (bind _returnvalue_3 (`KismetMathLibrary.VSize` _velocity))
  (`parent.ReceiveTick` DeltaSeconds)
  (`|ExecutionSequence`
    (:`then_0`
      (bind _outhit (`KismetSystemLibrary.SphereTraceSingleForObjects` _returnvalue (+ _returnvalue (* (`KismetMathLibrary.GetDirectionUnitVector` (`KismetMathLibrary.MakeVector` 0.0) (`MovementComponent.Velocity` (`self.ProjectileMovement`))) 1.0)) (* 50.0 _returnvalue_z) (`|MakeArray` "ObjectTypeQuery1" "ObjectTypeQuery5" "ObjectTypeQuery3" "ObjectTypeQuery6" :!type "EObjectTypeQuery Enum")))
      (bind (_bblockinghit _binitialoverlap _time _distance _location _impactpoint _normal _impactnormal _physmat _hitactor) (`GameplayStatics.BreakHitResult` _outhit))
      (cast `/Game/BP/Nova/BP_Bricks` _hitactor
        (:`then`
          (`/Engine/EditorBlueprintResources/StandardMacros.DoOnce` false :!label _label
            (:`Completed`
              (if (> (`self.BounceTimes`) 0)
                (bind _returnvalue_4 (`KismetMathLibrary.FindLookAtRotation` _returnvalue_2 _impactnormal))
                (bind (_returnvalue_roll _returnvalue_pitch _returnvalue_yaw) (`KismetMathLibrary.BreakRotator` (`KismetMathLibrary.NormalizedDeltaRotator` (`KismetMathLibrary.FindLookAtRotation` _returnvalue_2 (* (`MovementComponent.Velocity` (`self.ProjectileMovement`)) -1.0)) _returnvalue_4)))
                (bind _returnvalue_5 (* (`KismetMathLibrary.GetForwardVector` (`KismetMathLibrary.MakeRotator` 0.0 0.0 (- (.yaw _returnvalue_4) _returnvalue_yaw))) (`KismetMathLibrary.VSize` (`MovementComponent.Velocity` _projectilemovement))))
                (set `MovementComponent.Velocity` _returnvalue_5 _projectilemovement)
                (`|ExecutionSequence`
                  (:`then_0`
                    (bind _asbp_bricks_player (cast `/Game/BP/Nova/BP_Bricks_Player` _hitactor :!label _label_2))
                    (`/Game/BP/Nova/BP_Bricks.Destroyed` _asbp_bricks_player))
                  (:`then_1`
                    (`KismetSystemLibrary.Delay` 0.05)
                    (goto _label :!via `Reset`))
                  (:`then_2`
                    (`KismetSystemLibrary.Delay` 0.05)
                    (goto _label_3 :!via `Reset`))
                  (:`then_3`
                    (`/Engine/EditorBlueprintResources/StandardMacros.DecrementInt` (`self.BounceTimes`))))
                (else
                  (`self.Death`))))))
        (:`CastFailed`
          (cast `/Game/BP/Nova/BP_PLayer1` _hitactor
            (:`then`
              (goto _label))
            (:`CastFailed`
              (cast `/Game/BP/Nova/BP_Portal` _hitactor
                (:`then`
                  (goto _label))
                (:`CastFailed`
                  (cast `/Game/BP/Nova/BP_BounceBoard` _hitactor)
                  (`/Engine/EditorBlueprintResources/StandardMacros.DoOnce` false :!label _label_3
                    (:`Completed`
                      (set `MovementComponent.Velocity` (* _returnvalue_5 4.0) _projectilemovement)
                      (goto _label_2))))))))))
    (:`then_1`
      (if (> _returnvalue_3 700.0)
        (set `MovementComponent.Velocity` (* (`KismetMathLibrary.GetDirectionUnitVector` (`KismetMathLibrary.MakeVector` 0.0) _velocity) (* _returnvalue_3 0.99)) _projectilemovement_2)))
    (:`then_2`
      (if (>= (`KismetMathLibrary.Vector_Distance` (`self.K2_GetActorLocation`) (`self.K2_GetActorLocation` (`GameplayStatics.GetPlayerCharacter` 0))) 3000.0)
        (`self.Death`)))))

(fn `UserConstructionScript`
  (`parent.UserConstructionScript`))