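; Assault enemy that charges up and dashes in the player's facing line, launching the player on overlap.
; Spawns at a BP_Portal traced from the player, then a looping timer turns it until aligned, triggering a glow timeline and a lerped dash toward the traced portal.
; StartPush also loops homing projectile movement through random, trace-checked points near the player.
; Death spawns a collectible and VFX, then scales up and fades out before destruction.
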(event `self.ReceiveBeginPlay`
  (set `self.Scale` (`self.GetActorScale3D`)))

(event `self.Death`
  (bind _scale (`self.Scale`))
  (`parent.Death`)
  (`self.SpawnCollectible`)
  (`self.SetActorEnableCollision` false)
  (`NiagaraFunctionLibrary.SpawnSystemAtLocation` "/Game/VFX/BlinkAndDashVFX/VFX_Niagara/NS_Blink_Fire.NS_Blink_Fire" (`self.K2_GetActorLocation`) (struct) (0.5 0.5 0.5))
  (bind (_direction `_新建轨道_0`) (`Timeline|时间轴_3`)
    (:`Update`
      (`self.SetActorScale3D` (`KismetMathLibrary.VLerp` _scale (* _scale 3.0) `_新建轨道_0`))
      (`MeshComponent.SetScalarParameterValueOnMaterials` (`self.Cone`) "Opacity" (`KismetMathLibrary.Lerp` 1.0 0.0 `_新建轨道_0`)))
    (:`Finished`
      (`self.K2_DestroyActor`))))

(event `self.Box.OnComponentBeginOverlap`
  (params (OverlappedComponent :type "PrimitiveComponent Object Reference") (OtherActor :type "Actor Object Reference") (OtherComp :type "PrimitiveComponent Object Reference") (OtherBodyIndex :type Integer) (bFromSweep :type Boolean) (SweepResult :type "HitResult Structure (by ref)"))
  (if (`self.Dashing`)
    (bind _asbp_player_1 (cast `/Game/BP/Nova/BP_PLayer1` OtherActor))
    (`self.LaunchCharacter` _asbp_player_1 (* (`self.GetActorForwardVector`) 50.0) false false)))

(event `self.SpawnIn`
  (bind (_returnvalue_roll _returnvalue_pitch _returnvalue_yaw) (`KismetMathLibrary.BreakRotator` (`KismetMathLibrary.RandomRotator` false)))
  (bind _returnvalue (`self.K2_GetActorLocation` (`GameplayStatics.GetPlayerCharacter` 0)))
  (bind _returnvalue_2 (+ (`self.SpawnHitLocation`) (* (`KismetMathLibrary.GetForwardVector` (`self.SpawnRotation`)) 100.0)))
  (set `self.SpawnRotation` (`KismetMathLibrary.MakeRotator` 0.0 0.0 _returnvalue_yaw) :!label _label)
  (bind _outhit (`KismetSystemLibrary.LineTraceSingleForObjects` _returnvalue (+ _returnvalue (* (`KismetMathLibrary.GetForwardVector` (`self.SpawnRotation`)) 3000.0)) (`|MakeArray` "ObjectTypeQuery5" :!type "EObjectTypeQuery Enum") true (`|MakeArray` self :!type "Actor Object Reference")))
  (bind (_bblockinghit _binitialoverlap _time _distance _location _impactpoint _normal _impactnormal _physmat _hitactor) (`GameplayStatics.BreakHitResult` _outhit))
  (cast `/Game/BP/Nova/BP_Portal` _hitactor)
  (if (<= _distance 1000.0)
    (goto _label)
    (else
      (set `self.SpawnHitLocation` _location)
      (`self.K2_SetActorLocation` _returnvalue_2)
      (`self.K2_SetActorRotation` (`KismetMathLibrary.FindLookAtRotation` _returnvalue_2 (`self.K2_GetActorLocation` (`GameplayStatics.GetPlayerCharacter` 0))))
      (`self.StartPush` (`KismetMathLibrary.GetDirectionUnitVector` _returnvalue_2 (`self.SpawnHitLocation`)) 10.0)
      (`|ExecutionSequence`
        (:`then_0`
          (`KismetSystemLibrary.Delay` 1.0)
          (bind _returnvalue_3 (`KismetSystemLibrary.K2_SetTimer` null "RotationtoPlayer" 0.01 true :!label _label_2))
          (set `self.RotationHandle` _returnvalue_3)
          (`/Engine/EditorBlueprintResources/StandardMacros.Gate` false :!label _label_3
            (:`Exit`
              (`self.StartPush` (0.0 0.0 0.0) 0.0))))
        (:`then_1`
          (goto _label_3 :!via `Close`))))))

(event `StartRotation`
  (goto _label_2))

(event `Assault`
  (bind _startlocation (`self.StartLocation`))
  (bind _endlocation (`self.EndLocation`))
  (if (and (== (`KismetMathLibrary.FindLookAtRotation` (`self.K2_GetActorLocation`) (`self.K2_GetActorLocation` (`GameplayStatics.GetPlayerCharacter` 0))) (`self.K2_GetActorRotation`) :`ErrorTolerance` 3.0) (`KismetSystemLibrary.K2_IsValidTimerHandle` (`self.RotationHandle`)))
    (`/Engine/EditorBlueprintResources/StandardMacros.DoOnce` false :!label _label_4
      (:`Completed`
        (bind (_direction `_新建轨道_0`) (`Timeline|时间轴_0` :!via `PlayFromStart`)
          (:`Update`
            (`MeshComponent.SetScalarParameterValueOnMaterials` (`self.Cone`) "Intensity" (`KismetMathLibrary.Lerp` 10.0 70.0 `_新建轨道_0`)))
          (:`Finished`
            (`self.GetDashLocation`)
            (`|ExecutionSequence`
              (:`then_0`
                (`KismetSystemLibrary.K2_ClearAndInvalidateTimerHandle` (`self.RotationHandle`))
                (bind (_direction_2 `_新建轨道_0_2`) (`Timeline|时间轴_1` :!via `ReverseFromEnd`)
                  (:`Update`
                    (`MeshComponent.SetScalarParameterValueOnMaterials` (`self.Cone`) "Intensity" (`KismetMathLibrary.Lerp` 10.0 70.0 `_新建轨道_0_2`)))
                  (:`Finished`
                    (`KismetSystemLibrary.Delay` 1.5)
                    (`self.Reset Assault`))))
              (:`then_1`
                (`TimelineComponent.SetPlayRate` (`self.时间轴_2`) 2.0)
                (set `self.Dashing` true)
                (bind (_direction_3 `_新建轨道_0_3`) (`Timeline|时间轴_2` :!via `PlayFromStart`)
                  (:`Update`
                    (`self.K2_SetActorLocation` (`KismetMathLibrary.VLerp` _startlocation _endlocation `_新建轨道_0_3`)))
                  (:`Finished`
                    (set `self.Dashing` false)
                    (`self.StartPush` (`KismetMathLibrary.GetDirectionUnitVector` _startlocation _endlocation))
                    (bind _returnvalue (`KismetSystemLibrary.K2_SetTimer` null "RotationtoPlayer" 0.01 true))
                    (set `self.RotationHandle` _returnvalue)))))))))))

(event `Reset Assault`
  (goto _label_4 :!via `Reset`))

(event `self.StartPush`
  (params (PushDirection :type "Vector Structure") (`Push Force` :type "Float (double-precision)"))
  (bind _array (`|MakeArray` "ObjectTypeQuery5" :!type "EObjectTypeQuery Enum"))
  (bind _homingtarget (`self.HomingTarget`))
  (bind _x (.x (`self.RandomPoint`)))
  (bind _y (.y (`self.RandomPoint`)))
  (bind _z (.z (`self.RandomPoint`)))
  (`parent.StartPush` PushDirection `Push Force`)
  (`KismetSystemLibrary.RetriggerableDelay` 1.0 :!label _label_5)
  (set `ProjectileMovementComponent.bSimulationEnabled` true (`self.ProjectileMovement`) :!label _label_6)
  (bind _output_get (set `self.RandomPoint` (`KismetMathLibrary.RandomPointInBoundingBox` (`self.K2_GetActorLocation`) (`KismetMathLibrary.MakeVector` 5000.0 5000.0))))
  (if (<= (`KismetMathLibrary.Vector_Distance` _output_get (`self.K2_GetActorLocation` (`GameplayStatics.GetPlayerCharacter` 0))) 800.0)
    (bind (_outhit _returnvalue) (`KismetSystemLibrary.SphereTraceSingleForObjects` :`Start` _output_get :`End` _output_get :`Radius` 200.0 :`ObjectTypes` _array :`bTraceComplex` true :`DrawTime` 1.0))
    (bind (_outhit_2 _returnvalue_2) (`KismetSystemLibrary.LineTraceSingleForObjects` (`self.K2_GetActorLocation` (`GameplayStatics.GetPlayerCharacter` 0)) (`self.RandomPoint`) _array true))
    (if (or _returnvalue_2 _returnvalue)
      (goto _label_6)
      (else
        (`/Engine/EditorBlueprintResources/StandardMacros.IsValid` _homingtarget
          (:`Is Valid`
            (`self.K2_SetActorLocation` _homingtarget (`KismetMathLibrary.MakeVector` _x _y _z) false false))
          (:`Is Not Valid`
            (bind _returnvalue_3 (`|SpawnActorFromClass` "/Game/BP/Nova/BP_HomingTarget.BP_HomingTarget_C" (`KismetMathLibrary.MakeTransform` (`KismetMathLibrary.MakeVector` _x _y _z)) "Undefined" "MultiplyWithRoot" null null))
            (bind _output_get_2 (set `self.HomingTarget` _returnvalue_3))))
        (set `ProjectileMovementComponent.HomingTargetComponent` (`/Game/BP/Nova/BP_HomingTarget.Sphere` _output_get_2) (`self.ProjectileMovement`))
        (goto _label_5)))
    (else
      (goto _label_6))))

(fn `GetDashLocation`
  (bind _returnvalue (`self.K2_GetActorLocation`))
  (bind _startlocation (`self.StartLocation`))
  (set `self.StartLocation` _returnvalue)
  (bind _outhit (`KismetSystemLibrary.LineTraceSingleForObjects` _returnvalue (+ _returnvalue (* (`self.GetActorForwardVector`) 3000.0)) (`|MakeArray` "ObjectTypeQuery5" :!type "EObjectTypeQuery Enum") true))
  (bind (_bblockinghit _binitialoverlap _time _distance _location _impactpoint _normal _impactnormal _physmat _hitactor) (`GameplayStatics.BreakHitResult` _outhit))
  (cast `/Game/BP/Nova/BP_Portal` _hitactor)
  (bind _returnvalue_2 (+ _location (* (`KismetMathLibrary.GetDirectionUnitVector` _location (`self.K2_GetActorLocation`)) 300.0)))
  (set `self.EndLocation` (select `bool` (< (`KismetMathLibrary.Vector_Distance` _startlocation _returnvalue_2) (`KismetMathLibrary.Vector_Distance` _startlocation (`self.K2_GetActorLocation` (`GameplayStatics.GetPlayerCharacter` 0)))) :`false` _returnvalue_2 :`true` _location)))

(fn `RotationtoPlayer`
  (bind _returnvalue (`self.K2_GetActorRotation`))
  (bind _rotationspeed (`self.RotationSpeed`))
  (bind _rotationspeed_2 (`self.RotationSpeed`))
  (bind _returnvalue_2 (`KismetMathLibrary.FindLookAtRotation` (`self.K2_GetActorLocation`) (`self.K2_GetActorLocation` (`GameplayStatics.GetPlayerCharacter` 0))))
  (bind _pitch (.pitch (`KismetMathLibrary.NormalizedDeltaRotator` _returnvalue _returnvalue_2)))
  (bind _yaw (.yaw (`KismetMathLibrary.NormalizedDeltaRotator` _returnvalue _returnvalue_2)))
  (bind (_returnvalue_roll _returnvalue_pitch _returnvalue_yaw) (`KismetMathLibrary.BreakRotator` (`KismetMathLibrary.SelectRotator` _returnvalue (`KismetMathLibrary.MakeRotator` (.roll _returnvalue) (+ (.pitch _returnvalue) (* (`KismetMathLibrary.Lerp` (* _rotationspeed 1.0) _rotationspeed (/ (`KismetMathLibrary.Abs` _pitch) 90.0)) (* (`KismetMathLibrary.SignOfFloat` _pitch) -1.0))) (+ (.yaw _returnvalue) (* (`KismetMathLibrary.Lerp` (* _rotationspeed_2 1.0) _rotationspeed_2 (/ (`KismetMathLibrary.Abs` _yaw) 90.0)) (* (`KismetMathLibrary.SignOfFloat` _yaw) -1.0)))) (== _returnvalue _returnvalue_2 :`ErrorTolerance` 0.5))))
  (`self.K2_SetActorRotation` (`KismetMathLibrary.MakeRotator` 0.0 0.0 _returnvalue_yaw))
  (`self.Assault`))

(fn `UserConstructionScript`
  (`parent.UserConstructionScript`))