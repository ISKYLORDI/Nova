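; BP_Collectables is a glowing pickup that wanders until the player comes near, then flies to them.
; It spawns a BP_HomingTarget as its projectile homing target, periodically moved to random nearby horizontal points through Delays on Tick.
; Within CollectDistance, homing switches to the player with new speed settings and a faster timeline-driven emissive-intensity pulse.
; Overlapping BP_PLayer1 destroys the pickup and its target, with no reward logic here.
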(event `self.ReceiveBeginPlay`
  (bind _returnvalue (`|SpawnActorFromClass` "/Game/BP/BP_HomingTarget.BP_HomingTarget_C" (`self.GetTransform`) "Undefined" "MultiplyWithRoot" null null))
  (bind _output_get (set `self.Homingtarget` _returnvalue))
  (set `ProjectileMovementComponent.HomingTargetComponent` (`Actor.RootComponent` _output_get) (`self.ProjectileMovement`))
  (`|ExecutionSequence`
    (:`then_0`
      (bind (_direction `_新建轨道_0`) (`Timeline|时间轴`)
        (:`Update`
          (`MeshComponent.SetScalarParameterValueOnMaterials` (`self.Sphere`) "Intensity" (`KismetMathLibrary.Lerp` 10.0 40.0 `_新建轨道_0`)))))
    (:`then_1`
      (`self.K2_SetActorLocation` (`self.Homingtarget`) (`KismetMathLibrary.RandomPointInBoundingBox` (`self.K2_GetActorLocation`) (500.0 500.0 0.0)) false false :!label _label))))

(event `self.ReceiveTick`
  (params (DeltaSeconds :type "Float (single-precision)"))
  (bind _returnvalue (`GameplayStatics.GetPlayerCharacter` 0))
  (bind _projectilemovement (`self.ProjectileMovement`))
  (`KismetSystemLibrary.Delay` 0.1)
  (if (<= (`KismetMathLibrary.Vector_Distance` (`self.K2_GetActorLocation`) (`self.K2_GetActorLocation` _returnvalue)) (`self.CollectDistance`))
    (set `ProjectileMovementComponent.HomingTargetComponent` (`Actor.RootComponent` _returnvalue) _projectilemovement)
    (set `ProjectileMovementComponent.MaxSpeed` 1200.0 _projectilemovement)
    (set `ProjectileMovementComponent.HomingAccelerationMagnitude` 8000.0 _projectilemovement)
    (`TimelineComponent.SetPlayRate` (`self.时间轴`) 2.0)
    (else
      (`KismetSystemLibrary.Delay` 1.5)
      (goto _label))))

(event `self.Sphere.OnComponentBeginOverlap`
  (params (OverlappedComponent :type "PrimitiveComponent Object Reference") (OtherActor :type "Actor Object Reference") (OtherComp :type "PrimitiveComponent Object Reference") (OtherBodyIndex :type Integer) (bFromSweep :type Boolean) (SweepResult :type "HitResult Structure (by ref)"))
  (cast `/Game/BP/BP_PLayer1` OtherActor)
  (`/Engine/EditorBlueprintResources/StandardMacros.DoOnce` false
    (:`Completed`
      (`self.Hit`))))

(event `Hit`
  (`self.K2_DestroyActor` (`self.Homingtarget`))
  (`self.K2_DestroyActor`))

(fn `UserConstructionScript`)