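; Player character for a mouse-aimed shooter that toggles between two camera planes with Tab, pitching the camera 90° during slow motion.
; Movement is camera-relative, using LaunchCharacter for vertical motion in XView, while a looping timer rotates the player toward the cursor.
; Held left mouse fires spread volleys with recoil; Space performs a blink dash that carries leftover distance through BP_Portal via repeated traces.
; Number keys spawn enemies and a bounce ball.
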(event `InputAxis|MovementForward`
  (params (AxisValue :type "Float (single-precision)"))
  (bind _charactermovement (`self.CharacterMovement`))
  (bind _maxwalkspeed (`CharacterMovementComponent.MaxWalkSpeed` (`self.CharacterMovement`)))
  (bind (_velocity_x _velocity_y _velocity_z) (`KismetMathLibrary.BreakVector` (`MovementComponent.Velocity` _charactermovement)))
  (bind (_velocity_x_2 _velocity_y_2 _velocity_z_2) (`KismetMathLibrary.BreakVector` (`MovementComponent.Velocity` (`self.CharacterMovement`))))
  (bind _returnvalue (`SceneComponent.GetUpVector` (`/Game/BP/BP_Camera.Camera` (`self.CurrentCamera`))))
  (bind _returnvalue_2 (/ _maxwalkspeed 50.0))
  (bind _returnvalue_3 (* (`KismetMathLibrary.SignOfFloat` _velocity_z_2) -1.0))
  ;[0.4828 1 0.5202] 移动
  (if (`self.XView?`)
    (if (> (`KismetMathLibrary.Abs` AxisValue) 0.01)
      ;;[1 1 1] 竖着移动的方式
      (`self.LaunchCharacter` (* (* _returnvalue AxisValue) 10.0))
      (`|ExecutionSequence`
        (:`then_0`
          (`KismetSystemLibrary.RetriggerableDelay` 0.02 :!label _label)
          (`self.LaunchCharacter` (`KismetMathLibrary.MakeVector` 0.0 0.0 (* _returnvalue_2 _returnvalue_3)))
          (if (<= (`KismetMathLibrary.Abs` _velocity_z) _returnvalue_2)
            (set `MovementComponent.Velocity` (`KismetMathLibrary.MakeVector` _velocity_x _velocity_y) _charactermovement)
            (else
              (goto _label))))
        (:`then_1`
          ;;;[1 1 1] 最大速度限制
          (if (> (`KismetMathLibrary.Abs` _velocity_z_2) _maxwalkspeed) :!label _label_2
            (`self.LaunchCharacter` (`KismetMathLibrary.MakeVector` 0.0 0.0 (* _returnvalue_3 (`KismetMathLibrary.Lerp` 100.0 1.0 (/ _maxwalkspeed _velocity_z_2)))))
            (`KismetSystemLibrary.PrintString` (`KismetStringLibrary.Conv_DoubleToString` _velocity_z)))))
      (else
        (goto _label_2)))
    (else
      (`self.AddMovementInput` _returnvalue AxisValue))))

(event `Key|Tab`
  (params (Key :type "Key Structure"))
  (bind _originalrotation (`self.OriginalRotation`))
  (:`Pressed`
    (`GameplayStatics.SetGlobalTimeDilation` 0.1)
    (set `self.CustomTimeDilation` 0.2)
    (set `self.SwitchTime` (`KismetSystemLibrary.GetGameTimeInSeconds`))
    (set `self.PlayerRotationBeforeSwitch` (`Controller.GetControlRotation` (`GameplayStatics.GetPlayerController` 0)))
    (`/Engine/EditorBlueprintResources/StandardMacros.FlipFlop`
      (:`A`
        (set `self.XView?` true)
        (bind (_direction `_新建轨道_0`) (`Timeline|时间轴_0` :!via `PlayFromStart` :!label _label_3)
          (:`Update`
            (`self.K2_SetActorRotation` (`self.camera`) (`KismetMathLibrary.RLerp` _originalrotation (`KismetMathLibrary.MakeRotator` (.roll _originalrotation) (+ (.pitch _originalrotation) 90.0) (.yaw _originalrotation)) `_新建轨道_0` true) false))
          (:`Finished`
            (`GameplayStatics.SetGlobalTimeDilation` 1.0)
            (set `self.CustomTimeDilation` 1.0))))
      (:`B`
        (set `self.XView?` false)
        (goto _label_3 :!via `ReverseFromEnd`)))))

(event `InputAxis|MovementSide`
  (params (AxisValue :type "Float (single-precision)"))
  ;[0.4828 1 0.5202] 移动
  (`self.AddMovementInput` (`SceneComponent.GetRightVector` (`/Game/BP/BP_Camera.Camera` (`self.CurrentCamera`))) AxisValue))

(event `self.ReceiveBeginPlay`
  (bind _returnvalue (`GameplayStatics.GetPlayerController` 0))
  (bind _output_get (set `self.CurrentCamera` (`self.camera`)))
  (`PlayerController.SetViewTargetWithBlend` (`GameplayStatics.GetPlayerController` 0) _output_get 0.0 "VTBlend_Linear" 0.0 false)
  (set `PlayerController.bShowMouseCursor` true _returnvalue)
  (`self.EnableInput` _returnvalue)
  (`WidgetBlueprintLibrary.SetInputMode_GameAndUIEx` _returnvalue null "LockAlways" false)
  (set `self.Initial Launch` (`SceneComponent.RelativeLocation` (`self.LaunchPoint`)))
  (`KismetSystemLibrary.K2_SetTimer` null "RotationtoCursor" 0.01 true)
  (set `self.Initial Location` (`self.K2_GetActorLocation`))
  (set `self.OriginalRotation` (`self.K2_GetActorRotation` (`self.camera`))))

(event `Key|LeftMouseButton`
  (params (Key :type "Key Structure"))
  (:`Pressed`
    (set `self.Aiming` true))
  (:`Released`
    (set `self.Aiming` false)))

(event `Key|One`
  (params (Key :type "Key Structure"))
  (bind (_returnvalue_x _returnvalue_y _returnvalue_z) (`KismetMathLibrary.BreakVector` (`self.K2_GetActorLocation`)))
  ;[1 1 1] 敌人生成
  (:`Pressed`
    (bind _returnvalue (`|SpawnActorFromClass` "/Game/BP/BP_Enemy_Missile.BP_Enemy_Missile_C" (`KismetMathLibrary.MakeTransform` (`KismetMathLibrary.MakeVector` 0.0 0.0 _returnvalue_z) (struct) (0.7 0.7 0.7)) "AlwaysSpawn" "MultiplyWithRoot" null null))
    (`/Game/BP/BP_EnemyMaster.SpawnIn` _returnvalue)))

(event `Key|Four`
  (params (Key :type "Key Structure"))
  ;[1 1 1] 敌人生成
  (:`Pressed`
    (`|SpawnActorFromClass` "/Game/BP/BP_BounceBall.BP_BounceBall_C" (`self.GetTransform`) "AdjustIfPossibleButAlwaysSpawn" "MultiplyWithRoot" null null)))

(event `self.ReceiveTick`
  (params (DeltaSeconds :type "Float (single-precision)"))
  (bind _initial_launch (`self.Initial Launch`))
  (bind _maxbulletgap (`self.MaxBulletGap`))
  (bind _launchpoint (`self.LaunchPoint`))
  ;[1 0 0] 开火
  (`|ExecutionSequence`
    (:`then_0`
      (`KismetSystemLibrary.Delay` 0.01))
    (:`then_1`
      (if (`self.Aiming`)
        (`/Engine/EditorBlueprintResources/StandardMacros.DoOnce` false :!label _label_4
          (:`Completed`
            (`self.LaunchCharacter` (* (`self.GetActorForwardVector`) -6.0))
            (bind _counter (`/Engine/EditorBlueprintResources/StandardMacros.Do N` (`self.Bullets`) :!label _label_5)
              (:`Exit`
                (bind _returnvalue (* (* (* (/ 1.0 (`KismetMathLibrary.Conv_IntToDouble` (`self.Bullets`))) 1.0) _maxbulletgap) (`KismetMathLibrary.Round` (/ (`KismetMathLibrary.Conv_IntToDouble` _counter) 2.0))))
                (`SceneComponent.K2_SetRelativeLocation` _launchpoint (select `bool` (and (> (mod (`self.Bullets`) 2) 0) (== _counter (`self.Bullets`))) :`false` (select `bool` (> (mod _counter 2) 0) :`false` (- (+ _initial_launch _maxbulletgap) _returnvalue) :`true` (+ (- _initial_launch _maxbulletgap) _returnvalue)) :`true` (`self.Initial Launch`)) false false)
                (bind _returnvalue_2 (`|SpawnActorFromClass` "/Game/BP/BP_Projectile.BP_Projectile_C" (`SceneComponent.K2_GetComponentToWorld` _launchpoint) "Undefined" "MultiplyWithRoot" null null))
                (if (== (`KismetMathLibrary.FindLookAtRotation` (`KismetMathLibrary.MakeVector` 0.0) (`self.GetVelocity`)) (`SceneComponent.K2_GetComponentRotation` _launchpoint) :`ErrorTolerance` 60.0)
                  _
                  (else
                    _))
                (if (>= _counter (`self.Bullets`))
                  (`GameplayStatics.SpawnSound2D` "/Game/Sound/Plasmafire.Plasmafire" 0.2 1.0 0.0 null)
                  (`KismetSystemLibrary.Delay` 0.15)
                  (`self.ResetFire`)
                  (else
                    (goto _label_5)))))))))))

(event `ResetFire`
  ;[1 0 0] 开火
  (`|ExecutionSequence`
    (:`then_0`
      (goto _label_4 :!via `Reset`))
    (:`then_1`
      (goto _label_5 :!via `Reset`))))

(event `Key|Two`
  (params (Key :type "Key Structure"))
  (bind (_returnvalue_x _returnvalue_y _returnvalue_z) (`KismetMathLibrary.BreakVector` (`self.K2_GetActorLocation`)))
  ;[1 1 1] 敌人生成
  (:`Pressed`
    (bind _returnvalue (`|SpawnActorFromClass` "/Game/BP/BP_Enemy_Assault.BP_Enemy_Assault_C" (`KismetMathLibrary.MakeTransform` (`KismetMathLibrary.MakeVector` 0.0 0.0 _returnvalue_z) (struct) (0.7 0.7 0.7)) "AlwaysSpawn" "MultiplyWithRoot" null null))
    (`/Game/BP/BP_EnemyMaster.SpawnIn` _returnvalue)))

(event `Key|Three`
  (params (Key :type "Key Structure"))
  (bind (_returnvalue_x _returnvalue_y _returnvalue_z) (`KismetMathLibrary.BreakVector` (`self.K2_GetActorLocation`)))
  ;[1 1 1] 敌人生成
  (:`Pressed`
    (bind _returnvalue (`|SpawnActorFromClass` "/Game/BP/BP_Enemy_Boss.BP_Enemy_Boss_C" (`KismetMathLibrary.MakeTransform` (`KismetMathLibrary.MakeVector` 0.0 0.0 _returnvalue_z) (struct) (1.5 1.5 1.5)) "AlwaysSpawn" "MultiplyWithRoot" null null))
    (`/Game/BP/BP_EnemyMaster.SpawnIn` _returnvalue)))

(event `Key|SpaceBar`
  (params (Key :type "Key Structure"))
  ;[1 1 1] Dash
  (:`Pressed`
    (`/Engine/EditorBlueprintResources/StandardMacros.DoOnce` false :!label _label_6
      (:`Completed`
        (`self.DashProgress`)
        (`KismetSystemLibrary.Delay` 0.2)
        (`NiagaraFunctionLibrary.SpawnSystemAtLocation` "/Game/VFX/BlinkAndDashVFX/VFX_Niagara/NS_Blink_Psionic.NS_Blink_Psionic" (`self.K2_GetActorLocation`) (`self.K2_GetActorRotation`))
        (set `MovementComponent.Velocity` (`self.VelocityBeforeDash`) (`self.CharacterMovement`))
        (`self.SetActorHiddenInGame` false)
        (`self.SetActorEnableCollision` true)
        (`KismetSystemLibrary.Delay` 0.5)
        (`self.Reset Dash`)))))

(event `Reset Dash`
  ;[1 1 1] Dash
  (goto _label_6 :!via `Reset`))

(fn `DashDirection`
  (returns (ReturnValue :type "Vector Structure"))
  (bind _returnvalue (`self.GetInputAxisValue`))
  (bind _returnvalue_2 (`self.GetInputAxisValue`))
  (bind _camera (`/Game/BP/BP_Camera.Camera` (`self.CurrentCamera`)))
  (return (select `bool` (or (!= _returnvalue 0.0) (!= _returnvalue_2 0.0)) :`false` (`self.GetActorForwardVector`) :`true` (+ (* _returnvalue (`SceneComponent.GetUpVector` _camera)) (* (`SceneComponent.GetRightVector` _camera) _returnvalue_2)))))

(fn `DashProgress`
  (locals (DashDisplacement :type "Vector Structure") (RemainingDistance :type "Float (double-precision)"))
  (bind _returnvalue (`self.DashDirection`))
  (bind _charactermovement (`self.CharacterMovement`))
  (bind _returnvalue_2 (+ (`self.K2_GetActorLocation`) (* _returnvalue (`local.RemainingDistance`))))
  (`NiagaraFunctionLibrary.SpawnSystemAtLocation` "/Game/VFX/BlinkAndDashVFX/VFX_Niagara/NS_Blink_Psionic.NS_Blink_Psionic" (`self.K2_GetActorLocation`) (`self.K2_GetActorRotation`))
  (`self.SetActorHiddenInGame` true)
  (`self.SetActorEnableCollision` false)
  (set `self.VelocityBeforeDash` (`MovementComponent.Velocity` _charactermovement))
  (`MovementComponent.StopMovementImmediately` _charactermovement)
  (set `local.RemainingDistance` (`self.Dash Distance`))
  (bind _outhit (`KismetSystemLibrary.LineTraceSingleForObjects` (`self.K2_GetActorLocation`) _returnvalue_2 (`|MakeArray` "ObjectTypeQuery5" :!type "EObjectTypeQuery Enum") :!label _label))
  (set `local.DashDisplacement` _returnvalue_2)
  (bind (_bblockinghit _binitialoverlap _time _distance _location _impactpoint _normal _impactnormal _physmat _hitactor) (`GameplayStatics.BreakHitResult` _outhit))
  (bind _asbp_portal (cast `/Game/BP/BP_Portal` _hitactor)
    (:`then`
      (set `/Game/BP/BP_Portal.OverlappedActor` self _asbp_portal)
      (`/Game/BP/BP_Portal.ManualTP` _asbp_portal)
      (set `local.DashDisplacement` (- (`local.DashDisplacement`) (* _distance _returnvalue)))
      (set `local.RemainingDistance` (- (`self.Dash Distance`) _distance))
      (goto _label))
    (:`CastFailed`
      (`self.K2_SetActorLocation` (`local.DashDisplacement`))
      (return))))

(fn `RotationtoCursor`
  (bind _returnvalue (`self.K2_GetActorLocation`))
  (bind _worldlocation (`PlayerController.DeprojectMousePositionToWorld` (`GameplayStatics.GetPlayerController` 0)))
  (bind _pitch (.pitch (`KismetMathLibrary.FindLookAtRotation` _returnvalue (select `bool` (`self.XView?`) :`false` (`KismetMathLibrary.MakeVector` (.x _worldlocation) (.y _worldlocation) (.z _returnvalue)) :`true` (`KismetMathLibrary.MakeVector` (.x _returnvalue) (.y _worldlocation) (.z _worldlocation))))))
  (bind _yaw (.yaw (`KismetMathLibrary.FindLookAtRotation` _returnvalue (select `bool` (`self.XView?`) :`false` (`KismetMathLibrary.MakeVector` (.x _worldlocation) (.y _worldlocation) (.z _returnvalue)) :`true` (`KismetMathLibrary.MakeVector` (.x _returnvalue) (.y _worldlocation) (.z _worldlocation))))))
  (bind _returnvalue_2 (`KismetMathLibrary.SelectRotator` (`KismetMathLibrary.MakeRotator` 90.0 _pitch _yaw) (`KismetMathLibrary.MakeRotator` (.roll (`KismetMathLibrary.FindLookAtRotation` _returnvalue (select `bool` (`self.XView?`) :`false` (`KismetMathLibrary.MakeVector` (.x _worldlocation) (.y _worldlocation) (.z _returnvalue)) :`true` (`KismetMathLibrary.MakeVector` (.x _returnvalue) (.y _worldlocation) (.z _worldlocation))))) _pitch _yaw) (`self.XView?`)))
  (if (not (<= (- (`KismetSystemLibrary.GetGameTimeInSeconds`) (`self.SwitchTime`)) 0.1))
    (`Controller.SetControlRotation` (`GameplayStatics.GetPlayerController` 0) _returnvalue_2)
    (`self.K2_SetActorRotation` _returnvalue_2)))

(fn `UserConstructionScript`)