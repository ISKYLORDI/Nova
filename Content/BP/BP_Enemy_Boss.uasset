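; Boss enemy that emerges from a portal away from the player, spins constantly and moves by homing projectile movement.
; Phase 0 wanders between trace-validated random homing targets; a delay after spawn triggers Phase 1, a high-speed dash across the camera's sides before wandering resumes.
; Damage registers only while a projectile overlap on Sphere2 flags a core hit.
; Death spawns a collectible and Niagara burst, then scales up and fades out.
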(event `self.ReceiveBeginPlay`
  (set `self.Scale` (`self.GetActorScale3D`))
  (bind _returnvalue (`KismetSystemLibrary.K2_SetTimer` null "RotationtoPlayer" 0.01 true))
  (set `self.RotationHandle` _returnvalue))

(event `self.Death`
  (bind _homingtarget (`self.HomingTarget`))
  (bind _scale (`self.Scale`))
  (`parent.Death`)
  (`self.SpawnCollectible`)
  (`self.SetActorEnableCollision` false)
  (`NiagaraFunctionLibrary.SpawnSystemAtLocation` "/Game/VFX/BlinkAndDashVFX/VFX_Niagara/NS_Blink_Fire.NS_Blink_Fire" (`self.K2_GetActorLocation`) (struct) (0.5 0.5 0.5))
  (bind (_direction `_新建轨道_0`) (`Timeline|时间轴`)
    (:`Update`
      (`self.SetActorScale3D` (`KismetMathLibrary.VLerp` _scale (* _scale 3.0) `_新建轨道_0`))
      (`MeshComponent.SetScalarParameterValueOnMaterials` (`self.Sphere`) "Opacity" (`KismetMathLibrary.Lerp` 1.0 0.0 `_新建轨道_0`))
      (`MeshComponent.SetScalarParameterValueOnMaterials` (`self.Sphere1`) "Opacity" (`KismetMathLibrary.Lerp` 1.0 0.0 `_新建轨道_0`))
      (`MeshComponent.SetScalarParameterValueOnMaterials` (`self.Sphere2`) "Opacity" (`KismetMathLibrary.Lerp` 1.0 0.0 `_新建轨道_0`)))
    (:`Finished`
      (`/Engine/EditorBlueprintResources/StandardMacros.IsValid` _homingtarget
        (:`Is Valid`
          (`self.K2_DestroyActor` _homingtarget)
          (`self.K2_DestroyActor`))))))

(event `self.ReceiveAnyDamage`
  (params (Damage :type "Float (single-precision)") (DamageType :type "DamageType Object Reference") (InstigatedBy :type "Controller Object Reference") (DamageCauser :type "Actor Object Reference"))
  (if (`self.CoreHit`)
    (`parent.ReceiveAnyDamage` Damage DamageType InstigatedBy DamageCauser)))

(event `self.Sphere2.OnComponentBeginOverlap`
  (params (OverlappedComponent :type "PrimitiveComponent Object Reference") (OtherActor :type "Actor Object Reference") (OtherComp :type "PrimitiveComponent Object Reference") (OtherBodyIndex :type Integer) (bFromSweep :type Boolean) (SweepResult :type "HitResult Structure (by ref)"))
  (cast `/Game/BP/BP_Projectile` OtherActor)
  (set `self.CoreHit` true)
  (`GameplayStatics.ApplyDamage` self 0.1 null self)
  (`KismetSystemLibrary.RetriggerableDelay` 0.1)
  (set `self.CoreHit` false))

(event `self.SpawnIn`
  (bind (_returnvalue_roll _returnvalue_pitch _returnvalue_yaw) (`KismetMathLibrary.BreakRotator` (`KismetMathLibrary.RandomRotator` false)))
  (bind _returnvalue (`self.K2_GetActorLocation` (`GameplayStatics.GetPlayerCharacter` 0)))
  (bind _returnvalue_2 (+ (`self.SpawnHitLocation`) (* (`KismetMathLibrary.GetForwardVector` (`self.SpawnRotation`)) 100.0)))
  (set `self.SpawnRotation` (`KismetMathLibrary.MakeRotator` 0.0 0.0 _returnvalue_yaw) :!label _label)
  (bind _outhit (`KismetSystemLibrary.LineTraceSingleForObjects` _returnvalue (+ _returnvalue (* (`KismetMathLibrary.GetForwardVector` (`self.SpawnRotation`)) 3000.0)) (`|MakeArray` "ObjectTypeQuery5" :!type "EObjectTypeQuery Enum") true (`|MakeArray` self :!type "Actor Object Reference")))
  (bind (_bblockinghit _binitialoverlap _time _distance _location _impactpoint _normal _impactnormal _physmat _hitactor) (`GameplayStatics.BreakHitResult` _outhit))
  (cast `/Game/BP/BP_Portal` _hitactor)
  (if (<= _distance 1000.0)
    (goto _label)
    (else
      (set `self.SpawnHitLocation` _location)
      (`self.K2_SetActorLocation` _returnvalue_2)
      (`self.K2_SetActorRotation` (`KismetMathLibrary.FindLookAtRotation` _returnvalue_2 (`self.K2_GetActorLocation` (`GameplayStatics.GetPlayerCharacter` 0))))
      (`self.StartPush` (`KismetMathLibrary.GetDirectionUnitVector` _returnvalue_2 (`self.SpawnHitLocation`)) 10.0)
      (`|ExecutionSequence`
        (:`then_0`
          (`KismetSystemLibrary.Delay` 5.0)
          (set `self.Phase` 1))
        (:`then_1`
          (goto _label_2 :!via `Close`))))))

(event `StartRotation`
  (`/Engine/EditorBlueprintResources/StandardMacros.Gate` false :!label _label_2
    (:`Exit`
      (`self.StartPush` (0.0 0.0 0.0) 0.0))))

(event `Dash Through`
  (bind _homingtarget (`self.HomingTarget`))
  (`/Engine/EditorBlueprintResources/StandardMacros.DoOnce` false :!label _label_3
    (:`Completed`
      (bind _asbp_player_1 (cast `/Game/BP/BP_PLayer1` (`GameplayStatics.GetPlayerCharacter` 0)))
      (bind _camera (`/Game/BP/BP_PLayer1.camera` _asbp_player_1))
      (bind _output_get (set `self.DistancefromCenter` (* (`self.GetActorRightVector` _camera) (`KismetMathLibrary.SelectFloat` 800.0 -800.0 (`KismetMathLibrary.RandomBool`)))))
      (`/Engine/EditorBlueprintResources/StandardMacros.IsValid` _homingtarget
        (:`Is Valid`
          (bind (_returnvalue_x _returnvalue_y) (`KismetMathLibrary.BreakVector` (`self.K2_GetActorLocation` _camera)))
          (bind (_returnvalue_x_2 _returnvalue_y_2 _returnvalue_z) (`KismetMathLibrary.BreakVector` (`self.K2_GetActorLocation` _asbp_player_1)))
          (`self.K2_SetActorLocation` _homingtarget (+ _output_get (`KismetMathLibrary.MakeVector` _returnvalue_x _returnvalue_y _returnvalue_z)) false false))))))

(event `ResetDash`
  (goto _label_3 :!via `Reset`))

(event `self.StartPush`
  (params (PushDirection :type "Vector Structure") (`Push Force` :type "Float (double-precision)"))
  (bind (_returnvalue_x _returnvalue_y _returnvalue_z) (`KismetMathLibrary.BreakVector` (`self.K2_GetActorLocation`)))
  (bind _array (`|MakeArray` "ObjectTypeQuery5" :!type "EObjectTypeQuery Enum"))
  (bind _homingtarget (`self.HomingTarget`))
  (bind _x (.x (`self.RandomPoint`)))
  (bind _y (.y (`self.RandomPoint`)))
  (`parent.StartPush` PushDirection `Push Force`)
  (`KismetSystemLibrary.RetriggerableDelay` 2.0 :!label _label_4)
  (switch `int` (`self.Phase`)
    (:`0`
      (set `ProjectileMovementComponent.bSimulationEnabled` true (`self.ProjectileMovement`) :!label _label_5)
      (bind _output_get (set `self.RandomPoint` (`KismetMathLibrary.RandomPointInBoundingBox` (`self.K2_GetActorLocation`) (`KismetMathLibrary.MakeVector` 3000.0 3000.0 3000.0))))
      (if (>= (`KismetMathLibrary.Vector_Distance` _output_get (`self.K2_GetActorLocation` (`GameplayStatics.GetPlayerCharacter` 0))) 500.0)
        (bind (_outhit _returnvalue) (`KismetSystemLibrary.SphereTraceSingleForObjects` :`Start` _output_get :`End` _output_get :`Radius` 500.0 :`ObjectTypes` _array :`bTraceComplex` true :`DrawTime` 1.0))
        (bind (_outhit_2 _returnvalue_2) (`KismetSystemLibrary.LineTraceSingleForObjects` (`self.K2_GetActorLocation` (`GameplayStatics.GetPlayerCharacter` 0)) (`self.RandomPoint`) _array true))
        (if (or _returnvalue_2 _returnvalue)
          (goto _label_5)
          (else
            (`/Engine/EditorBlueprintResources/StandardMacros.IsValid` _homingtarget
              (:`Is Valid`
                (`self.K2_SetActorLocation` _homingtarget (`KismetMathLibrary.MakeVector` _x _y _returnvalue_z) false false))
              (:`Is Not Valid`
                (bind _returnvalue_3 (`|SpawnActorFromClass` "/Game/BP/BP_HomingTarget.BP_HomingTarget_C" (`KismetMathLibrary.MakeTransform` (`KismetMathLibrary.MakeVector` _x _y _returnvalue_z)) "Undefined" "MultiplyWithRoot" null null))
                (bind _output_get_2 (set `self.HomingTarget` _returnvalue_3))))
            (set `ProjectileMovementComponent.HomingTargetComponent` (`/Game/BP/BP_HomingTarget.Sphere` _output_get_2) (`self.ProjectileMovement`))
            (goto _label_4)))
        (else
          (goto _label_5))))))

(event `self.ReceiveTick`
  (params (DeltaSeconds :type "Float (single-precision)"))
  (bind _homingtarget (`self.HomingTarget`))
  (bind _homingtarget_2 (`self.HomingTarget`))
  (bind _projectilemovement (`self.ProjectileMovement`))
  (switch `int` (`self.Phase`)
    (:`1`
      (`self.Dash Through`)
      (`/Engine/EditorBlueprintResources/StandardMacros.IsValid` _homingtarget
        (:`Is Valid`
          (if (<= (`KismetMathLibrary.Vector_Distance` (`self.K2_GetActorLocation`) (`self.K2_GetActorLocation` _homingtarget)) 50.0)
            (`|ExecutionSequence`
              (:`then_0`
                (`/Engine/EditorBlueprintResources/StandardMacros.Gate` false :!label _label_6
                  (:`Exit`
                    (`self.K2_SetActorLocation` _homingtarget_2 (- (`self.K2_GetActorLocation` _homingtarget_2) (* (`self.DistancefromCenter`) 2.0)) false false)
                    (set `ProjectileMovementComponent.MaxSpeed` (* (`ProjectileMovementComponent.MaxSpeed` _projectilemovement) 20.0) _projectilemovement)
                    (set `ProjectileMovementComponent.HomingAccelerationMagnitude` (* (`ProjectileMovementComponent.HomingAccelerationMagnitude` _projectilemovement) 50.0) _projectilemovement)
                    (`|ExecutionSequence`
                      (:`then_0`
                        (goto _label_6 :!via `Close`))
                      (:`then_1`
                        (`KismetSystemLibrary.Delay` 0.1)
                        (goto _label_7 :!via `Open`))))))
              (:`then_1`
                (`/Engine/EditorBlueprintResources/StandardMacros.Gate` true :!label _label_7
                  (:`Exit`
                    (`KismetSystemLibrary.PrintString` "Hello")
                    (set `self.Phase` 0)
                    (set `ProjectileMovementComponent.MaxSpeed` (* (`ProjectileMovementComponent.MaxSpeed` _projectilemovement) 0.05) _projectilemovement)
                    (set `ProjectileMovementComponent.HomingAccelerationMagnitude` (* (`ProjectileMovementComponent.HomingAccelerationMagnitude` _projectilemovement) 0.02) _projectilemovement)
                    (`self.ChooseRandomTarget`)
                    (`|ExecutionSequence`
                      (:`then_0`
                        (goto _label_6 :!via `Open`))
                      (:`then_1`
                        (goto _label_7 :!via `Close`)))))))))))))

(event `ChooseRandomTarget`
  (goto _label_5))

(fn `RotationtoPlayer`
  (`self.K2_AddActorWorldRotation` (`KismetMathLibrary.MakeRotator` 0.0 0.0 (`self.RotationSpeed`))))

(fn `UserConstructionScript`
  (`parent.UserConstructionScript`))