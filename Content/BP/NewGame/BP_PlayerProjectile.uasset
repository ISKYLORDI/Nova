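; Player fireball for the grid-based game that takes size, damage, stun, pushback and fire settings from GridPlayerController or SpawnEvent.
; It hovers on a spawned BP_HomingTarget until TargetSet moves that target, then homes in or, in Low mode, flies straight.
; Overlap or proximity triggers impact: big shots spawn BP_Shockwave, small ones apply damage, pushback, stun and burning ground.
; ChainSpawn launches a follow-up low projectile on impact.
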(event `TargetSet`
  (params (NewLocation :type "Vector Structure"))
  (bind _returnvalue_x (`KismetMathLibrary.BreakVector` (`self.GetActorScale3D`)))
  (bind _homingactor (`self.HomingActor`))
  (bind _projectilemovement (`self.ProjectileMovement`))
  (bind _projectilemovement_2 (`self.ProjectileMovement`))
  (bind _returnvalue (> _returnvalue_x 2.0))
  (`self.SetLifeSpan` 5.0)
  (`self.K2_DetachFromActor` _homingactor "KeepWorld" "KeepWorld" "KeepWorld")
  (`self.K2_SetActorLocation` _homingactor NewLocation false false)
  (set `self.Launched` true)
  (if (`self.Low`)
    (bind _returnvalue_2 (`GameplayStatics.SpawnEmitterAttached` "/Game/VFX/MagicProjectilesVol2/Particles/Projectiles/P_Projectile_Trail02_Red.P_Projectile_Trail02_Red" (`self.Sphere`) "None" (0.0 0.0 0.0) (struct) (1.0 1.0 1.0) "SnapToTargetIncludingScale"))
    (set `self.Trail` _returnvalue_2)
    (set `ProjectileMovementComponent.bIsHomingProjectile` false _projectilemovement)
    (set `ProjectileMovementComponent.MaxSpeed` 2000.0 _projectilemovement)
    (set `MovementComponent.Velocity` (* (`KismetMathLibrary.GetDirectionUnitVector` (`self.K2_GetActorLocation` (`/Game/BP/NewGame/GridPlayerController.BPPlayer` (`self.Controller`))) (`self.K2_GetActorLocation` (`self.HomingActor`))) 10000.0) (`self.ProjectileMovement`))
    (else
      (set `ProjectileMovementComponent.HomingAccelerationMagnitude` 5000.0 _projectilemovement_2)
      (set `ProjectileMovementComponent.MaxSpeed` (select `bool` _returnvalue :`false` 2000.0 :`true` 4000.0 :!type "Float (single-precision)") _projectilemovement_2)))
  (`self.SetActorEnableCollision` true)
  (`GameplayStatics.PlaySound2D` (select `bool` (`self.Low`) :`false` (select `bool` _returnvalue :`false` "/Game/Sound/SFX/Skills/Fireball/S_Tiny_Fireball_02.S_Tiny_Fireball_02" :`true` "/Game/Sound/SFX/Skills/Fireball/S_Huge_Fireball_Clash.S_Huge_Fireball_Clash" :!type "SoundBase Object Reference") :`true` "/Engine/EditorSounds/GamePreview/PossessPlayer.PossessPlayer") 0.6 1.0 0.0 null null))

(event `self.ReceiveBeginPlay`
  (bind _projectilemovement (`self.ProjectileMovement`))
  (bind _controller (`self.Controller`))
  (bind _big (`self.Big`))
  (bind _asgrid_player_controller (cast `/Game/BP/NewGame/GridPlayerController` (`GameplayStatics.GetPlayerController` 0)))
  (set `self.Controller` _asgrid_player_controller)
  (set `self.Big` (`.>0` (`/Game/BP/NewGame/GridPlayerController.Number` _controller "NewEnumerator5")))
  (set `self.Stun` (`.>0` (`/Game/BP/NewGame/GridPlayerController.Number` _controller "NewEnumerator3")))
  (set `self.Force` (`KismetMathLibrary.Conv_IntToDouble` (`/Game/BP/NewGame/GridPlayerController.Number` _controller "NewEnumerator7")))
  (set `self.Power` (`/Game/BP/NewGame/GridPlayerController.Power` _controller))
  (set `self.Fire` (`.>0` (`/Game/BP/NewGame/GridPlayerController.Number` _controller "NewEnumerator6")))
  (set `self.Range` (`/Game/BP/NewGame/GridPlayerController.Range` _controller))
  (set `self.Damage` (select `bool` _big :`false` 1.0 :`true` 2.0))
  (`self.SetActorScale3D` (select `bool` _big :`false` (1.0 1.0 1.0) :`true` (3.0 3.0 3.0) :!type "Vector Structure") :!label _label)
  (`SceneComponent.SetWorldScale3D` (`self.Sphere`) (`KismetMathLibrary.Conv_DoubleToVector` 0.2))
  (`self.SetActorEnableCollision` false)
  (bind _output_get (set `self.Initial Scale` (`self.GetActorScale3D`)))
  (set `ProjectileMovementComponent.HomingAccelerationMagnitude` (* (.x _output_get) 300.0) _projectilemovement)
  (set `MovementComponent.Velocity` (* (`MovementComponent.Velocity` _projectilemovement) (.x _output_get)) _projectilemovement)
  (`LightComponent.SetIntensity` (`self.PointLight`) (* (.x _output_get) 7000.0))
  (`TimelineComponent.SetPlayRate` (`self.时间轴`) (/ 1.0 (.x _output_get)))
  (bind (_direction `_新建轨道_0`) (`Timeline|时间轴` :!via `PlayFromStart`)
    (:`Update`
      (`self.SetActorScale3D` (`KismetMathLibrary.VLerp` (0.0 0.0 0.0) (`self.Initial Scale`) `_新建轨道_0`)))))

(event `Launch`
  (bind _returnvalue (`|SpawnActorFromClass` "/Game/BP/Nova/BP_HomingTarget.BP_HomingTarget_C" (`KismetMathLibrary.MakeTransform` (+ (`SceneComponent.K2_GetComponentLocation` (`/Game/BP/NewGame/BP_GridBased_Player.Projectille` (`/Game/BP/NewGame/GridPlayerController.BPPlayer` (`self.Controller`)))) (`KismetMathLibrary.MakeVector` (`KismetMathLibrary.RandomFloatInRange` -20.0 20.0) (`KismetMathLibrary.RandomFloatInRange` -20.0 20.0) (`KismetMathLibrary.SelectFloat` 400.0 100.0 (`self.Big`))))) "Undefined" "MultiplyWithRoot" null null))
  (bind _output_get (set `self.HomingActor` _returnvalue))
  (set `ProjectileMovementComponent.HomingTargetComponent` (`Actor.RootComponent` _output_get) (`self.ProjectileMovement`))
  (set `self.Low` false)
  (`self.K2_AttachToActor` _returnvalue (`/Game/BP/NewGame/GridPlayerController.BPPlayer` (`self.Controller`)) "None" "KeepWorld" "KeepWorld" "KeepWorld" true)
  (bind _returnvalue_2 (`GameplayStatics.SpawnEmitterAttached` (select `bool` (`self.Big`) :`false` "/Game/VFX/MagicProjectilesVol2/Particles/Projectiles/P_Projectile_Fireball05_Orange.P_Projectile_Fireball05_Orange" :`true` "/Game/VFX/MagicProjectilesVol2/Particles/Projectiles/P_Projectile_Fireball04_Orange.P_Projectile_Fireball04_Orange" :!type "ParticleSystem Object Reference") (`self.ParticleSystem`) "None" (0.0 0.0 0.0) (struct) (1.0 1.0 1.0) "SnapToTargetIncludingScale"))
  (set `self.Emitter` _returnvalue_2))

(event `SpawnEvent`
  (params (Big :type Boolean) (Stun :type Boolean) (Force :type "Float (double-precision)") (Power :type "Float (double-precision)") (Fire :type Boolean) (Range :type "Float (double-precision)") (Damage :type "Float (double-precision)"))
  (set `self.Big` Big)
  (set `self.Stun` Stun)
  (set `self.Force` Force)
  (set `self.Power` Power)
  (set `self.Fire` Fire)
  (set `self.Range` Range)
  (set `self.Damage` Damage)
  (goto _label))

(event `LaunchLow`
  (bind _projectilemovement (`self.ProjectileMovement`))
  (bind _returnvalue (`|SpawnActorFromClass` "/Game/BP/Nova/BP_HomingTarget.BP_HomingTarget_C" (`KismetMathLibrary.MakeTransform` (`SceneComponent.K2_GetComponentLocation` (`/Game/BP/NewGame/BP_GridBased_Player.ProjectilleLow` (`/Game/BP/NewGame/GridPlayerController.BPPlayer` (`self.Controller`))))) "Undefined" "MultiplyWithRoot" null null))
  (bind _output_get (set `self.HomingActor` _returnvalue))
  (set `ProjectileMovementComponent.HomingTargetComponent` (`Actor.RootComponent` _output_get) (`self.ProjectileMovement`))
  (`self.K2_AttachToActor` _returnvalue (`/Game/BP/NewGame/GridPlayerController.BPPlayer` (`self.Controller`)) "None" "KeepWorld" "KeepWorld" "KeepWorld" true)
  (set `self.Low` true)
  (set `ProjectileMovementComponent.bIsHomingProjectile` false _projectilemovement)
  (set `ProjectileMovementComponent.MaxSpeed` 0.0 _projectilemovement)
  (`MovementComponent.StopMovementImmediately` _projectilemovement)
  (bind _returnvalue_2 (`GameplayStatics.SpawnEmitterAttached` (select `bool` (`self.Big`) :`false` "/Game/VFX/MagicProjectilesVol2/Particles/Projectiles/P_Projectile_Firefrost01_Orange.P_Projectile_Firefrost01_Orange" :`true` "/Game/VFX/MagicProjectilesVol2/Particles/Projectiles/P_Projectile_Firefrost01_Orange.P_Projectile_Firefrost01_Orange" :!type "ParticleSystem Object Reference") (`self.ParticleSystem`) "None" (0.0 0.0 0.0) (struct) (1.0 1.0 1.0) "SnapToTargetIncludingScale"))
  (set `self.Emitter` _returnvalue_2))

(event `self.Sphere.OnComponentBeginOverlap`
  (params (OverlappedComponent :type "PrimitiveComponent Object Reference") (OtherActor :type "Actor Object Reference") (OtherComp :type "PrimitiveComponent Object Reference") (OtherBodyIndex :type Integer) (bFromSweep :type Boolean) (SweepResult :type "HitResult Structure (by ref)"))
  (bind _returnvalue (`self.K2_GetActorLocation`))
  (bind _returnvalue_2 (`self.K2_GetActorLocation`))
  (bind _returnvalue_3 (`self.K2_GetActorLocation`))
  (bind _homingactor (`self.HomingActor`))
  (bind _projectilemovement (`self.ProjectileMovement`))
  (bind _collidingactor (`self.CollidingActor`))
  (bind _returnvalue_4 (`self.K2_GetActorLocation` (`self.HomingActor`)))
  (bind _returnvalue_5 (* (`KismetMathLibrary.GetDirectionUnitVector` (`self.K2_GetActorLocation` (`/Game/BP/NewGame/GridPlayerController.BPPlayer` (`self.Controller`))) _returnvalue_4) 100.0))
  (bind _returnvalue_6 (+ _returnvalue_4 _returnvalue_5))
  (if (`self.Low`)
    (bind _asbp_grid_based_pawn_enemy (cast `/Game/BP/NewGame/BP_GridBasedPawn_Enemy` OtherActor)
      (:`then`
        (set `self.CollidingEnemy` _asbp_grid_based_pawn_enemy))
      (:`CastFailed`
        (cast `/Game/BP/NewGame/BP_GridedObstacle` OtherActor)))
    (set `self.CollidingActor` OtherActor)
    (`/Engine/EditorBlueprintResources/StandardMacros.DoOnce` false
      (:`Completed`
        (if (`self.Big`)
          (`GameplayStatics.PlaySoundAtLocation` "/Game/Sound/SFX/Skills/Fireball/S_Huge_Fireball_Clash.S_Huge_Fireball_Clash" _returnvalue_3 (struct) 1.0 1.0 0.0 null null null null)
          (`/Engine/EditorBlueprintResources/StandardMacros.DoOnce` false :!label _label_2
            (:`Completed`
              (`/Game/BP/NewGame/GridPlayerController.EliminateBoxes` (`self.Controller`))
              (bind _returnvalue_7 (`|SpawnActorFromClass` "/Game/BP/NewGame/BP_Shockwave.BP_Shockwave_C" (`KismetMathLibrary.MakeTransform` (select `bool` (`self.Low`) :`false` (`self.K2_GetActorLocation` (`self.HomingActor`)) :`true` (select `bool` (`self.IsValid` _collidingactor) :`false` (`self.K2_GetActorLocation`) :`true` (`self.K2_GetActorLocation` _collidingactor)))) "Undefined" "MultiplyWithRoot" self null))
              (`/Game/BP/NewGame/BP_Shockwave.SpawnEvent` _returnvalue_7 (`self.Damage`) 150.0 (`self.Force`) (`self.Fire`) (`self.Stun`) (`self.Power`))
              (`GameplayStatics.SpawnEmitterAtLocation` "/Game/VFX/MagicProjectilesVol2/Particles/Hits/P_Hit_Fireball04_Orange.P_Hit_Fireball04_Orange" _returnvalue (struct :`Roll` 90.0) (* (`self.GetActorScale3D`) 0.5))
              (`NiagaraFunctionLibrary.SpawnSystemAtLocation` "/Game/VFX/BlinkAndDashVFX/VFX_Niagara/NS_Blink_Fire.NS_Blink_Fire" _returnvalue)))
          (else
            (`GameplayStatics.PlaySoundAtLocation` "/Game/Sound/SFX/Skills/Fireball/S_Tiny_Fireball_02.S_Tiny_Fireball_02" _returnvalue_3 (struct) 1.0 1.0 0.0 null null null null)
            (`/Engine/EditorBlueprintResources/StandardMacros.DoOnce` false :!label _label_3
              (:`Completed`
                (`GameplayStatics.SpawnEmitterAtLocation` (select `bool` (`self.Low`) :`false` "/Game/VFX/MagicProjectilesVol2/Particles/Hits/P_Hit_Orb05_Orange.P_Hit_Orb05_Orange" :`true` "/Game/VFX/MagicProjectilesVol2/Particles/Hits/P_Hit_Trail02_Purple.P_Hit_Trail02_Purple" :!type "ParticleSystem Object Reference") _returnvalue_2 (`KismetMathLibrary.FindLookAtRotation` _returnvalue_2 (`self.K2_GetActorLocation` (`/Game/BP/NewGame/GridPlayerController.BPPlayer` (`self.Controller`)))))
                (`self.DamageInRange` 70.0 (`self.Damage`))))))
        (`|ExecutionSequence`
          (:`then_0`
            (`self.SetActorEnableCollision` false :!label _label_4)
            (bind _trail (`self.Trail`)
              (:`then`
                (`ActorComponent.Deactivate` _trail))
              (:`else`
                _))
            (`ActorComponent.Deactivate` (`self.Emitter`))
            (`MovementComponent.StopMovementImmediately` _projectilemovement)
            (set `ProjectileMovementComponent.bIsHomingProjectile` false _projectilemovement)
            (`KismetSystemLibrary.Delay` 0.5)
            (set `self.Intensity` (`LightComponentBase.Intensity` (`self.PointLight`)))
            (bind (_direction `_新建轨道_0`) (`Timeline|时间轴_0` :!via `PlayFromStart`)
              (:`Update`
                (`LightComponent.SetIntensity` (`self.PointLight`) (`KismetMathLibrary.Lerp` (`self.Intensity`) 0.0 `_新建轨道_0`)))
              (:`Finished`
                (`/Engine/EditorBlueprintResources/StandardMacros.IsValid` _homingactor
                  (:`Is Valid`
                    (`self.K2_DestroyActor` _homingactor))
                  (:`Is Not Valid`
                    _))
                (`self.K2_DestroyActor`))))
          (:`then_1`
            (if (`self.ChainSpawn`)
              (bind _returnvalue_8 (`|SpawnActorFromClass` "BP_PlayerProjectile_C" (`KismetMathLibrary.MakeTransform` _returnvalue_6 (struct) (select `bool` (`self.Big`) :`false` (1.0 1.0 1.0) :`true` (3.0 3.0 3.0) :!type "Vector Structure")) "Undefined" "MultiplyWithRoot" null null))
              (`self.SpawnEvent` _returnvalue_8 (`self.Big`) (`self.Stun`) (`self.Force`) (`self.Power`) (`self.Fire`) (`self.Range`) (`self.Damage`))
              (`self.LaunchLow` _returnvalue_8)
              (`self.TargetSet` _returnvalue_8 (+ _returnvalue_6 _returnvalue_5)))))))))

(event `Dissapate`
  (if (not (`self.Launched`))
    (goto _label_4)))

(event `self.ReceiveTick`
  (params (DeltaSeconds :type "Float (single-precision)"))
  (bind _launched (`self.Launched`))
  (bind _returnvalue (`KismetMathLibrary.Vector_Distance` (`self.K2_GetActorLocation` (`self.HomingActor`)) (`self.K2_GetActorLocation`)))
  (if (not (`self.Low`))
    (`|ExecutionSequence`
      (:`then_0`
        (if (and (<= (`KismetMathLibrary.Vector_Distance` (`self.K2_GetActorLocation` (`self.HomingActor`)) (`self.K2_GetActorLocation`)) 300.0) (`self.Launched`))
          (set `ProjectileMovementComponent.HomingAccelerationMagnitude` 100000.0 (`self.ProjectileMovement`))))
      (:`then_1`
        (if (`self.Big`)
          (if (and _launched (<= _returnvalue 60.0))
            (set `self.CollidingActor` (`self.HomingActor`))
            (goto _label_2))
          (elif (and _launched (<= _returnvalue 30.0))
            (goto _label_3)))))))

(fn `DamageInRange`
  (params (Range :type "Float (double-precision)") (BaseDamage :type "Float (single-precision)"))
  (bind _returnvalue (`self.K2_GetActorLocation`))
  (bind _controller (`self.Controller`))
  (bind _stun (`self.Stun`))
  (bind _collidingenemy (`self.CollidingEnemy`))
  (bind _fire (`self.Fire`))
  (bind _low (`self.Low`))
  (bind _controller_2 (`self.Controller`))
  (bind _stun_2 (`self.Stun`))
  (`/Engine/EditorBlueprintResources/StandardMacros.IsValid` (`self.CollidingEnemy`)
    (:`Is Valid`
      (`|ExecutionSequence`
        (:`then_0`
          (`GameplayStatics.ApplyDamage` (`self.CollidingEnemy`) BaseDamage null self)
          (`/Game/BP/NewGame/BP_GridBasedPawn_Enemy.Pushback` _collidingenemy 0.0 (`KismetMathLibrary.Round` (`self.Force`)) (`self.K2_GetActorLocation` (`/Game/BP/NewGame/GridPlayerController.BPPlayer` (`self.Controller`))) :!label _label)
          (if (`self.Stun`)
            (`/Game/BP/NewGame/BP_GridBasedPawn_Enemy.GetStunned` _collidingenemy (+ (`KismetMathLibrary.Round` (`self.Power`)) 1))))
        (:`then_1`
          (if _fire
            (if _low
              (`/Game/BP/NewGame/GridPlayerController.UpdateFireground` _controller (`self.K2_GetActorLocation` (`self.CollidingEnemy`)) _stun)
              (else
                (`/Game/BP/NewGame/GridPlayerController.UpdateFireground` _controller (`self.K2_GetActorLocation` (`self.HomingActor`)) _stun :!label _label_2)))))))
    (:`Is Not Valid`
      (bind _outactors (`GameplayStatics.GetAllActorsOfClass` "/Game/BP/NewGame/BP_GridBasedPawn.BP_GridBasedPawn_C"))
      (for _array_element _outactors
        (cast `/Game/BP/NewGame/BP_GridBased_Player` _array_element
          (:`CastFailed`
            (if (<= (`KismetMathLibrary.Vector_Distance` (`self.K2_GetActorLocation` _array_element) (select `bool` (`self.Low`) :`false` (`self.K2_GetActorLocation` (`self.HomingActor`)) :`true` (`self.K2_GetActorLocation`))) Range)
              (`GameplayStatics.ApplyDamage` _array_element BaseDamage null self)
              (bind _asbp_grid_based_pawn_enemy (cast `/Game/BP/NewGame/BP_GridBasedPawn_Enemy` _array_element))
              (set `self.CollidingEnemy` _asbp_grid_based_pawn_enemy)
              (goto _label)))))
      (if _fire
        (if _low
          (bind _outactors_2 (`GameplayStatics.GetAllActorsOfClass` "/Game/BP/NewGame/BP_GridBasedPawn_Enemy.BP_GridBasedPawn_Enemy_C"))
          (bind _outhit (`KismetSystemLibrary.SphereTraceSingle` _returnvalue (+ _returnvalue (0.0 0.0 -100.0)) 5.0 "TraceTypeQuery1" false _outactors_2))
          (bind (_bblockinghit _binitialoverlap _time _distance _location _impactpoint _normal _impactnormal _physmat _hitactor) (`GameplayStatics.BreakHitResult` _outhit))
          (bind _asbp_ground_actor (cast `/Game/BP/NewGame/BP_GroundActor` _hitactor)
            (:`then`
              (`/Game/BP/NewGame/GridPlayerController.UpdateFireground` _controller_2 (+ (`self.K2_GetActorLocation` _asbp_ground_actor) (0.0 0.0 50.0)) _stun_2))
            (:`CastFailed`
              (bind _asbp_grided_obstacle (cast `/Game/BP/NewGame/BP_GridedObstacle` _hitactor))
              (`/Game/BP/NewGame/GridPlayerController.UpdateFireground` _controller_2 (`self.K2_GetActorLocation` _asbp_grided_obstacle) _stun_2)))
          (else
            (goto _label_2)))))))

(fn `IsValid`
  (params (Object :type "Object Object Reference"))
  (returns (Valid :type Boolean))
  (`/Engine/EditorBlueprintResources/StandardMacros.IsValid` Object
    (:`Is Valid`
      (return true))
    (:`Is Not Valid`
      (return false))))

(fn `UserConstructionScript`)