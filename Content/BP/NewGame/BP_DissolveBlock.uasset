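; BP_DissolveBlock is a scan-driven dissolve mask volume that feeds its position and size to materials.
; Holding E or calling Startscan enables Sphere query collision and plays a timeline lerping actor scale between one and zero; release or Endscan disables collision and reverses it.
; Tick and the Construction Script write Location's position and scale, plus Endofline's scale, to MP_DissolveMask, keeping both components at zero world rotation.
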(event `self.ReceiveBeginPlay`
  (`self.EnableInput` (`GameplayStatics.GetPlayerController` 0)))

(event `Startscan`
  (`PrimitiveComponent.SetCollisionEnabled` (`self.Sphere`) "QueryOnly" :!label _label)
  (bind (_direction `_新建轨道_0`) (`Timeline|时间轴` :!label _label_2)
    (:`Update`
      (`self.SetActorRelativeScale3D` (`KismetMathLibrary.VLerp` (`KismetMathLibrary.Conv_DoubleToVector` 1.0) (`KismetMathLibrary.Conv_DoubleToVector` 0.0) `_新建轨道_0`)))))

(event `Endscan`
  (`PrimitiveComponent.SetCollisionEnabled` (`self.Sphere`) "NoCollision" :!label _label_3)
  (goto _label_2 :!via `Reverse`))

(event `Key|E`
  (params (Key :type "Key Structure"))
  (:`Pressed`
    (goto _label))
  (:`Released`
    (goto _label_3)))

(event `self.ReceiveTick`
  (params (DeltaSeconds :type "Float (single-precision)"))
  (`KismetMaterialLibrary.SetVectorParameterValue` "/Game/Materials/Functions/MP_DissolveMask.MP_DissolveMask" "WorldLocation" (`KismetMathLibrary.Conv_VectorToLinearColor` (`SceneComponent.K2_GetComponentLocation` (`self.Location`))))
  (`KismetMaterialLibrary.SetVectorParameterValue` "/Game/Materials/Functions/MP_DissolveMask.MP_DissolveMask" "BoundingBoxBounds" (`KismetMathLibrary.Conv_VectorToLinearColor` (`SceneComponent.K2_GetComponentScale` (`self.Location`))))
  (`KismetMaterialLibrary.SetVectorParameterValue` "/Game/Materials/Functions/MP_DissolveMask.MP_DissolveMask" "EndOfLine" (`KismetMathLibrary.Conv_VectorToLinearColor` (`SceneComponent.K2_GetComponentScale` (`self.Endofline`))))
  (`SceneComponent.K2_SetWorldRotation` :`self` (`self.Endofline`))
  (`SceneComponent.K2_SetWorldRotation` :`self` (`self.Location`)))

(fn `UserConstructionScript`
  (`KismetMaterialLibrary.SetVectorParameterValue` "/Game/Materials/Functions/MP_DissolveMask.MP_DissolveMask" "WorldLocation" (`KismetMathLibrary.Conv_VectorToLinearColor` (`SceneComponent.K2_GetComponentLocation` (`self.Location`))))
  (`KismetMaterialLibrary.SetVectorParameterValue` "/Game/Materials/Functions/MP_DissolveMask.MP_DissolveMask" "BoundingBoxBounds" (`KismetMathLibrary.Conv_VectorToLinearColor` (`SceneComponent.K2_GetComponentScale` (`self.Location`))))
  (`KismetMaterialLibrary.SetVectorParameterValue` "/Game/Materials/Functions/MP_DissolveMask.MP_DissolveMask" "EndOfLine" (`KismetMathLibrary.Conv_VectorToLinearColor` (`SceneComponent.K2_GetComponentScale` (`self.Endofline`))))
  (`SceneComponent.K2_SetWorldRotation` :`self` (`self.Endofline`))
  (`SceneComponent.K2_SetWorldRotation` :`self` (`self.Location`)))