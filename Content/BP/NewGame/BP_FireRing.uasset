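; BP_FireRing is an expanding ring effect actor with a sphere component that grows and fades in when spawned.
; On BeginPlay a timeline lerps actor scale up from zero and drives the sphere material's Opacity parameter.
; The Reverse event plays the timeline backwards, then destroys the actor after a short delay.
; It caches the BP_GridBased_Player, but a ViewRange-based size calculation is left unconnected, so the final scale is fixed.
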(event `self.ReceiveBeginPlay`
  (bind _returnvalue (`GameplayStatics.GetActorOfClass` "/Game/BP/NewGame/BP_GridBased_Player.BP_GridBased_Player_C"))
  (set `self.Player` _returnvalue)
  (bind (_direction `_新建轨道_0`) (`Timeline|时间轴` :!label _label)
    (:`Update`
      (`self.SetActorScale3D` (`KismetMathLibrary.VLerp` (0.0 0.0 0.0) (`KismetMathLibrary.Conv_DoubleToVector` 10.0) `_新建轨道_0`))
      (`MeshComponent.SetScalarParameterValueOnMaterials` (`self.Sphere`) "Opacity" (`KismetMathLibrary.Lerp` 0.0 0.3 `_新建轨道_0`)))))

(event `Reverse`
  (`|ExecutionSequence`
    (:`then_0`
      (goto _label :!via `Reverse`))
    (:`then_1`
      (`KismetSystemLibrary.Delay` 0.1)
      (`self.K2_DestroyActor`))))

(fn `UserConstructionScript`)