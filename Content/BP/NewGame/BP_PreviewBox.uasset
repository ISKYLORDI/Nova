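; BP_PreviewBox is a grid tile marker for a possible player move, fading in on spawn through a timeline driving plane opacity.
; MovePlayer sends the owning BP_GridBased_Player to the box's location, dismisses all preview boxes, and optionally charges move cost and spawns new move boxes.
; DestroyFrame disables collision and reverses the fade before destroying the actor, and also runs when an enemy pawn overlaps the box.
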(event `self.ReceiveBeginPlay`
  (bind (_direction `_新建轨道_0`) (`Timeline|时间轴` :!label _label)
    (:`Update`
      (`MeshComponent.SetScalarParameterValueOnMaterials` (`self.Plane`) "Opacity" `_新建轨道_0`))
    (:`Finished`
      (if (`self.Destroyed`)
        (`self.K2_DestroyActor`)))))

(event `DestroyFrame`
  (set `self.Destroyed` true)
  (`self.SetActorEnableCollision` false)
  (goto _label :!via `Reverse`))

(event `MovePlayer`
  (params (Cost :type Boolean :default true))
  (bind _asbp_grid_based_player (cast `/Game/BP/NewGame/BP_GridBased_Player` (`self.OwnerActor`)))
  (set `/Game/BP/NewGame/BP_GridBasedPawn.EndLoc` (`self.K2_GetActorLocation`) _asbp_grid_based_player)
  (`/Game/BP/NewGame/BP_GridBased_Player.TakeNextStep` _asbp_grid_based_player true)
  (bind _outactors (`GameplayStatics.GetAllActorsOfClass` "BP_PreviewBox_C"))
  (for _array_element _outactors
    (`self.DestroyFrame` _array_element))
  (if Cost
    (`/Game/BP/NewGame/BP_GridBased_Player.MoveCost` _asbp_grid_based_player 0.0 0.0 1.0)
    (`/Game/BP/NewGame/BP_GridBased_Player.SpawnMoveBoxes` _asbp_grid_based_player 0.25 false false 150.0)))

(event `self.Box.OnComponentBeginOverlap`
  (params (OverlappedComponent :type "PrimitiveComponent Object Reference") (OtherActor :type "Actor Object Reference") (OtherComp :type "PrimitiveComponent Object Reference") (OtherBodyIndex :type Integer) (bFromSweep :type Boolean) (SweepResult :type "HitResult Structure (by ref)"))
  (cast `/Game/BP/NewGame/BP_GridBasedPawn_Enemy` OtherActor)
  (`self.DestroyFrame`))

(fn `UserConstructionScript`)