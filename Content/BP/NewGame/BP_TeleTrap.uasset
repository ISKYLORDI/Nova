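; Teleport trap that sends the affected player to a randomly chosen other teleporter location.
; BeginPlay fills the list of possible teleport coordinates, with a length check that can trim its third entry.
; SpecialEffect copies that list, drops this trap's own TeleporterIndex, sets the player's EndLoc to a random remaining entry and ends their turn.
; Overlap and Tick events are disabled.
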(event `self.ReceiveBeginPlay`
  (bind _possibletelecoords (`self.PossibleTeleCoords`))
  (`parent.ReceiveBeginPlay`)
  (set `self.PossibleTeleCoords` (`|MakeArray` (`self.[ 0]`) (`self.[ 1]`) (`self.[ 2]`)))
  (if (== (`KismetArrayLibrary.Array_Length` _possibletelecoords) 2)
    (`KismetArrayLibrary.Array_Remove` _possibletelecoords 2)))

(fn `SpecialEffect`
  (params (player :type "/Game/BP/NewGame/BP_GridBased_Player Object Reference"))
  (locals (OtherTeleports :type "Array of Vector Structure"))
  (bind _output_get (set `local.OtherTeleports` (`self.PossibleTeleCoords`)))
  (`KismetArrayLibrary.Array_Remove` _output_get (`self.TeleporterIndex`))
  (set `/Game/BP/NewGame/BP_GridBasedPawn.EndLoc` (`KismetArrayLibrary.Array_Random` (`local.OtherTeleports`)) player)
  ;[1 1 1] 可以替换为其他特效函数
  (`/Game/BP/NewGame/BP_GridBased_Player.EndTurn` player))

(fn `UserConstructionScript`
  (`parent.UserConstructionScript`))