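; BP_PlayerTurn is an actor that marks its open movement options by spawning BP_PreviewBox actors around itself.
; SpawnMoveBoxes tests eight spots: one and two move distances forward, back, right and left, relative to its facing.
; SpawnBoxes line traces on Visibility to each spot and spawns a box owned by this actor only when nothing is hit, so a near obstacle also blocks the farther spot.
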(event `SpawnMoveBoxes`
  (`self.SpawnBoxes` (`self.GetActorForwardVector`) (`self.MoveDistance_0`))
  (`self.SpawnBoxes` (`self.GetActorForwardVector`) (* (`self.MoveDistance_0`) 2.0))
  (`self.SpawnBoxes` (`self.GetActorForwardVector`) (* (`self.MoveDistance_0`) -1.0))
  (`self.SpawnBoxes` (`self.GetActorForwardVector`) (* (`self.MoveDistance_0`) -2.0))
  (`self.SpawnBoxes` (`self.GetActorRightVector`) (`self.MoveDistance_0`))
  (`self.SpawnBoxes` (`self.GetActorRightVector`) (* (`self.MoveDistance_0`) 2.0))
  (`self.SpawnBoxes` (`self.GetActorRightVector`) (* (`self.MoveDistance_0`) -1.0))
  (`self.SpawnBoxes` (`self.GetActorRightVector`) (* (`self.MoveDistance_0`) -2.0)))

(fn `SpawnBoxes`
  (params (Direction :type "Vector Structure") (Distance :type "Float (double-precision)"))
  (bind _returnvalue (`self.K2_GetActorLocation`))
  (bind _returnvalue_2 (+ _returnvalue (* Direction Distance)))
  (bind (_outhit _returnvalue_3) (`KismetSystemLibrary.LineTraceSingle` _returnvalue _returnvalue_2 "TraceTypeQuery1"))
  (if (not _returnvalue_3)
    (bind _returnvalue_4 (`|SpawnActorFromClass` "/Game/BP/NewGame/BP_PreviewBox.BP_PreviewBox_C" (`KismetMathLibrary.MakeTransform` _returnvalue_2) "Undefined" "MultiplyWithRoot" null null))
    (set `/Game/BP/NewGame/BP_PreviewBox.OwnerActor` self _returnvalue_4)))

(fn `UserConstructionScript`)