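; Base grid pawn that hops to a target cell like a board-game piece, with collision off during the move.
; A timeline lerps location with a vertical arc and optionally turns the model to a 90-degree-multiple yaw, then plays a landing sound.
; Enemy subclasses then trace downward and, without close ground, fall via a second timeline and call Death.
; The construction script snaps the pawn to the grid when the Update flag is set.
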(event `self.ReceiveBeginPlay`)

(event `TakeNextStep`
  (params (`Rotate?` :type Boolean :default true))
  (bind (_returnvalue_roll _returnvalue_pitch _returnvalue_yaw) (`KismetMathLibrary.BreakRotator` (`SceneComponent.K2_GetComponentRotation` (`self.RotateModel`))))
  (bind (_returnvalue_roll_2 _returnvalue_pitch_2 _returnvalue_yaw_2) (`KismetMathLibrary.BreakRotator` (`KismetMathLibrary.FindLookAtRotation` (`self.StartLoc`) (`self.EndLoc`))))
  (bind (_remainder _returnvalue) (`KismetMathLibrary.FMod` _returnvalue_yaw_2 90.0))
  (set `self.Rotate?` `Rotate?`)
  (set `self.StartLoc` (`self.K2_GetActorLocation`))
  (set `self.Moving` true)
  (set `self.StartRot` (`KismetMathLibrary.MakeRotator` 0.0 0.0 _returnvalue_yaw))
  (`self.SetActorEnableCollision` false)
  (`TimelineComponent.SetPlayRate` (`self.时间轴`) 0.6)
  (bind (_direction `_新建轨道_0` `_新建轨道_1`) (`Timeline|时间轴` :!via `PlayFromStart`)
    (:`Update`
      (bind (_returnvalue_x _returnvalue_y _returnvalue_z) (`KismetMathLibrary.BreakVector` (`KismetMathLibrary.VLerp` (`self.StartLoc`) (`self.EndLoc`) `_新建轨道_0`)))
      (bind (_returnvalue_x_2 _returnvalue_y_2 _returnvalue_z_2) (`KismetMathLibrary.BreakVector` (`KismetMathLibrary.VLerp` (0.0 0.0 0.0) (0.0 0.0 100.0) `_新建轨道_1`)))
      (`self.K2_SetActorLocation` (`KismetMathLibrary.MakeVector` _returnvalue_x _returnvalue_y (+ _returnvalue_z _returnvalue_z_2)))
      (if (`self.Rotate?`)
        (`SceneComponent.K2_SetWorldRotation` (`self.RotateModel`) (`KismetMathLibrary.RLerp` (`self.StartRot`) (`KismetMathLibrary.MakeRotator` 0.0 0.0 (- (`KismetMathLibrary.Conv_IntToDouble` (* (+ (`KismetMathLibrary.Round64` _remainder) _returnvalue) 90)) 90.0)) `_新建轨道_0` true) false false)))
    (:`Finished`
      (`GameplayStatics.SpawnSoundAtLocation` "/Game/Sound/SFX/Characters/Chess/S_Chess_Move_Upstairs01_Cue.S_Chess_Move_Upstairs01_Cue" (`self.K2_GetActorLocation`) (struct) 1.0 1.0 0.0 null null)
      (`self.SetActorEnableCollision` true)
      (set `self.Moving` false)
      (bind _asbp_grid_based_pawn_enemy (cast `/Game/BP/NewGame/BP_GridBasedPawn_Enemy` self))
      (bind _returnvalue_2 (`self.K2_GetActorLocation` _asbp_grid_based_pawn_enemy))
      (bind (_outhit _returnvalue_3) (`KismetSystemLibrary.LineTraceSingle` _returnvalue_2 (+ _returnvalue_2 (* (`self.GetActorUpVector` _asbp_grid_based_pawn_enemy) (0.0 0.0 -1000.0))) "TraceTypeQuery1"))
      (if _returnvalue_3
        (if (> (`.Distance` (`GameplayStatics.BreakHitResult` _outhit)) 102.0)
          (bind _output_get (set `self.EndLoc` (`self.K2_GetActorLocation` _asbp_grid_based_pawn_enemy) :!label _label))
          (bind (_direction_2 `_新建轨道_0_2`) (`Timeline|FallDown` :!via `PlayFromStart`)
            (:`Update`
              (`self.K2_SetActorLocation` _asbp_grid_based_pawn_enemy (`KismetMathLibrary.VLerp` _output_get (+ _output_get (* (`self.GetActorUpVector` _asbp_grid_based_pawn_enemy) (0.0 0.0 -500.0))) `_新建轨道_0_2`) false false))
            (:`Finished`
              (bind _asbp_grid_based_pawn_enemy_2 (cast `/Game/BP/NewGame/BP_GridBasedPawn_Enemy` self))
              (`/Game/BP/NewGame/BP_GridBasedPawn_Enemy.Death` _asbp_grid_based_pawn_enemy_2))))
        (else
          (goto _label))))))

(fn `UserConstructionScript`
  (bind (_returnvalue_x _returnvalue_y _returnvalue_z) (`KismetMathLibrary.BreakVector` (`self.K2_GetActorLocation`)))
  (if (`self.Update`)
    (`self.K2_SetActorLocation` (`KismetMathLibrary.MakeVector` (`KismetMathLibrary.Conv_IntToDouble` (* (`.ReturnValue` (`KismetMathLibrary.FMod` _returnvalue_x 100.0)) 100)) (`KismetMathLibrary.Conv_IntToDouble` (* (`.ReturnValue` (`KismetMathLibrary.FMod` _returnvalue_y 100.0)) 100)) (`KismetMathLibrary.Conv_IntToDouble` (* (`.ReturnValue` (`KismetMathLibrary.FMod` _returnvalue_z 50.0)) 50))))
    (set `self.Update` false)))