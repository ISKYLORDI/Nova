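; Fire ground hazard for the grid-based, turn-based game, shown as a blue fire wall in its stun variant and red otherwise.
; SpawnEvent sets the variant and enables collision after a short delay; the stun variant stuns each enemy on its first overlap.
; DamageEvent damages overlapping pawns, hurting the player less, while TurnPassed counts turns and fades out and destroys the fire after three.
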(event `self.ReceiveBeginPlay`
  (`parent.ReceiveBeginPlay`)
  (bind _asgrid_player_controller (cast `/Game/BP/NewGame/GridPlayerController` (`GameplayStatics.GetPlayerController` 0)))
  (set `self.Controler` _asgrid_player_controller))

(event `Spawn Event`
  (params (Stun :type Boolean))
  (bind _output_get (set `self.Stun` Stun))
  (`ParticleSystemComponent.SetTemplate` (`self.ParticleSystem`) (select `bool` _output_get :`false` "/Game/VFX/Realistic_Starter_VFX_Pack_Vol2/Particles/Fire/P_Fire_WallRed.P_Fire_WallRed" :`true` "/Game/VFX/Realistic_Starter_VFX_Pack_Vol2/Particles/Fire/P_Fire_WallBlue.P_Fire_WallBlue" :!type "ParticleSystem Object Reference"))
  (`KismetSystemLibrary.Delay` 0.1)
  (`PrimitiveComponent.SetCollisionEnabled` (`self.CollisionBox`) "QueryOnly"))

(event `TurnPassed`
  (bind _result (`/Engine/EditorBlueprintResources/StandardMacros.IncrementInt` (`self.TurnsPassed`))
    (:`  `
      (if (>= _result 3)
        (`ActorComponent.Deactivate` (`self.ParticleSystem`))
        (`self.SetActorEnableCollision` false)
        (`KismetSystemLibrary.Delay` 3.0)
        (`self.K2_DestroyActor`)))))

(event `self.CollisionBox.OnComponentBeginOverlap`
  (params (OverlappedComponent :type "PrimitiveComponent Object Reference") (OtherActor :type "Actor Object Reference") (OtherComp :type "PrimitiveComponent Object Reference") (OtherBodyIndex :type Integer) (bFromSweep :type Boolean) (SweepResult :type "HitResult Structure (by ref)"))
  (bind _asbp_grid_based_pawn_enemy (cast `/Game/BP/NewGame/BP_GridBasedPawn_Enemy` OtherActor))
  (if (not (`KismetArrayLibrary.Array_Contains` (`self.DamagedEnemies`) _asbp_grid_based_pawn_enemy))
    (`KismetArrayLibrary.Array_Add` (`self.DamagedEnemies`) _asbp_grid_based_pawn_enemy)
    (if (`self.Stun`)
      (`/Game/BP/NewGame/BP_GridBasedPawn_Enemy.GetStunned` _asbp_grid_based_pawn_enemy 1))))

(event `DamageEvent`
  (for _array_element (`PrimitiveComponent.GetOverlappingActors` (`self.CollisionBox`) "/Game/BP/NewGame/BP_GridBasedPawn.BP_GridBasedPawn_C")
    (bind _asbp_grid_based_player (cast `/Game/BP/NewGame/BP_GridBased_Player` _array_element)
      (:`then`
        (`GameplayStatics.ApplyDamage` _asbp_grid_based_player 0.1 null self))
      (:`CastFailed`
        (`GameplayStatics.ApplyDamage` _array_element 0.5 null self)))))

(fn `UserConstructionScript`
  (`parent.UserConstructionScript`))