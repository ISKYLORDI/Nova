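; BP_EnemySpawner is a placeable spawner that creates a BP_GridBasedPawn_Enemy of a configured EnemyType at its own location.
; BeginPlay spawns the enemy with a 90-degree yaw offset, stores it, then sets its type and calls UpdateType.
; SpawnEnemy destroys any existing spawned enemy and repeats that spawn.
; The construction script shows the monster component matching EnemyType, though Firethrower shows none of the three.
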(event `self.ReceiveBeginPlay`
  (bind (_returnvalue_location _returnvalue_rotation) (`KismetMathLibrary.BreakTransform` (`self.GetTransform`)))
  (bind _returnvalue (`|SpawnActorFromClass` "/Game/BP/NewGame/BP_GridBasedPawn_Enemy.BP_GridBasedPawn_Enemy_C" (`KismetMathLibrary.MakeTransform` _returnvalue_location (`KismetMathLibrary.MakeRotator` 0.0 0.0 (+ (.yaw _returnvalue_rotation) 90.0))) "Undefined" "MultiplyWithRoot" null null :!label _label))
  (bind _output_get (set `self.EnemySpawned` _returnvalue))
  (set `/Game/BP/NewGame/BP_GridBasedPawn_Enemy.EnemyType` (`self.EnemyType`) _returnvalue)
  (`/Game/BP/NewGame/BP_GridBasedPawn_Enemy.UpdateType` _output_get))

(event `SpawnEnemy`
  (bind _enemyspawned (`self.EnemySpawned`))
  (`/Engine/EditorBlueprintResources/StandardMacros.IsValid` _enemyspawned
    (:`Is Valid`
      (`self.K2_DestroyActor` _enemyspawned)
      (goto _label))
    (:`Is Not Valid`
      (goto _label))))

(fn `UserConstructionScript`
  (`SceneComponent.SetVisibility` (`self.monster1_1_`) (select `/Game/BP/NewGame/EN_GridEnemyType` (`self.EnemyType`) :`NewEnumerator0` true) true)
  (`SceneComponent.SetVisibility` (`self.monster2_1_`) (select `/Game/BP/NewGame/EN_GridEnemyType` (`self.EnemyType`) :`NewEnumerator2` true) true)
  (`SceneComponent.SetVisibility` (`self.monster3_1_`) (select `/Game/BP/NewGame/EN_GridEnemyType` (`self.EnemyType`) :`NewEnumerator3` true) true))