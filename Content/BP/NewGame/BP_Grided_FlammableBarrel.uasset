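; BP_Grided_FlammableBarrel is a destructible, flammable barrel for a grid-based, turn-based game.
; Damage reduces HitPoints; at zero, or on DeathExplosion, a DoOnce spawns a fire BP_Shockwave with sound, then a timeline scales the barrel up before destroying it.
; Each passed turn decrements fire and checks fire spread.
; Tick yaws the health-bar widget and Scene1 to match the camera's facing.
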(event `self.ReceiveBeginPlay`
  (`parent.ReceiveBeginPlay`)
  (bind _asw_health_bar (cast `/Game/BP/NewGame/W_HealthBar` (`WidgetComponent.GetWidget` (`self.Widget`))))
  (set `self.HPwidget` _asw_health_bar)
  (set `/Game/BP/NewGame/W_HealthBar.Pawn` self _asw_health_bar))

(event `self.DeathExplosion`
  (params (SystemTemplate :type "NiagaraSystem Object Reference") (Sound :type "SoundBase Object Reference"))
  (bind _fireemitter (`self.FireEmitter`))
  (`parent.DeathExplosion` SystemTemplate Sound)
  (`/Engine/EditorBlueprintResources/StandardMacros.DoOnce` false :!label _label
    (:`Completed`
      (bind _returnvalue (`|SpawnActorFromClass` "/Game/BP/NewGame/BP_Shockwave.BP_Shockwave_C" (`self.GetTransform`) "Undefined" "MultiplyWithRoot" null null))
      (`/Game/BP/NewGame/BP_Shockwave.SpawnEvent` _returnvalue 2.0 150.0 0.0 true false 1.0 true false)
      (`GameplayStatics.PlaySoundAtLocation` "/Game/Sound/SFX/Skills/Fire_Ground/S_Fire_AOE_Burst_02.S_Fire_AOE_Burst_02" (`self.K2_GetActorLocation`) (struct) 1.0 1.0 0.0 "/Game/Sound/SFX/Att.Att" null null null)
      (`self.SetActorEnableCollision` false)
      (bind (_direction `_新建轨道_0`) (`Timeline|Timeline` :!via `PlayFromStart`)
        (:`Update`
          (`self.SetActorRelativeScale3D` (`KismetMathLibrary.VLerp` (`KismetMathLibrary.Conv_DoubleToVector` 1.0) (`KismetMathLibrary.Conv_DoubleToVector` 1.5) `_新建轨道_0`)))
        (:`Finished`
          (`/Engine/EditorBlueprintResources/StandardMacros.IsValid` _fireemitter
            (:`Is Valid`
              (`ActorComponent.Deactivate` _fireemitter))
            (:`Is Not Valid`
              _))
          (`self.K2_DestroyActor`))))))

(event `self.ReceiveAnyDamage`
  (params (Damage :type "Float (single-precision)") (DamageType :type "DamageType Object Reference") (InstigatedBy :type "Controller Object Reference") (DamageCauser :type "Actor Object Reference"))
  (bind _output_get (set `self.HitPoints` (- (`self.HitPoints`) Damage)))
  (if (<= _output_get 0.0)
    (goto _label)))

(event `self.TurnPassed`
  (`parent.TurnPassed`)
  (`self.FireDecrement`)
  (`self.FirespreadCheck` 85.0))

(event `self.ReceiveTick`
  (params (DeltaSeconds :type "Float (single-precision)"))
  (bind _returnvalue (`GameplayStatics.GetPlayerCameraManager` 0))
  (bind _returnvalue_2 (`self.K2_GetActorLocation` _returnvalue))
  (bind (_returnvalue_roll _returnvalue_pitch _returnvalue_yaw) (`KismetMathLibrary.BreakRotator` (`KismetMathLibrary.FindLookAtRotation` (+ _returnvalue_2 (* (`self.GetActorForwardVector` _returnvalue) 500.0)) _returnvalue_2)))
  (`SceneComponent.K2_SetWorldRotation` (`self.Widget`) (`KismetMathLibrary.MakeRotator` 0.0 0.0 _returnvalue_yaw) false false)
  (`SceneComponent.K2_SetWorldRotation` (`self.Scene1`) (`KismetMathLibrary.MakeRotator` 0.0 0.0 _returnvalue_yaw) false false))

(fn `UserConstructionScript`
  (`parent.UserConstructionScript`))