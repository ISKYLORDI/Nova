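; BP_TargetBox is a clickable grid target marker for skill targeting that glides toward its SnapLocation by lerping every tick.
; A timeline fades the plane's opacity in on spawn, and DestroyFrame disables collision and reverses it, destroying the actor when finished.
; Clicks notify the GridPlayerController according to its SkillStatus: Big Fireball always confirms, while Teleport confirms only if no player or enemy pawn overlaps the box.
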(event `self.ReceiveBeginPlay`
  (bind _asgrid_player_controller (cast `/Game/BP/NewGame/GridPlayerController` (`GameplayStatics.GetPlayerController` 0)))
  (set `self.Controller` _asgrid_player_controller)
  (bind (_direction `_新建轨道_0`) (`Timeline|时间轴` :!label _label)
    (:`Update`
      (`MeshComponent.SetScalarParameterValueOnMaterials` (`self.Plane`) "Opacity" `_新建轨道_0`))
    (:`Finished`
      (if (`self.Destroyed`)
        (`self.K2_DestroyActor`)))))

(event `DestroyFrame`
  (set `self.Destroyed` true)
  (`self.SetActorEnableCollision` false)
  (goto _label :!via `Reverse`))

(event `self.ReceiveTick`
  (params (DeltaSeconds :type "Float (single-precision)"))
  (`self.K2_SetActorLocation` (`KismetMathLibrary.VLerp` (`self.K2_GetActorLocation`) (`self.SnapLocation`) 0.5)))

(event `Clicked`
  (switch `/Game/BP/NewGame/EN_GridSkillSets` (`/Game/BP/NewGame/GridPlayerController.SkillStatus` (`self.Controller`))
    (:`NewEnumerator1`
      (if (not (or (> (`KismetArrayLibrary.Array_Length` (`self.GetOverlappingActors` "/Game/BP/NewGame/BP_GridBasedPawn_Enemy.BP_GridBasedPawn_Enemy_C")) 0) (> (`KismetArrayLibrary.Array_Length` (`self.GetOverlappingActors` "/Game/BP/NewGame/BP_GridBased_Player.BP_GridBased_Player_C")) 0)))
        (`/Game/BP/NewGame/GridPlayerController.TargetClicked` (`self.Controller`) :!label _label_2)))
    (:`NewEnumerator5`
      (goto _label_2))))

(fn `UserConstructionScript`)