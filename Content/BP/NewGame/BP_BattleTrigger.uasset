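; Battle arena trigger that locks the player inside and starts a fight when BP_GridBased_Player enters its box.
; The construction script sizes the box and builds four wall colliders around it, disabled until activation.
; On first overlap it spawns enemies from overlapping BP_EnemySpawners, enables the walls and shows the cube.
; A looping timer lifts the lockdown when no enemy is close, re-arming only if the player died.
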(event `self.Box.OnComponentBeginOverlap`
  (params (OverlappedComponent :type "PrimitiveComponent Object Reference") (OtherActor :type "Actor Object Reference") (OtherComp :type "PrimitiveComponent Object Reference") (OtherBodyIndex :type Integer) (bFromSweep :type Boolean) (SweepResult :type "HitResult Structure (by ref)"))
  (bind _asbp_grid_based_player (cast `/Game/BP/NewGame/BP_GridBased_Player` OtherActor))
  (set `self.Char` _asbp_grid_based_player)
  (`/Engine/EditorBlueprintResources/StandardMacros.DoOnce` false :!label _label
    (:`Completed`
      (for _array_element (`PrimitiveComponent.GetOverlappingActors` (`self.Box`) "/Game/BP/NewGame/BP_EnemySpawner.BP_EnemySpawner_C")
        (bind _asbp_enemy_spawner (cast `/Game/BP/NewGame/BP_EnemySpawner` _array_element))
        (`/Game/BP/NewGame/BP_EnemySpawner.SpawnEnemy` _asbp_enemy_spawner 0.0))
      (set `self.Activated` true)
      (for _array_element_2 (`self.Collisions`)
        (`PrimitiveComponent.SetCollisionEnabled` _array_element_2 "QueryAndPhysics"))
      (`SceneComponent.SetHiddenInGame` (`self.Cube`) false false)
      (bind _returnvalue (`KismetSystemLibrary.K2_SetTimer` null "DeactivateCheck" 0.2 true 0.0 0.2))
      (set `self.DeactivateHandle` _returnvalue))))

(event `ResetTrigger`
  (goto _label :!via `Reset`))

(event `DeactivateBattle`
  (`SceneComponent.SetHiddenInGame` (`self.Cube`) true false)
  (for _array_element (`self.Collisions`)
    (`PrimitiveComponent.SetCollisionEnabled` _array_element "NoCollision"))
  (set `self.Activated` false))

(fn `DeactivateCheck`
  (bind _char (`self.Char`))
  (if (not (`/Game/BP/NewGame/BP_GridBased_Player.IfEnemyClose` _char))
    (`KismetSystemLibrary.K2_ClearAndInvalidateTimerHandle` (`self.DeactivateHandle`))
    (`self.DeactivateBattle`)
    (if (`/Game/BP/NewGame/BP_GridBased_Player.Dead` _char)
      (`self.ResetTrigger`))))

(fn `UserConstructionScript`
  (bind (_returnvalue_x _returnvalue_y) (`KismetMathLibrary.BreakVector` (`self.GetActorScale3D`)))
  (bind _box (`self.Box`))
  (bind _thickness (`self.Thickness`))
  (bind _thickness_2 (`self.Thickness`))
  (bind _thickness_3 (`self.Thickness`))
  (bind _thickness_4 (`self.Thickness`))
  (bind _thickness_5 (`self.Thickness`))
  (bind _thickness_6 (`self.Thickness`))
  (bind (_origin _boxextent) (`KismetSystemLibrary.GetComponentBounds` (`self.Box`)))
  (bind _returnvalue (+ _thickness_3 (.z _boxextent) _thickness_3))
  (`SceneComponent.SetWorldScale3D` _box (1.0 1.0 1.0))
  (`BoxComponent.SetBoxExtent` _box (* (`self.Extent`) (`self.GetActorScale3D`)) true)
  (`SceneComponent.SetWorldScale3D` (`self.Cube`) (`KismetMathLibrary.MakeVector` _returnvalue_x _returnvalue_y 10.0))
  (`KismetArrayLibrary.Array_Clear` (`self.Collisions`))
  (`|ExecutionSequence`
    (:`then_0`
      (bind _returnvalue_2 (`AddComponent|NODE_AddBoxComponent-4`))
      (`SceneComponent.K2_SetWorldLocation` _returnvalue_2 (+ _origin (`KismetMathLibrary.MakeVector` (.x _boxextent)) (`KismetMathLibrary.MakeVector` _thickness_5)) false false)
      (`BoxComponent.SetBoxExtent` _returnvalue_2 (`KismetMathLibrary.MakeVector` _thickness_2 (+ _thickness_2 (.y _boxextent) _thickness_2) _returnvalue) true)
      (`KismetArrayLibrary.Array_Add` (`self.Collisions`) _returnvalue_2)
      (bind _returnvalue_3 (`AddComponent|NODE_AddBoxComponent-5`))
      (`SceneComponent.K2_SetWorldLocation` _returnvalue_3 (- _origin (`KismetMathLibrary.MakeVector` (.x _boxextent)) (`KismetMathLibrary.MakeVector` _thickness_5)) false false)
      (`BoxComponent.SetBoxExtent` _returnvalue_3 (`KismetMathLibrary.MakeVector` _thickness (+ _thickness (.y _boxextent) _thickness) _returnvalue) true)
      (`KismetArrayLibrary.Array_Add` (`self.Collisions`) _returnvalue_3))
    (:`then_1`
      (bind _returnvalue_4 (`AddComponent|NODE_AddBoxComponent-6`))
      (`SceneComponent.K2_SetWorldLocation` _returnvalue_4 (+ _origin (`KismetMathLibrary.MakeVector` 0.0 (.y _boxextent)) (`KismetMathLibrary.MakeVector` 0.0 _thickness_5)) false false)
      (`BoxComponent.SetBoxExtent` _returnvalue_4 (`KismetMathLibrary.MakeVector` (+ _thickness_6 (.x _boxextent) _thickness_6) _thickness_6 _returnvalue) true)
      (`KismetArrayLibrary.Array_Add` (`self.Collisions`) _returnvalue_4)
      (bind _returnvalue_5 (`AddComponent|NODE_AddBoxComponent-7`))
      (`SceneComponent.K2_SetWorldLocation` _returnvalue_5 (- _origin (`KismetMathLibrary.MakeVector` 0.0 (.y _boxextent)) (`KismetMathLibrary.MakeVector` 0.0 _thickness_5)) false false)
      (`BoxComponent.SetBoxExtent` _returnvalue_5 (`KismetMathLibrary.MakeVector` (+ _thickness_4 (.x _boxextent) _thickness_4) _thickness_4 _returnvalue) true)
      (`KismetArrayLibrary.Array_Add` (`self.Collisions`) _returnvalue_5))
    (:`then_2`
      (for _array_element (`self.Collisions`)
        (`SceneComponent.SetWorldScale3D` _array_element (1.0 1.0 1.0))
        (`PrimitiveComponent.SetCollisionEnabled` _array_element "NoCollision")))))