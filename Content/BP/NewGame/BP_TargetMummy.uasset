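; BP_TargetMummy is a target that dies only when hit by damage matching its list of skill Requirements.
; BeginPlay shows each requirement as a skill button in a widget, which Tick keeps turned toward the camera.
; AnyDamage tests the damage causer's class, flags and shockwave owner against the requirements, allowing combinations such as AOE with Fireball.
; A valid hit triggers Dead once, playing Niagara and sphere-fade effects, clearing the icons and destroying the actor.
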(event `self.ReceiveBeginPlay`
  (bind _asui_horizontal_box (cast `/Game/BP/NewGame/UI/UI_HorizontalBox` (`WidgetComponent.GetWidget` (`self.Widget`))))
  (set `self.HorizontalBox` _asui_horizontal_box)
  (for _array_element (`self.Requirements`)
    (bind _returnvalue (`|CreateWidget` "/Game/BP/NewGame/W_skillbutton.W_skillbutton_C"))
    (set `/Game/BP/NewGame/W_skillbutton.SkillIndex` (select `/Game/BP/NewGame/EN_GridSkillSets` _array_element :`NewEnumerator1` 3 :`NewEnumerator2` 8 :`NewEnumerator3` 4 :`NewEnumerator5` 7 :`NewEnumerator6` 5 :`NewEnumerator7` 6 :`NewEnumerator8` 2 :`NewEnumerator9` 3) _returnvalue)
    (`KismetArrayLibrary.Array_Add` (`self.Skills`) _returnvalue)
    (`PanelWidget.AddChild` (`/Game/BP/NewGame/UI/UI_HorizontalBox.HorizontalBox` (`self.HorizontalBox`)) _returnvalue))
  (`KismetSystemLibrary.Delay` 0.1)
  (for _array_element_2 (`self.Skills`)
    (`/Game/BP/NewGame/W_skillbutton.UpdateButtonOutlook` _array_element_2)))

(event `Dead`
  (bind _sphere (`self.Sphere`))
  (`/Engine/EditorBlueprintResources/StandardMacros.DoOnce` false
    (:`Completed`
      (`self.SetActorEnableCollision` false)
      (`NiagaraFunctionLibrary.SpawnSystemAtLocation` "/Game/VFX/BlinkAndDashVFX/VFX_Niagara/NS_Blink_Fire.NS_Blink_Fire" (`self.K2_GetActorLocation`))
      (`|ExecutionSequence`
        (:`then_0`
          (bind (_direction _newtrack_0) (`Timeline|Timeline` :!via `PlayFromStart`)
            (:`Update`
              (`SceneComponent.SetWorldScale3D` (`self.Sphere`) (`KismetMathLibrary.VLerp` (`KismetMathLibrary.Conv_DoubleToVector` 0.6) (`KismetMathLibrary.Conv_DoubleToVector` 3.0) _newtrack_0))
              (`MeshComponent.SetScalarParameterValueOnMaterials` _sphere "Opacity" (`KismetMathLibrary.Lerp` 1.0 0.0 _newtrack_0))
              (`MeshComponent.SetScalarParameterValueOnMaterials` _sphere "Intensity" (`KismetMathLibrary.Lerp` 1.0 5.0 _newtrack_0)))
            (:`Finished`
              (`KismetSystemLibrary.Delay` 0.5)
              (`self.K2_DestroyActor`))))
        (:`then_1`
          (for _array_element (`self.Skills`)
            (`/Game/BP/NewGame/W_skillbutton.TurnBlank` _array_element)
            (`/Game/BP/NewGame/W_skillbutton.Dissappear` _array_element)))))))

(event `self.ReceiveAnyDamage`
  (params (Damage :type "Float (single-precision)") (DamageType :type "DamageType Object Reference") (InstigatedBy :type "Controller Object Reference") (DamageCauser :type "Actor Object Reference"))
  (set `self.NA` false)
  (for _array_element (`self.Requirements`)
    (switch `/Game/BP/NewGame/EN_GridSkillSets` _array_element
      (:`NewEnumerator0`
        (set `self.NA` true))
      (:`NewEnumerator1`
        (bind _asbp_player_projectile (cast `/Game/BP/NewGame/BP_PlayerProjectile` DamageCauser)
          (:`then`
            (if (`/Game/BP/NewGame/BP_PlayerProjectile.Low` _asbp_player_projectile)
              (set `self.NA` true :!label _label)))
          (:`CastFailed`
            (if (not (`self.Find` "NewEnumerator5")) :!label _label_2
              (goto _label)))))
      (:`NewEnumerator2`
        (bind _asbp_player_projectile_2 (cast `/Game/BP/NewGame/BP_PlayerProjectile` DamageCauser)
          (:`then`
            (if (not (`/Game/BP/NewGame/BP_PlayerProjectile.Low` _asbp_player_projectile_2))
              (goto _label)))
          (:`CastFailed`
            (goto _label_2))))
      (:`NewEnumerator3`
        (bind _asbp_player_projectile_3 (cast `/Game/BP/NewGame/BP_PlayerProjectile` DamageCauser)
          (:`then`
            (if (not (`/Game/BP/NewGame/BP_PlayerProjectile.Stun` _asbp_player_projectile_3))
              (set `self.NA` true :!label _label_3)))
          (:`CastFailed`
            (bind _asbp_shockwave (cast `/Game/BP/NewGame/BP_Shockwave` DamageCauser))
            (if (not (`/Game/BP/NewGame/BP_Shockwave.Stun` _asbp_shockwave))
              (goto _label_3)))))
      (:`NewEnumerator5`
        (bind _asbp_shockwave_2 (cast `/Game/BP/NewGame/BP_Shockwave` DamageCauser)
          (:`then`
            (if (`self.Find` "NewEnumerator2")
              (bind _returnvalue (`self.GetOwner` _asbp_shockwave_2))
              (bind _asbp_player_projectile_4 (cast `/Game/BP/NewGame/BP_PlayerProjectile` _returnvalue)
                (:`then`
                  (if (not (`/Game/BP/NewGame/BP_PlayerProjectile.Low` _asbp_player_projectile_4))
                    (set `self.NA` true :!label _label_4)))
                (:`CastFailed`
                  (goto _label_4)))
              (elif (`self.Find` "NewEnumerator1")
                (bind _asbp_player_projectile_5 (cast `/Game/BP/NewGame/BP_PlayerProjectile` _returnvalue)
                  (:`then`
                    (if (`/Game/BP/NewGame/BP_PlayerProjectile.Low` _asbp_player_projectile_5)
                      (goto _label_4)))
                  (:`CastFailed`
                    (goto _label_4))))))
          (:`CastFailed`
            (goto _label_4))))
      (:`NewEnumerator6`
        (cast `/Game/BP/NewGame/BP_GridBased_FireGround` DamageCauser
          (:`CastFailed`
            (goto _label_3))))
      (:`NewEnumerator7`
        (bind _asbp_player_projectile_6 (cast `/Game/BP/NewGame/BP_PlayerProjectile` DamageCauser)
          (:`then`
            (if (not (> (`/Game/BP/NewGame/BP_PlayerProjectile.Force` _asbp_player_projectile_6) 0.0))
              (set `self.NA` true :!label _label_5)))
          (:`CastFailed`
            (bind _asbp_shockwave_3 (cast `/Game/BP/NewGame/BP_Shockwave` DamageCauser))
            (if (not (> (`/Game/BP/NewGame/BP_Shockwave.Force` _asbp_shockwave_3) 0.0))
              (goto _label_5)))))))
  (if (not (`self.NA`))
    (`self.Dead`)))

(event `self.ReceiveTick`
  (params (DeltaSeconds :type "Float (single-precision)"))
  (bind _returnvalue (`GameplayStatics.GetPlayerCameraManager` 0))
  (bind _returnvalue_2 (`self.K2_GetActorLocation` _returnvalue))
  (`SceneComponent.K2_SetWorldRotation` (`self.Widget`) (`KismetMathLibrary.FindLookAtRotation` (+ _returnvalue_2 (* (`self.GetActorForwardVector` _returnvalue) 500.0)) _returnvalue_2) false false))

(fn `Find`
  (params (ItemToFind :type "/Game/BP/NewGame/EN_GridSkillSets Enum" :default "NewEnumerator0"))
  (returns (Have :type Boolean))
  (return (!= (`KismetArrayLibrary.Array_Find` (`self.Requirements`) ItemToFind) -1)))

(fn `UserConstructionScript`)