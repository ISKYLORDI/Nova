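; Grid-based flammable plant that spreads fire, ignites pawns and burns away.
; While on fire it ignites overlapping player or enemy pawns, though fire-shielded players are spared.
; Each passed turn decrements its fire and runs a spread check in a fixed radius.
; Only damage caused by flammable plants reduces its health; at zero it plays a burst sound, stops the emitter and shrinks away before being destroyed.
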(event `self.ReceiveBeginPlay`
  (bind (_returnvalue_roll _returnvalue_pitch _returnvalue_yaw) (`KismetMathLibrary.BreakRotator` (`KismetMathLibrary.RandomRotator` false)))
  (`parent.ReceiveBeginPlay`)
  (`SceneComponent.K2_SetRelativeRotation` (`self.StaticMesh`) (`KismetMathLibrary.MakeRotator` 0.0 0.0 _returnvalue_yaw) false false))

(event `self.CollisionBox.OnComponentBeginOverlap`
  (params (OverlappedComponent :type "PrimitiveComponent Object Reference") (OtherActor :type "Actor Object Reference") (OtherComp :type "PrimitiveComponent Object Reference") (OtherBodyIndex :type Integer) (bFromSweep :type Boolean) (SweepResult :type "HitResult Structure (by ref)"))
  (bind _asbp_grid_based_player (cast `/Game/BP/NewGame/BP_GridBased_Player` OtherActor)
    (:`then`
      (if (not (> (`/Game/BP/NewGame/BP_GridBased_Player.FireShielded` _asbp_grid_based_player) 0))
        (if (> (`self.OnFire`) 0) :!label _label
          (bind _asbp_grid_based_pawn (cast `/Game/BP/NewGame/BP_GridBasedPawn` OtherActor))
          (`self.Ignited` _asbp_grid_based_pawn 2))))
    (:`CastFailed`
      (cast `/Game/BP/NewGame/BP_GridBasedPawn_Enemy` OtherActor)
      (goto _label))))

(event `self.ReceiveAnyDamage`
  (params (Damage :type "Float (single-precision)") (DamageType :type "DamageType Object Reference") (InstigatedBy :type "Controller Object Reference") (DamageCauser :type "Actor Object Reference"))
  (cast `/Game/BP/NewGame/BP_Grided_FlammablePlants` DamageCauser)
  (bind _output_get (set `self.Health` (- (`self.Health`) Damage)))
  (if (<= _output_get 0.0)
    (`/Engine/EditorBlueprintResources/StandardMacros.DoOnce` false
      (:`Completed`
        (`GameplayStatics.PlaySoundAtLocation` "/Game/Sound/SFX/Skills/Fire_Ground/S_Fire_AOE_Burst_03.S_Fire_AOE_Burst_03" (`self.K2_GetActorLocation`) (struct) 1.0 1.0 0.0 "/Game/Sound/SFX/Att.Att" null null null)
        (`ActorComponent.Deactivate` (`self.FireEmitter`))
        (bind (_direction `_新建轨道_0`) (`Timeline|Timeline` :!via `PlayFromStart`)
          (:`Update`
            (`self.SetActorRelativeScale3D` (`KismetMathLibrary.VLerp` (`KismetMathLibrary.Conv_DoubleToVector` 1.0) (`KismetMathLibrary.Conv_DoubleToVector` 0.0) `_新建轨道_0`)))
          (:`Finished`
            (`self.K2_DestroyActor`)))))))

(event `self.TurnPassed`
  (`parent.TurnPassed`)
  (`self.FireDecrement`)
  (`self.FirespreadCheck` 85.0))

(event `SpawnAnim`
  (bind (_direction `_新建轨道_0`) (`Timeline|Timeline_0` :!via `ReverseFromEnd`)
    (:`Update`
      (bind (_returnvalue_x _returnvalue_y _returnvalue_z) (`KismetMathLibrary.BreakVector` (`KismetMathLibrary.VLerp` (`KismetMathLibrary.Conv_DoubleToVector` 3.5) (`KismetMathLibrary.Conv_DoubleToVector` 0.0) `_新建轨道_0`)))
      (`SceneComponent.SetRelativeScale3D` (`self.StaticMesh`) (`KismetMathLibrary.MakeVector` 2.25 2.25 _returnvalue_z)))))

(fn `UserConstructionScript`
  (`parent.UserConstructionScript`))