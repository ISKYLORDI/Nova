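; Flammable grid actor that bursts into a fire shockwave the first time it takes any damage.
; On damage it spawns a fire-enabled BP_Shockwave, plays fire VFX and sound, and disables its collision.
; A timeline then scales the actor up before destroying it.
; Each passed turn calls the parent's handling and then FireDecrement.
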(event `self.ReceiveAnyDamage`
  (params (Damage :type "Float (single-precision)") (DamageType :type "DamageType Object Reference") (InstigatedBy :type "Controller Object Reference") (DamageCauser :type "Actor Object Reference"))
  (bind _returnvalue (`self.K2_GetActorLocation`))
  (`/Engine/EditorBlueprintResources/StandardMacros.DoOnce` false
    (:`Completed`
      (bind _returnvalue_2 (`|SpawnActorFromClass` "/Game/BP/NewGame/BP_Shockwave.BP_Shockwave_C" (`self.GetTransform`) "Undefined" "MultiplyWithRoot" null null))
      (`/Game/BP/NewGame/BP_Shockwave.SpawnEvent` _returnvalue_2 2.0 150.0 0.0 true false 1.0)
      (`NiagaraFunctionLibrary.SpawnSystemAtLocation` "/Game/VFX/BlinkAndDashVFX/VFX_Niagara/NS_Blink_Fire.NS_Blink_Fire" _returnvalue)
      (`GameplayStatics.PlaySoundAtLocation` "/Game/Sound/SFX/Skills/Fire_Ground/S_Fire_AOE_Burst_02.S_Fire_AOE_Burst_02" _returnvalue (struct) 1.0 1.0 0.0 "/Game/Sound/SFX/Att.Att" null null null)
      (`self.SetActorEnableCollision` false)
      (bind (_direction `_新建轨道_0`) (`Timeline|Timeline` :!via `PlayFromStart`)
        (:`Update`
          (`self.SetActorRelativeScale3D` (`KismetMathLibrary.VLerp` (`KismetMathLibrary.Conv_DoubleToVector` 1.0) (`KismetMathLibrary.Conv_DoubleToVector` 1.5) `_新建轨道_0`)))
        (:`Finished`
          (`self.K2_DestroyActor`))))))

(event `self.TurnPassed`
  (`parent.TurnPassed`)
  (`self.FireDecrement`))

(fn `UserConstructionScript`
  (`parent.UserConstructionScript`))