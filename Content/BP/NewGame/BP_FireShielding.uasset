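; Fire shield actor for the player in a grid-based game, fading in its sphere material on spawn with modifiers set through SpawnEvent.
; MoveEvent updates fire ground or plants at the player's location for Fire or Stun.
; TurnEnd with Force pushes back nearby enemies, found by overlaps with temporary move boxes.
; Trigger fades out and destroys the shield, spawning a shockwave for AOE and converting damage into fire resource for Absorb.
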(event `self.ReceiveBeginPlay`
  (bind _sphere (`self.Sphere`))
  (`GameplayStatics.PlaySound2D` "/Game/Sound/SFX/Skills/S_Shield.S_Shield" 0.6 1.0 0.0 null null)
  (bind _asgrid_player_controller (cast `/Game/BP/NewGame/GridPlayerController` (`GameplayStatics.GetPlayerController` 0)))
  (set `self.Ctrler` _asgrid_player_controller)
  (bind (_direction `_新建轨道_0`) (`Timeline|Timeline` :!via `PlayFromStart`)
    (:`Update`
      (`MeshComponent.SetScalarParameterValueOnMaterials` _sphere "Opacity" `_新建轨道_0`)
      (`MeshComponent.SetScalarParameterValueOnMaterials` _sphere "Intensity" (`KismetMathLibrary.Lerp` 0.0 10.0 `_新建轨道_0`)))))

(event `SpawnEvent`
  (params (Force :type "Float (double-precision)") (Fire :type Boolean) (Stun :type Boolean) (AOE :type Boolean) (Absorb :type Boolean))
  (set `self.Force` Force)
  (set `self.Fire` Fire)
  (set `self.Stun` Stun)
  (set `self.AOE` AOE)
  (set `self.Absorb` Absorb)
  (`self.MoveEvent`))

(event `Trigger`
  (params (Damage :type "Float (double-precision)"))
  (`|ExecutionSequence`
    (:`then_0`
      (bind (_direction `_新建轨道_0`) (`Timeline|Timeline_0` :!via `PlayFromStart`)
        (:`Update`
          (`MeshComponent.SetScalarParameterValueOnMaterials` (`self.Sphere`) "Opacity" `_新建轨道_0`))
        (:`Finished`
          (`self.K2_DestroyActor`))))
    (:`then_1`
      (if (`self.AOE`)
        (bind _returnvalue (`|SpawnActorFromClass` "/Game/BP/NewGame/BP_Shockwave.BP_Shockwave_C" (`KismetMathLibrary.MakeTransform` (`self.K2_GetActorLocation`)) "Undefined" "MultiplyWithRoot" null null))
        (`/Game/BP/NewGame/BP_Shockwave.SpawnEvent` _returnvalue 2.0 150.0 (`self.Force`) (`self.Fire`) (`self.Stun`) 1.0 false false)))
    (:`then_2`
      (if (`self.Absorb`)
        (`/Game/BP/NewGame/BP_GridBased_Player.MoveCost` (`/Game/BP/NewGame/GridPlayerController.BPPlayer` (`self.Ctrler`)) 0.0 (* Damage -0.5) 0.0)))))

(event `MoveEvent`
  (bind _returnvalue (`self.K2_GetActorLocation` (`/Game/BP/NewGame/GridPlayerController.BPPlayer` (`self.Ctrler`))))
  (`|ExecutionSequence`
    (:`then_0`
      (if (`self.Fire`)
        (`/Game/BP/NewGame/GridPlayerController.UpdateFireground` (`self.Ctrler`) _returnvalue false)))
    (:`then_1`
      (if (`self.Stun`)
        (`|ExecutionSequence`
          (:`then_0`
            (`/Game/BP/NewGame/GridPlayerController.UpdatePlants` (`self.Ctrler`) _returnvalue)))))))

(event `TurnEnd`
  (bind _returnvalue (`self.K2_GetActorLocation`))
  (if (> (`self.Force`) 0.0)
    (`/Game/BP/NewGame/BP_GridBased_Player.SpawnBoxesUsingRange` (`/Game/BP/NewGame/GridPlayerController.BPPlayer` (`self.Ctrler`)) 100.0 _returnvalue true false false true)
    (`GameplayStatics.PlaySoundAtLocation` "/Game/Sound/plasmarifle_Cue.plasmarifle_Cue" _returnvalue (struct) 1.0 1.0 0.0 null null null null)
    (`NiagaraFunctionLibrary.SpawnSystemAtLocation` "/Game/VFX/BlinkAndDashVFX/VFX_Niagara/NS_Blink_Fire.NS_Blink_Fire" _returnvalue (struct) (0.3 0.3 0.3))
    (bind _outactors (`GameplayStatics.GetAllActorsOfClass` "/Game/BP/NewGame/BP_MoveBox.BP_MoveBox_C"))
    (for _array_element _outactors
      (for _array_element_2 (`self.GetOverlappingActors` _array_element "/Game/BP/NewGame/BP_GridBasedPawn_Enemy.BP_GridBasedPawn_Enemy_C")
        (bind _asbp_grid_based_pawn_enemy (cast `/Game/BP/NewGame/BP_GridBasedPawn_Enemy` _array_element_2))
        (`/Game/BP/NewGame/BP_GridBasedPawn_Enemy.Pushback` _asbp_grid_based_pawn_enemy 0.0 (`KismetMathLibrary.Round` (`self.Force`)) (`self.K2_GetActorLocation` (`/Game/BP/NewGame/GridPlayerController.BPPlayer` (`self.Ctrler`))) 180.0))
      (`self.K2_DestroyActor` _array_element))))

(fn `UserConstructionScript`)