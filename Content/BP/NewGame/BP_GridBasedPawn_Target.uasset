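; BP_GridBasedPawn_Target is an ignitable fire bowl that acts as a checkpoint and, when flagged End, the level goal.
; Player overlap refills fire and light and saves the revive location to the game instance, then once ignites particles, sound and a point-light timeline.
; End targets also fade fog darkness, blend dark to light post-process, then open the next or current level.
; FocusEvent briefly highlights the bowl via custom depth and a retriggerable delay.
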(event `self.ReceiveBeginPlay`
  (bind _postlight (`self.PostLight`))
  (`parent.ReceiveBeginPlay`)
  (`AudioComponent.AdjustVolume` (`self.Audio`) 0.0 0.01 "Linear")
  (`/Engine/EditorBlueprintResources/StandardMacros.IsValid` _postlight
    (:`Is Valid`
      (set `PostProcessVolume.BlendWeight` 0.0 _postlight)
      (set `PostProcessVolume.BlendWeight` 1.0 (`self.PostDark`)))))

(event `self.ClickBox.OnComponentBeginOverlap`
  (params (OverlappedComponent :type "PrimitiveComponent Object Reference") (OtherActor :type "Actor Object Reference") (OtherComp :type "PrimitiveComponent Object Reference") (OtherBodyIndex :type Integer) (bFromSweep :type Boolean) (SweepResult :type "HitResult Structure (by ref)"))
  (bind _particlesystem (`self.ParticleSystem`))
  (bind _level (`self.Level`))
  (bind _postlight (`self.PostLight`))
  (bind _asbp_grid_based_player (cast `/Game/BP/NewGame/BP_GridBased_Player` OtherActor))
  (set `/Game/BP/NewGame/BP_GridBased_Player.FireCounts` 1.0 _asbp_grid_based_player)
  (`/Game/BP/NewGame/BP_GridBased_Player.ChangeIntensity` _asbp_grid_based_player 10000.0 5000.0)
  (bind _asgi_instance (cast `/Game/BP/NewGame/GI_Instance` (`GameplayStatics.GetGameInstance`)))
  (set `/Game/BP/NewGame/GI_Instance.ReviveLocation` (`self.K2_GetActorLocation` _asbp_grid_based_player) _asgi_instance)
  (`/Engine/EditorBlueprintResources/StandardMacros.DoOnce` false
    (:`Completed`
      (`|ExecutionSequence`
        (:`then_0`
          (`AudioComponent.AdjustVolume` (`self.Audio`) 1.0 1.0 "Linear")
          (bind _returnvalue (`GameplayStatics.GetActorOfClass` "/Game/BP/NewGame/BP_DissolveBlock.BP_DissolveBlock_C"))
          (bind (_direction `_新建轨道_0` `_新建轨道_1`) (`Timeline|时间轴_0` :!via `PlayFromStart`)
            (:`Update`
              (`LightComponent.SetIntensity` (`self.PointLight`) (`KismetMathLibrary.Lerp` 1000.0 30000.0 `_新建轨道_0`))
              (if (`self.End`)
                (`MeshComponent.SetScalarParameterValueOnMaterials` (`/Game/BP/NewGame/BP_DissolveBlock.FogSphere` _returnvalue) "Darkness" (`KismetMathLibrary.Lerp` 1.0 0.0 `_新建轨道_0`))
                (`/Engine/EditorBlueprintResources/StandardMacros.IsValid` _postlight
                  (:`Is Valid`
                    (set `PostProcessVolume.BlendWeight` `_新建轨道_0` _postlight)
                    (set `PostProcessVolume.BlendWeight` (`KismetMathLibrary.Lerp` 1.0 0.0 `_新建轨道_0`) (`self.PostDark`))
                    (set `PostProcessVolume.Settings` (make `PostProcessSettings` :`BloomIntensity` (`KismetMathLibrary.Lerp` 0.5 100.0 `_新建轨道_1`)) _postlight)))))
            (:`Finished`
              (if (`self.End`)
                (`KismetSystemLibrary.Delay` 3.0)
                (bind _returnvalue_2 (`GameplayStatics.GetCurrentLevelName` true))
                (if (`KismetSystemLibrary.IsValidSoftObjectReference` _level)
                  (`GameplayStatics.OpenLevelBySoftObjectPtr` _level)
                  (else
                    (`GameplayStatics.OpenLevel` (`KismetStringLibrary.Conv_StringToName` _returnvalue_2))))))))
        (:`then_1`
          (if (`self.End`)
            (`GameplayStatics.SpawnSound2D` "/Game/Sound/SFX/Motion/S_Ignite_fire_boom_02_Cue.S_Ignite_fire_boom_02_Cue" 1.0 1.0 0.0 null)
            (`KismetSystemLibrary.Delay` 0.6)
            (`ActorComponent.Activate` _particlesystem false)
            (else
              (`GameplayStatics.SpawnSound2D` "/Game/Sound/SFX/Motion/S_Ignite_Fire_boom_01_Cue.S_Ignite_Fire_boom_01_Cue" 1.0 1.0 0.0 null)
              (`ActorComponent.Activate` _particlesystem false))))))))

(event `FocusEvent`
  (bind _bowl_low (`self.Bowl_Low`))
  (`PrimitiveComponent.SetRenderCustomDepth` _bowl_low true)
  (`KismetSystemLibrary.RetriggerableDelay` 0.05)
  (`PrimitiveComponent.SetRenderCustomDepth` _bowl_low false))

(fn `UserConstructionScript`
  (`parent.UserConstructionScript`))