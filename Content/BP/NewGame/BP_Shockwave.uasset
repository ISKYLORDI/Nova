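; Shockwave actor for the grid-based game that hits non-player pawns around it when SpawnEvent fires, then destroys itself.
; DamageInRange uses a per-axis box check to apply Power-scaled damage, pushing enemies back with index-staggered timing and stunning them if Stun is set without Fire.
; A timeline expands and fades the sphere alongside a Niagara burst.
; With Fire, temporary move boxes from the player mark tiles for fire-ground updates.
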(event `self.ReceiveBeginPlay`
  (bind _asgrid_player_controller (cast `/Game/BP/NewGame/GridPlayerController` (`GameplayStatics.GetPlayerController` 0)))
  (set `self.Controller` _asgrid_player_controller))

(event `SpawnEvent`
  (params (Damage :type "Float (double-precision)") (Range :type "Float (double-precision)") (Force :type "Float (double-precision)") (Fire :type Boolean) (Stun :type Boolean) (Power :type "Float (double-precision)" :default 1.0))
  (bind _controller (`self.Controller`))
  (bind _range (`self.Range`))
  (bind _returnvalue (/ _range 50.0))
  (bind _output_get (set `self.Force` Force))
  (bind _output_get_2 (set `self.Damage` Damage))
  (bind _output_get_3 (set `self.Range` Range))
  (set `self.Fire` Fire)
  (set `self.Stun` Stun)
  (set `self.Power` Power)
  (`self.DamageInRange` _output_get_3 _output_get_2 _output_get)
  (`NiagaraFunctionLibrary.SpawnSystemAtLocation` "/Game/VFX/BlinkAndDashVFX/VFX_Niagara/NS_Blink_Fire.NS_Blink_Fire" (`self.K2_GetActorLocation`) (struct) (`KismetMathLibrary.Conv_DoubleToVector` (/ (`self.Range`) 350.0)))
  (`|ExecutionSequence`
    (:`then_0`
      (`TimelineComponent.SetPlayRate` (`self.时间轴`) (/ (`self.Range`) 100.0))
      (bind (_direction `_新建轨道_0`) (`Timeline|时间轴` :!via `PlayFromStart`)
        (:`Update`
          (`self.SetActorScale3D` (`KismetMathLibrary.VLerp` (0.0 0.0 0.0) (`KismetMathLibrary.MakeVector` _returnvalue _returnvalue (/ _range 100.0)) `_新建轨道_0`))
          (`MeshComponent.SetScalarParameterValueOnMaterials` (`self.Sphere`) "Opacity" (`KismetMathLibrary.Lerp` 0.8 0.0 `_新建轨道_0`)))
        (:`Finished`
          (`self.SetActorEnableCollision` false)
          (`KismetSystemLibrary.Delay` 3.0)
          (`self.K2_DestroyActor`))))
    (:`then_1`
      (`KismetSystemLibrary.Delay` 0.25)
      (if (`self.HitEnemy`)
        _))
    (:`then_2`
      (if (`self.Fire`)
        (`/Game/BP/NewGame/BP_GridBased_Player.SpawnBoxesUsingRange` (`/Game/BP/NewGame/GridPlayerController.BPPlayer` (`self.Controller`)) (`self.Range`) (`self.K2_GetActorLocation`) true false true false)
        (bind _outactors (`GameplayStatics.GetAllActorsOfClass` "/Game/BP/NewGame/BP_MoveBox.BP_MoveBox_C"))
        (for _array_element _outactors
          (if (not (`/Game/BP/NewGame/BP_MoveBox.Destroyed` _array_element))
            (`/Game/BP/NewGame/GridPlayerController.UpdateFireground` _controller (`self.K2_GetActorLocation` _array_element) (`self.Stun`))))
        (`/Game/BP/NewGame/GridPlayerController.EliminateBoxes` _controller)))))

(fn `DamageInRange`
  (params (Range :type "Float (double-precision)") (BaseDamage :type "Float (single-precision)") (Movepoints :type "Float (double-precision)"))
  (locals (Hit :type Boolean))
  (bind _outactors (`GameplayStatics.GetAllActorsOfClass` "/Game/BP/NewGame/BP_GridBasedPawn.BP_GridBasedPawn_C"))
  (for (_array_element _array_index) _outactors
    (cast `/Game/BP/NewGame/BP_GridBased_Player` _array_element
      (:`CastFailed`
        (bind (_returnvalue_x _returnvalue_y _returnvalue_z) (`KismetMathLibrary.BreakVector` (`KismetMathLibrary.Vector_GetAbs` (- (`self.K2_GetActorLocation` _array_element) (`self.K2_GetActorLocation`)))))
        (if (and (<= _returnvalue_x Range) (<= _returnvalue_y Range) (<= _returnvalue_z Range))
          (`|ExecutionSequence`
            (:`then_0`
              (bind _asbp_grid_based_pawn_enemy (cast `/Game/BP/NewGame/BP_GridBasedPawn_Enemy` _array_element))
              (`/Game/BP/NewGame/BP_GridBasedPawn_Enemy.Pushback` _asbp_grid_based_pawn_enemy (* _array_index 0.01) (`KismetMathLibrary.Round` Movepoints) (`self.K2_GetActorLocation`))
              (set `self.HitEnemy` true)
              (if (`self.Stun`)
                (if (not (`self.Fire`))
                  (`/Game/BP/NewGame/BP_GridBasedPawn_Enemy.GetStunned` _asbp_grid_based_pawn_enemy (+ (`KismetMathLibrary.Round` (`self.Power`)) 1)))))
            (:`then_1`
              (`GameplayStatics.ApplyDamage` _array_element (* BaseDamage (`self.Power`)) null self)))))))
  (return))

(fn `UserConstructionScript`)