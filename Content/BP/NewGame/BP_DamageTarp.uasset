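; BP_DamageTarp is a one-shot effect actor that randomly raises or lowers a player's FireCounts.
; SpecialEffect runs its logic only while the New flag set on BeginPlay is true, then clears it.
; A weighted roll subtracts 40% of the time and otherwise adds, using a random amount interpolated between XMax and XMin.
; The file contains no call to SpecialEffect, and its overlap and tick events are disabled.
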(event `self.ReceiveBeginPlay`
  (`parent.ReceiveBeginPlay`)
  (set `self.New` true))

(fn `SpecialEffect`
  (params (player :type "/Game/BP/NewGame/BP_GridBased_Player Object Reference"))
  (bind _firecounts (`/Game/BP/NewGame/BP_GridBased_Player.FireCounts` player))
  (bind _returnvalue (`KismetMathLibrary.Lerp` (`self.XMax`) (`self.XMin`) (`KismetMathLibrary.RandomFloat`)))
  (if (`self.New`)
    (set `self.New` false)
    (if (< (`KismetMathLibrary.RandomFloat`) 0.4)
      (set `/Game/BP/NewGame/BP_GridBased_Player.FireCounts` (- _firecounts _returnvalue) player)
      (else
        (set `/Game/BP/NewGame/BP_GridBased_Player.FireCounts` (+ _firecounts _returnvalue) player)))))

(fn `UserConstructionScript`
  (`parent.UserConstructionScript`))