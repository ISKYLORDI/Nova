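; BP_FloatingText is an actor that shows a text string in the world through a widget component hosting W_FloatingText.
; The construction script and BeginPlay both copy the actor's Text variable into the widget.
; Every tick it billboards by rotating to face opposite the player camera's forward vector, so it stays parallel to the view rather than aimed at the camera's position.
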(event `self.ReceiveBeginPlay`
  (bind _asw_floating_text (cast `/Game/BP/NewGame/W_FloatingText` (`WidgetComponent.GetWidget` (`self.Widget`))))
  (set `/Game/BP/NewGame/W_FloatingText.Text` (`self.Text`) _asw_floating_text))

(event `self.ReceiveTick`
  (params (DeltaSeconds :type "Float (single-precision)"))
  (bind _returnvalue (`self.K2_GetActorLocation`))
  (`self.K2_SetActorRotation` (`KismetMathLibrary.FindLookAtRotation` _returnvalue (+ _returnvalue (* (`self.GetActorForwardVector` (`GameplayStatics.GetPlayerCameraManager` 0)) -1.0)))))

(fn `UserConstructionScript`
  (bind _asw_floating_text (cast `/Game/BP/NewGame/W_FloatingText` (`WidgetComponent.GetWidget` (`self.Widget`))))
  (set `/Game/BP/NewGame/W_FloatingText.Text` (`self.Text`) _asw_floating_text))