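; Grid rock obstacle that rises from the ground on spawn and crumbles as damage and passing turns drain its hit points.
; SpawnEvent stores its modifiers, then uses temporary range boxes to apply fire ground, stun or pushback to nearby tiles and enemies.
; Death runs once, spawning a BP_Shockwave carrying those modifiers if Explosive, otherwise a small burst plus fire ground if Fire.
; Tick yaws the health bar toward the camera.
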(event `self.ReceiveBeginPlay`
  (bind _returnvalue (`self.K2_GetActorLocation`))
  (bind _staticmesh (`self.StaticMesh`))
  (bind (_relativelocation_x _relativelocation_y) (`KismetMathLibrary.BreakVector` (`SceneComponent.RelativeLocation` _staticmesh)))
  (`parent.ReceiveBeginPlay`)
  (bind _asgrid_player_controller (cast `/Game/BP/NewGame/GridPlayerController` (`GameplayStatics.GetPlayerController` 0)))
  (set `self.As Grid Player Controller` _asgrid_player_controller)
  (bind _asw_health_bar (cast `/Game/BP/NewGame/W_HealthBar` (`WidgetComponent.GetWidget` (`self.Widget`))))
  (set `/Game/BP/NewGame/W_HealthBar.Pawn` self _asw_health_bar)
  (`|ExecutionSequence`
    (:`then_0`
      (bind (_direction `_新建轨道_0`) (`Timeline|Timeline` :!via `PlayFromStart`)
        (:`Update`
          (`SceneComponent.K2_SetRelativeLocation` _staticmesh (`KismetMathLibrary.MakeVector` _relativelocation_x _relativelocation_y (`KismetMathLibrary.Lerp` -100.0 -20.592808 `_新建轨道_0`)) false false))))
    (:`then_1`
      (`KismetSystemLibrary.Delay` 0.1)
      (`self.SetActorEnableCollision` true))
    (:`then_2`
      (`NiagaraFunctionLibrary.SpawnSystemAtLocation` "/Game/VFX/BlinkAndDashVFX/VFX_Niagara/NS_Dash_Fire.NS_Dash_Fire" _returnvalue (struct :`Pitch` 90.0) (0.2 0.2 0.2))
      (`GameplayStatics.PlaySoundAtLocation` "/Game/Sound/SFX/Skills/Force_Still/S_HoldEnemy_Normal_Cue.S_HoldEnemy_Normal_Cue" _returnvalue (struct) 1.0 1.0 0.0 null null null null))))

(event `self.TurnPassed`
  (`parent.TurnPassed`)
  (bind _output_get (set `self.HitPoints` (- (`self.HitPoints`) 1.0)))
  (if (<= _output_get 0.0)
    (`/Engine/EditorBlueprintResources/StandardMacros.DoOnce` false :!label _label
      (:`Completed`
        (if (`self.Explosive`)
          (`self.DeathExplosion` "/Game/VFX/BlinkAndDashVFX/VFX_Niagara/NS_Blink_Fire.NS_Blink_Fire" "/Game/Sound/SFX/Characters/Chess/S_Chess_Damage_Crush1_Cue.S_Chess_Damage_Crush1_Cue")
          (bind _returnvalue (`|SpawnActorFromClass` "/Game/BP/NewGame/BP_Shockwave.BP_Shockwave_C" (`KismetMathLibrary.MakeTransform` (`self.K2_GetActorLocation`)) "Undefined" "MultiplyWithRoot" null null))
          (`/Game/BP/NewGame/BP_Shockwave.SpawnEvent` _returnvalue 2.0 150.0 (`self.Force`) (`self.Fire`) (`self.Stun`) 1.0 false false)
          (else
            (if (`self.Fire`)
              (`/Game/BP/NewGame/GridPlayerController.UpdateFireground` (`self.As Grid Player Controller`) (`self.K2_GetActorLocation`) false))
            (`self.DeathExplosion` "/Game/VFX/BlinkAndDashVFX/VFX_Niagara/NS_Blink_FireSmall.NS_Blink_FireSmall" "/Game/Sound/SFX/Characters/Chess/S_Chess_Damage_Crush1_Cue.S_Chess_Damage_Crush1_Cue")))))
    (else
      (`GameplayStatics.SpawnEmitterAtLocation` "/Game/VFX/MagicProjectilesVol2/Particles/Muzzles/P_Muzzle_Fireball04_Orange.P_Muzzle_Fireball04_Orange" (`self.K2_GetActorLocation`) (struct :`Pitch` 90.0)))))

(event `self.ReceiveAnyDamage`
  (params (Damage :type "Float (single-precision)") (DamageType :type "DamageType Object Reference") (InstigatedBy :type "Controller Object Reference") (DamageCauser :type "Actor Object Reference"))
  (bind _output_get (set `self.HitPoints` (- (`self.HitPoints`) Damage)))
  (if (<= _output_get 0.0)
    (goto _label)))

(event `self.DeathExplosion`
  (params (SystemTemplate :type "NiagaraSystem Object Reference") (Sound :type "SoundBase Object Reference"))
  (`parent.DeathExplosion` SystemTemplate Sound)
  (goto _label))

(event `SpawnEvent`
  (params (Explosive :type Boolean) (Fire :type Boolean) (Stun :type Boolean) (Force :type "Float (double-precision)") (Absorb :type Boolean))
  (bind _as_grid_player_controller (`self.As Grid Player Controller`))
  (set `self.Explosive` Explosive)
  (set `self.Fire` Fire)
  (set `self.Stun` Stun)
  (bind _output_get (set `self.Force` Force))
  (set `self.Absorb` Absorb)
  (if (or (`self.Fire`) (`self.Stun`) (> _output_get 0.0))
    (bind _returnarray (`/Game/BP/NewGame/BP_GridBased_Player.SpawnBoxesUsingRange` (`/Game/BP/NewGame/GridPlayerController.BPPlayer` (`self.As Grid Player Controller`)) 100.0 (`self.K2_GetActorLocation`) true false false true))
    (for _array_element _returnarray
      (`|ExecutionSequence`
        (:`then_0`
          (for _array_element_2 (`self.GetOverlappingActors` _array_element "/Game/BP/NewGame/BP_GridBasedPawn_Enemy.BP_GridBasedPawn_Enemy_C")
            (bind _asbp_grid_based_pawn_enemy (cast `/Game/BP/NewGame/BP_GridBasedPawn_Enemy` _array_element_2))
            (`|ExecutionSequence`
              (:`then_0`
                (if (`self.Stun`)
                  (`/Game/BP/NewGame/BP_GridBasedPawn_Enemy.GetStunned` _asbp_grid_based_pawn_enemy 1)))
              (:`then_1`
                (if (> (`self.Force`) 0.0)
                  (`/Game/BP/NewGame/BP_GridBasedPawn_Enemy.Pushback` _asbp_grid_based_pawn_enemy 0.0 1 (`self.K2_GetActorLocation`) 180.0 true))))))
        (:`then_1`
          (if (`self.Fire`)
            (bind _returnvalue (`self.K2_GetActorLocation` _array_element))
            (`/Game/BP/NewGame/GridPlayerController.UpdateFireground` _as_grid_player_controller _returnvalue false)))
        (:`then_2`
          (if (`self.Stun`)
            (`/Game/BP/NewGame/GridPlayerController.UpdatePlants` _as_grid_player_controller _returnvalue)))
        (:`then_3`
          (`self.K2_DestroyActor` _array_element))))
    (`|ExecutionSequence`
      (:`then_0`
        (if (`self.Stun`)
          (`GameplayStatics.PlaySoundAtLocation` "/Game/Sound/SFX/Skills/Force_Still/S_HoldEnemy_Normal_Cue.S_HoldEnemy_Normal_Cue" (`self.K2_GetActorLocation`) (struct) 1.0 1.0 0.0 "/Game/Sound/SFX/Att.Att" null null null)))
      (:`then_1`
        (if (`self.Fire`)
          (`GameplayStatics.PlaySoundAtLocation` "/Game/Sound/SFX/Skills/Fire_Ground/S_Fire_AOE_Burst_02.S_Fire_AOE_Burst_02" (`self.K2_GetActorLocation`) (struct) 1.0 1.0 0.0 "/Game/Sound/SFX/Att.Att" null null null)))
      (:`then_2`
        (if (> (`self.Force`) 0.0)
          (`GameplayStatics.PlaySoundAtLocation` "/Game/Sound/plasmarifle_Cue.plasmarifle_Cue" (`self.K2_GetActorLocation`) (struct) 1.0 1.0 0.0 "/Game/Sound/SFX/Att.Att" null null null))))))

(event `self.ReceiveTick`
  (params (DeltaSeconds :type "Float (single-precision)"))
  (bind _returnvalue (`GameplayStatics.GetPlayerCameraManager` 0))
  (bind _returnvalue_2 (`self.K2_GetActorLocation` _returnvalue))
  (bind (_returnvalue_roll _returnvalue_pitch _returnvalue_yaw) (`KismetMathLibrary.BreakRotator` (`KismetMathLibrary.FindLookAtRotation` (+ _returnvalue_2 (* (`self.GetActorForwardVector` _returnvalue) 500.0)) _returnvalue_2)))
  (`SceneComponent.K2_SetWorldRotation` (`self.Widget`) (`KismetMathLibrary.MakeRotator` 0.0 0.0 _returnvalue_yaw) false false)
  (`SceneComponent.K2_SetWorldRotation` (`self.Scene1`) (`KismetMathLibrary.MakeRotator` 0.0 0.0 _returnvalue_yaw) false false))

(fn `UserConstructionScript`
  (`parent.UserConstructionScript`))