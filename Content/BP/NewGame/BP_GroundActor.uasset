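; Ground tile actor for a grid-based level that arranges and dresses itself in its Construction Script.
; When Update is toggled, it snaps to the grid and steps aside or upward while overlapping something.
; Four-direction traces guide that offset and, with GenerateEdges, show trims on open sides, while position parity alternates two meshes in a checkerboard.
; FocusEvent briefly shows a decal and custom-depth highlight, held by retriggerable delay.
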(event `EdgeDetection`
  (`self.UpdateEdgesandNavs`))

(event `self.ReceiveBeginPlay`)

(event `FocusEvent`
  (bind _decal (`self.Decal`))
  (`PrimitiveComponent.SetRenderCustomDepth` (`self.SM_G4`) true)
  (`PrimitiveComponent.SetRenderCustomDepth` (`self.SM_G2`) true)
  (`SceneComponent.SetVisibility` _decal true false)
  (`KismetSystemLibrary.RetriggerableDelay` 0.05)
  (`PrimitiveComponent.SetRenderCustomDepth` (`self.SM_G4`) false)
  (`PrimitiveComponent.SetRenderCustomDepth` (`self.SM_G2`) false)
  (`SceneComponent.SetVisibility` _decal false false))

(fn `4DirectionTrace`
  (params (FrontStart :type "Float (double-precision)") (SideStart :type "Float (double-precision)"))
  (returns (Front :type Boolean) (Back :type Boolean) (Right :type Boolean) (Left :type Boolean))
  (bind _returnvalue (`self.GetActorForwardVector`))
  (bind _returnvalue_2 (`self.GetActorRightVector`))
  (bind _returnvalue_x (`KismetMathLibrary.BreakVector` (`self.GetActorScale3D`)))
  (bind _array (`|MakeArray` (`self.GridedObstacle`) (`self.Player`) :!type "Actor Object Reference"))
  (bind _returnvalue_3 (* SideStart _returnvalue_2))
  (bind _returnvalue_4 (* 99.0 _returnvalue_x))
  (bind _returnvalue_5 (+ (`self.K2_GetActorLocation`) (* _returnvalue FrontStart)))
  (bind _returnvalue_6 (+ (`self.K2_GetActorLocation`) _returnvalue_3))
  (bind _returnvalue_7 (* _returnvalue_4 -1.0))
  (bind (_outhit _returnvalue_8) (`KismetSystemLibrary.LineTraceSingle` _returnvalue_5 (+ _returnvalue_5 (* _returnvalue _returnvalue_4)) "TraceTypeQuery1" false _array))
  (bind (_outhit_2 _returnvalue_9) (`KismetSystemLibrary.LineTraceSingle` (+ (`self.K2_GetActorLocation`) (* FrontStart (`self.GetActorForwardVector`) -1.0)) (+ _returnvalue_5 (* _returnvalue _returnvalue_7)) "TraceTypeQuery1" false _array))
  (bind (_outhit_3 _returnvalue_10) (`KismetSystemLibrary.LineTraceSingle` _returnvalue_6 (+ _returnvalue_6 (* _returnvalue_2 _returnvalue_4)) "TraceTypeQuery1" false _array))
  (bind (_outhit_4 _returnvalue_11) (`KismetSystemLibrary.LineTraceSingle` (+ (`self.K2_GetActorLocation`) (* _returnvalue_3 -1.0)) (+ _returnvalue_6 (* _returnvalue_2 _returnvalue_7)) "TraceTypeQuery1" false _array))
  (return _returnvalue_8 _returnvalue_9 _returnvalue_10 _returnvalue_11))

(fn `TileVariation`
  (bind (_returnvalue_x _returnvalue_y) (`KismetMathLibrary.BreakVector` (`self.K2_GetActorLocation`)))
  (bind _sm_g2 (`self.SM_G2`))
  (bind _sm_g4 (`self.SM_G4`))
  (bind _sm_g2_2 (`self.SM_G2`))
  (bind _sm_g4_2 (`self.SM_G4`))
  (bind _returnvalue (> (mod (`KismetMathLibrary.Abs_Int` (`.ReturnValue` (`KismetMathLibrary.FMod` _returnvalue_y 100.0))) 2) 0))
  (if (> (mod (`KismetMathLibrary.Abs_Int` (`.ReturnValue` (`KismetMathLibrary.FMod` _returnvalue_x 100.0))) 2) 0)
    (if _returnvalue
      (`SceneComponent.SetVisibility` _sm_g2 true false)
      (`SceneComponent.SetVisibility` _sm_g4 false false)
      (else
        (`SceneComponent.SetVisibility` _sm_g2 false false)
        (`SceneComponent.SetVisibility` _sm_g4 true false)))
    (elif _returnvalue
      (`SceneComponent.SetVisibility` _sm_g2_2 false false)
      (`SceneComponent.SetVisibility` _sm_g4_2 true false)
      (else
        (`SceneComponent.SetVisibility` _sm_g2_2 true false)
        (`SceneComponent.SetVisibility` _sm_g4_2 false false)))))

(fn `TraceOverlappedGround`
  (returns (Overlapped :type Boolean))
  (bind _returnvalue (`self.K2_GetActorLocation`))
  (bind (_outhit _returnvalue_2) (`KismetSystemLibrary.SphereTraceSingle` _returnvalue _returnvalue 20.0 "TraceTypeQuery1"))
  (if _returnvalue_2
    (return true)
    (else
      (return false))))

(fn `TraceStandingActor`
  (returns (ReturnValue :type Boolean) (HitActor :type "Actor Object Reference"))
  (bind (_outhit _returnvalue) (`KismetSystemLibrary.LineTraceSingle` :`Start` (+ (`self.K2_GetActorLocation`) (0.0 0.0 1.0)) :`End` (+ (`self.K2_GetActorLocation`) (0.0 0.0 50.0)) :`TraceChannel` "TraceTypeQuery1" :`DrawTime` 1.0))
  (return _returnvalue (`.HitActor` (`GameplayStatics.BreakHitResult` _outhit))))

(fn `UpdateEdgesandNavs`
  (bind (_front _back _right _left) (`self.4DirectionTrace` 0.0))
  (`SceneComponent.SetVisibility` (`self.TrimF`) (not _front) true)
  (`SceneComponent.SetVisibility` (`self.TrimB`) (not _back) true)
  (`SceneComponent.SetVisibility` (`self.TrimR`) (not _right) true)
  (`SceneComponent.SetVisibility` (`self.TrimL`) (not _left) true))

(fn `UserConstructionScript`
  (locals (Obstacle :type "/Game/BP/NewGame/BP_GridedObstacle Object Reference"))
  (bind _returnvalue (`self.K2_GetActorLocation`))
  (bind (_returnvalue_x _returnvalue_y _returnvalue_z) (`KismetMathLibrary.BreakVector` (`self.K2_GetActorLocation`)))
  (bind (_front _back _right _left) (`self.4DirectionTrace` 50.0 50.0))
  (bind (_remainder _returnvalue_2) (`KismetMathLibrary.FMod` _returnvalue_z 50.0))
  (bind (_remainder_2 _returnvalue_3) (`KismetMathLibrary.FMod` _returnvalue_x 100.0))
  (bind (_remainder_3 _returnvalue_4) (`KismetMathLibrary.FMod` _returnvalue_y 100.0))
  (`PrimitiveComponent.SetMaterial` (`self.SM_G4`) 0 (select `bool` (`self.Bricks`) :`false` "/Game/Meshes/Materials/M_g.M_g" :`true` "/Game/Meshes/Materials/M_g_2.M_g_2" :!type "MaterialInterface Object Reference"))
  (bind _returnvalue_5 (`GameplayStatics.GetActorOfClass` "/Game/BP/NewGame/BP_GridBased_Player.BP_GridBased_Player_C"))
  (set `self.Player` _returnvalue_5)
  (bind _outhit (`KismetSystemLibrary.LineTraceSingle` _returnvalue (+ _returnvalue (0.0 0.0 -50.0)) "TraceTypeQuery1"))
  (bind _asbp_grided_obstacle (cast `/Game/BP/NewGame/BP_GridedObstacle` (`.HitActor` (`GameplayStatics.BreakHitResult` _outhit)))
    (:`then`
      (set `self.GridedObstacle` _asbp_grided_obstacle))
    (:`CastFailed`
      _))
  (`|ExecutionSequence`
    (:`then_0`
      (if (`self.Update`)
        (set `self.Update` false)
        (`self.K2_SetActorLocation` (`KismetMathLibrary.MakeVector` (`KismetMathLibrary.Conv_IntToDouble` (* (+ (`KismetMathLibrary.Round64` (/ _remainder_2 100.0)) _returnvalue_3) 100)) (`KismetMathLibrary.Conv_IntToDouble` (* (+ (`KismetMathLibrary.Round64` (/ _remainder_3 100.0)) _returnvalue_4) 100)) (`KismetMathLibrary.Conv_IntToDouble` (* (+ (`KismetMathLibrary.Round64` (/ _remainder 50.0)) _returnvalue_2) 50))) :!label _label)
        (if (`self.TraceOverlappedGround`)
          (`self.K2_AddActorWorldOffset` (select `bool` _front :`false` (100.0 0.0 0.0) :`true` (select `bool` _right :`false` (0.0 100.0 0.0) :`true` (select `bool` _left :`false` (0.0 -100.0 0.0) :`true` (select `bool` _back :`false` (-100.0 0.0 0.0) :`true` (0.0 0.0 50.0) :!type "Vector Structure")))))
          (goto _label)
          (else
            (if (`self.GenerateEdges`) :!label _label_2
              (`self.UpdateEdgesandNavs`)
              (else
                (`SceneComponent.SetVisibility` (`self.TrimR`) false false)
                (`SceneComponent.SetVisibility` (`self.TrimB`) false false)
                (`SceneComponent.SetVisibility` (`self.TrimF`) false false)
                (`SceneComponent.SetVisibility` (`self.TrimL`) false false)))))))
    (:`then_1`
      (goto _label_2))
    (:`then_2`
      (`self.TileVariation`))))