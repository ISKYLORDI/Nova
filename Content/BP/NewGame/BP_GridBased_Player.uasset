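; Player pawn for a turn-based grid game where fire level is health, also driving light and vision dissolver size.
; Line traces place preview boxes on valid neighboring tiles, allowing one-level height steps, until move points run out.
; EndTurn clears boxes and starts the first enemy's move; PlayerEnd restores boxes and ticks down the damage-halving fire shield.
; A looping timer keeps the dissolver on the player or active fireball; death reloads the level.
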(event `self.ReceiveBeginPlay`
  (bind _asgrid_player_controller (cast `/Game/BP/NewGame/GridPlayerController` (`GameplayStatics.GetPlayerController` 0)))
  (set `self.Player Controller` _asgrid_player_controller)
  (`self.SpawnMoveBoxes` 0.0)
  (bind _returnvalue (`|CreateWidget` "/Game/BP/NewGame/W_Firebar.W_Firebar_C"))
  (`UserWidget.AddToViewport` _returnvalue 0)
  (set `self.MovePoints` (`KismetMathLibrary.Conv_IntToDouble` (`self.InitialMovepoints`)))
  (bind _returnvalue_2 (`|SpawnActorFromClass` "/Game/BP/NewGame/BP_DissolveBlock.BP_DissolveBlock_C" (`KismetMathLibrary.MakeTransform` (0.0 0.0 0.0)) "Undefined" "MultiplyWithRoot" null null))
  (set `self.Dissolver` _returnvalue_2)
  (`self.K2_AttachToActor` _returnvalue_2 self "None" "SnapToTarget" "KeepRelative" "KeepRelative" true)
  (`KismetSystemLibrary.K2_SetTimer` null "UpdateEnemyVisibility" 0.1 true)
  (`self.UpdateEnemyVisibility`)
  (set `self.RotateModel` (`self.Char`))
  (set `self.IsFromTeleport` false))

(event `self.ReceiveAnyDamage`
  (params (Damage :type "Float (single-precision)") (DamageType :type "DamageType Object Reference") (InstigatedBy :type "Controller Object Reference") (DamageCauser :type "Actor Object Reference"))
  (bind _output_get (set `self.FireCounts` (`KismetMathLibrary.FClamp` (- (`self.FireCounts`) (* Damage (`self.DamageMultiplier`))))))
  (if (<= _output_get 0.0)
    (`self.Death`)))

(event `self.CollisionBox.OnComponentBeginOverlap`
  (params (OverlappedComponent :type "PrimitiveComponent Object Reference") (OtherActor :type "Actor Object Reference") (OtherComp :type "PrimitiveComponent Object Reference") (OtherBodyIndex :type Integer) (bFromSweep :type Boolean) (SweepResult :type "HitResult Structure (by ref)"))
  (cast `/Game/BP/NewGame/BP_GridBasedPawn_Enemy` OtherActor))

(event `Death`
  (`/Engine/EditorBlueprintResources/StandardMacros.DoOnce` false
    (:`Completed`
      (bind _returnvalue (`GameplayStatics.GetActorOfClass` "/Game/BP/Nova/BP_Camera.BP_Camera_C"))
      (`self.K2_SetActorLocation` _returnvalue (`self.K2_GetActorLocation`) false false)
      (`KismetSystemLibrary.Delay` 1.5)
      (bind _returnvalue_2 (`GameplayStatics.GetCurrentLevelName` true))
      (`GameplayStatics.OpenLevel` (`KismetStringLibrary.Conv_StringToName` _returnvalue_2)))))

(event `SpawnMoveBoxes`
  (params (Delay :type "Float (single-precision)"))
  (if (not (>= (`self.MovedTimes`) (`self.MovePoints`)))
    (`KismetSystemLibrary.Delay` Delay)
    (for _index (range 1 2)
      (set `self.SpawnBoxIndex` _index)
      (`self.SpawnBoxes` (`self.GetActorForwardVector`) (* (`self.MoveDistance`) (`self.SpawnBoxIndex`)))
      (`self.SpawnBoxes` (`self.GetActorForwardVector`) (* (* (`self.MoveDistance`) -1.0) (`self.SpawnBoxIndex`)))
      (`self.SpawnBoxes` (`self.GetActorRightVector`) (* (`self.MoveDistance`) (`self.SpawnBoxIndex`)))
      (`self.SpawnBoxes` (`self.GetActorRightVector`) (* (* (`self.MoveDistance`) -1.0) (`self.SpawnBoxIndex`)))
      (`self.SpawnBoxes` (+ (`self.GetActorForwardVector`) (`self.GetActorRightVector`)) (* (`self.MoveDistance`) (`self.SpawnBoxIndex`)))
      (`self.SpawnBoxes` (+ (* (`self.GetActorForwardVector`) -1.0) (`self.GetActorRightVector`)) (* (`self.MoveDistance`) (`self.SpawnBoxIndex`)))
      (`self.SpawnBoxes` (+ (`self.GetActorForwardVector`) (* (`self.GetActorRightVector`) -1.0)) (* (`self.MoveDistance`) (`self.SpawnBoxIndex`)))
      (`self.SpawnBoxes` (+ (`self.GetActorForwardVector`) (`self.GetActorRightVector`)) (* (* (`self.MoveDistance`) -1.0) (`self.SpawnBoxIndex`))))))

(event `MoveCost`
  (params (SkillCost :type "Float (double-precision)" :default 0.0) (FireCost :type "Float (double-precision)" :default 0.05) (MoveCost :type "Float (double-precision)" :default 1.0))
  (set `self.MovedTimes` (+ MoveCost (`self.MovedTimes`)))
  (set `self.SkillMove` (+ (`self.SkillMove`) SkillCost))
  (bind _output_get (set `self.FireCounts` (`KismetMathLibrary.FClamp` (- (`self.FireCounts`) FireCost))))
  (`self.ChangeIntensity` (+ (* _output_get 3000.0) 1000.0) (* _output_get 5000.0))
  (`self.SpawnMoveBoxes` 0.2))

(event `ChangeIntensity`
  (params (TargetIntensity :type "Float (double-precision)") (NewRadius :type "Float (single-precision)"))
  (bind _pointlight (`self.PointLight`))
  (set `self.CurrentIntensity` (`LightComponentBase.Intensity` _pointlight))
  (set `self.CurrentRadius` (`LocalLightComponent.AttenuationRadius` _pointlight))
  (bind (_direction `_新建轨道_0`) (`Timeline|时间轴_0_0` :!via `PlayFromStart`)
    (:`Update`
      (`LightComponent.SetIntensity` _pointlight (`KismetMathLibrary.Lerp` (`self.CurrentIntensity`) TargetIntensity `_新建轨道_0`))
      (`LocalLightComponent.SetAttenuationRadius` _pointlight (`KismetMathLibrary.Lerp` (`self.CurrentRadius`) NewRadius `_新建轨道_0`)))))

(event `EndTurn`
  ;[1 1 1] EndTurn
  (`/Engine/EditorBlueprintResources/StandardMacros.DoOnce` false :!label _label
    (:`Completed`
      (set `self.MovedTimes` 0.0)
      (set `self.SkillMove` 0.0)
      (set `self.MovePoints` (`KismetMathLibrary.Conv_IntToDouble` (`self.InitialMovepoints`)))
      (bind _outactors (`GameplayStatics.GetAllActorsOfClass` "/Game/BP/NewGame/BP_GridBasedPawn_Enemy.BP_GridBasedPawn_Enemy_C"))
      (bind _output_get (set `self.EnemyTurns` _outactors))
      (`/Game/BP/NewGame/GridPlayerController.EliminateBoxes` (`self.Player Controller`))
      (`/Game/BP/NewGame/BP_GridBasedPawn_Enemy.EnemyMove` (`|GetArrayItem` _output_get) 0.1))))

(event `Reset Endturn`
  ;[1 1 1] EndTurn
  (goto _label :!via `Reset`))

(event `PlayerEnd`
  ;[1 1 1] EndTurn
  (`self.SpawnMoveBoxes` 0.0)
  (`KismetSystemLibrary.Delay` 0.2)
  (`self.Reset Endturn`)
  (`self.ShieldDecrease`))

(event `Teleport`
  (params (NewLocation :type "Vector Structure"))
  (bind (_direction `_新建轨道_0`) (`Timeline|时间轴_1` :!via `PlayFromStart`)
    (:`Update`
      (`self.SetActorRelativeScale3D` (`KismetMathLibrary.Conv_DoubleToVector` `_新建轨道_0`)))
    (:`Finished`
      (`self.K2_SetActorLocation` NewLocation)
      (bind (_direction_2 `_新建轨道_0_2`) (`Timeline|时间轴_2` :!via `ReverseFromEnd`)
        (:`Update`
          (`self.SetActorRelativeScale3D` (`KismetMathLibrary.Conv_DoubleToVector` `_新建轨道_0_2`)))))))

(event `FireShield`
  (params (Turns :type Integer))
  (bind _sphere (`self.Sphere`))
  ;[1 1 1] 火焰护盾
  (set `self.DamageMultiplier` 0.5)
  (set `self.FireShielded` (+ (`self.FireShielded`) Turns))
  (`SceneComponent.SetVisibility` (`self.Sphere`) true false)
  (bind (_direction `_新建轨道_0`) (`Timeline|时间轴_3` :!via `PlayFromStart`)
    (:`Update`
      (`MeshComponent.SetScalarParameterValueOnMaterials` _sphere "Opacity" `_新建轨道_0`)
      (`MeshComponent.SetScalarParameterValueOnMaterials` _sphere "Intensity" (`KismetMathLibrary.Lerp` 0.0 10.0 `_新建轨道_0`)))))

(event `ShieldDecrease`
  (bind _fireshielded (`self.FireShielded`))
  (bind _sphere (`self.Sphere`))
  ;[1 1 1] 火焰护盾
  (if (> _fireshielded 0)
    (bind _output_get (set `self.FireShielded` (`KismetMathLibrary.Clamp` (- _fireshielded 1) 0 10)))
    (if (not (> _output_get 0))
      (set `self.DamageMultiplier` 1.0)
      (`SceneComponent.SetVisibility` _sphere true false)
      (bind (_direction `_新建轨道_0`) (`Timeline|时间轴_4` :!via `PlayFromStart`)
        (:`Update`
          (`MeshComponent.SetScalarParameterValueOnMaterials` _sphere "Opacity" `_新建轨道_0`))))))

(fn `SpawnBoxes`
  (params (Direction :type "Vector Structure") (Distance :type "Float (double-precision)"))
  (bind _returnvalue (`self.K2_GetActorLocation`))
  (bind _spawnboxindex (`self.SpawnBoxIndex`))
  (bind _returnvalue_2 (+ _returnvalue (* Direction Distance)))
  (bind _returnvalue_3 (+ _returnvalue_2 (0.0 0.0 100.0)))
  (bind _outhit (`KismetSystemLibrary.LineTraceSingle` (+ _returnvalue_2 (0.0 0.0 150.0)) (+ _returnvalue_2 (0.0 0.0 -150.0)) "TraceTypeQuery1"))
  (cast `/Game/BP/NewGame/BP_GridBasedPawn_Enemy` (`.HitActor` (`GameplayStatics.BreakHitResult` _outhit))
    (:`CastFailed`
      (bind (_outhit_2 _returnvalue_4) (`KismetSystemLibrary.LineTraceSingle` _returnvalue _returnvalue_2 "TraceTypeQuery1"))
      (if _returnvalue_4
        (bind (_outhit_3 _returnvalue_5) (`KismetSystemLibrary.LineTraceSingle` _returnvalue_3 (+ _returnvalue_2 (0.0 0.0 50.1)) "TraceTypeQuery1"))
        (if _returnvalue_5
          _
          (elif (> _spawnboxindex 1)
            (bind (_outhit_4 _returnvalue_6) (`KismetSystemLibrary.LineTraceSingle` _returnvalue_3 (+ _returnvalue_3 (* (`KismetMathLibrary.GetDirectionUnitVector` _returnvalue_3 (+ (`self.K2_GetActorLocation`) (0.0 0.0 100.0))) (* (`self.MoveDistance`) _spawnboxindex))) "TraceTypeQuery1"))
            (if (not _returnvalue_6)
              (bind _returnvalue_7 (`|SpawnActorFromClass` "/Game/BP/NewGame/BP_PreviewBox.BP_PreviewBox_C" (`KismetMathLibrary.MakeTransform` _returnvalue_3) "Undefined" "MultiplyWithRoot" null null :!label _label))
              (set `/Game/BP/NewGame/BP_PreviewBox.OwnerActor` self _returnvalue_7))
            (else
              (goto _label))))
        (else
          (bind (_outhit_5 _returnvalue_8) (`KismetSystemLibrary.LineTraceSingle` _returnvalue_2 (+ _returnvalue_2 (0.0 0.0 -101.0)) "TraceTypeQuery1"))
          (if _returnvalue_8
            (bind _returnvalue_9 (`|SpawnActorFromClass` "/Game/BP/NewGame/BP_PreviewBox.BP_PreviewBox_C" (`KismetMathLibrary.MakeTransform` _returnvalue_2) "Undefined" "MultiplyWithRoot" null null))
            (set `/Game/BP/NewGame/BP_PreviewBox.OwnerActor` self _returnvalue_9)
            (else
              (bind (_outhit_6 _returnvalue_10) (`KismetSystemLibrary.LineTraceSingle` _returnvalue_2 (+ _returnvalue_2 (0.0 0.0 -201.0)) "TraceTypeQuery1"))
              (if _returnvalue_10
                (bind _returnvalue_11 (`|SpawnActorFromClass` "/Game/BP/NewGame/BP_PreviewBox.BP_PreviewBox_C" (`KismetMathLibrary.MakeTransform` (+ _returnvalue_2 (0.0 0.0 -100.0))) "Undefined" "MultiplyWithRoot" null null))
                (set `/Game/BP/NewGame/BP_PreviewBox.OwnerActor` self _returnvalue_11)))))))))

(fn `UpdateEnemyVisibility`
  (bind _dissolver (`self.Dissolver`))
  (bind _returnvalue (`KismetMathLibrary.Lerp` 2.0 10.0 (`self.FireCounts`)))
  (bind _spawnedfireball (`/Game/BP/NewGame/GridPlayerController.SpawnedFireball` (`self.Player Controller`)))
  (set `self.ViewRange` (+ (* _returnvalue 100.0) 100.0))
  (`self.SetActorScale3D` (`self.Dissolver`) (`KismetMathLibrary.Conv_DoubleToVector` _returnvalue))
  (`/Engine/EditorBlueprintResources/StandardMacros.IsValid` _spawnedfireball
    (:`Is Valid`
      (`self.K2_SetActorLocation` _dissolver (`self.K2_GetActorLocation` _spawnedfireball) false false))
    (:`Is Not Valid`
      (`self.K2_SetActorLocation` _dissolver (`self.K2_GetActorLocation`) false false))))

(fn `UserConstructionScript`
  (`SceneComponent.K2_SetWorldLocation` (`self.PointLight`) (`SceneComponent.K2_GetComponentLocation` (`self.FireAttachment`)) false false))