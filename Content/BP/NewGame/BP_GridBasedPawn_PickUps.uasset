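; Skill pickup that grants the player a skill button when BP_GridBased_Player overlaps its ClickBox, detected by both overlap event and delayed Tick check.
; Construction builds a dynamic material showing the SkillIndex icon.
; Pickup runs once, fading out via timeline before destroying itself.
; CombineSlot adds an unconfigured button to SkillBoxCombined; otherwise it appends a configured, key-numbered button to SkillBox, or fills the first empty slot once over four exist.
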(event `self.ReceiveBeginPlay`
  (`parent.ReceiveBeginPlay`))

(event `self.ReceiveTick`
  (params (DeltaSeconds :type "Float (single-precision)"))
  (bind _mid (`self.MID`))
  (`KismetSystemLibrary.Delay` 0.1)
  (bind _returnvalue (`GameplayStatics.GetActorOfClass` "/Game/BP/NewGame/BP_GridBased_Player.BP_GridBased_Player_C"))
  (if (`PrimitiveComponent.IsOverlappingActor` (`self.ClickBox`) _returnvalue)
    (`/Engine/EditorBlueprintResources/StandardMacros.DoOnce` false :!label _label
      (:`Completed`
        (bind _returnvalue_2 (`GameplayStatics.GetActorOfClass` "/Game/BP/NewGame/BP_GridBased_Player.BP_GridBased_Player_C"))
        (`|ExecutionSequence`
          (:`then_0`
            (`TimelineComponent.SetPlayRate` (`self.时间轴_1`) 5.0)
            (bind (_direction `_新建轨道_1`) (`Timeline|时间轴_0` :!via `PlayFromStart`)
              (:`Update`
                (`MaterialInstanceDynamic.SetScalarParameterValue` _mid "Opacity" `_新建轨道_1`)
                (`MaterialInstanceDynamic.SetScalarParameterValue` _mid "Intensity" (`KismetMathLibrary.Lerp` 5.0 1.0 `_新建轨道_1`)))
              (:`Finished`
                (`self.K2_DestroyActor`))))
          (:`then_1`
            (if (`self.CombineSlot`)
              (bind _returnvalue_3 (`|CreateWidget` "/Game/BP/NewGame/W_skillbutton.W_skillbutton_C"))
              (bind _playerui (`/Game/BP/NewGame/BP_GridBased_Player.PlayerUI` _returnvalue_2))
              (`PanelWidget.AddChild` (`/Game/BP/NewGame/W_Firebar.SkillBoxCombined` _playerui) _returnvalue_3)
              (else
                (bind _skillbox (`/Game/BP/NewGame/W_Firebar.SkillBox` _playerui))
                (bind _returnvalue_4 (`PanelWidget.GetAllChildren` _skillbox))
                (if (> (`KismetArrayLibrary.Array_Length` _returnvalue_4) 4)
                  (`self.SetSlotSkill` _returnvalue_4)
                  (else
                    (bind _returnvalue_5 (`|CreateWidget` "/Game/BP/NewGame/W_skillbutton.W_skillbutton_C"))
                    (`PanelWidget.AddChild` _skillbox _returnvalue_5)
                    (set `/Game/BP/NewGame/W_skillbutton.SkillIndex` (`self.SkillIndex`) _returnvalue_5)
                    (`/Game/BP/NewGame/W_skillbutton.UpdateButtonOutlook` _returnvalue_5)
                    (set `/Game/BP/NewGame/W_skillbutton.KeyBinding` (`KismetTextLibrary.Conv_IntToText` (`PanelWidget.GetChildrenCount` _skillbox)) _returnvalue_5)))))))))))

(event `self.ClickBox.OnComponentBeginOverlap`
  (params (OverlappedComponent :type "PrimitiveComponent Object Reference") (OtherActor :type "Actor Object Reference") (OtherComp :type "PrimitiveComponent Object Reference") (OtherBodyIndex :type Integer) (bFromSweep :type Boolean) (SweepResult :type "HitResult Structure (by ref)"))
  (cast `/Game/BP/NewGame/BP_GridBased_Player` OtherActor)
  (goto _label))

(fn `SetSlotSkill`
  (params (Array :type "Array of Widget Object Reference"))
  (for _array_element Array
    (bind _asw_skillbutton (cast `/Game/BP/NewGame/W_skillbutton` _array_element))
    (if (== (`/Game/BP/NewGame/W_skillbutton.SkillIndex` _asw_skillbutton) 0)
      (`/Engine/EditorBlueprintResources/StandardMacros.DoOnce` false
        (:`Completed`
          (set `/Game/BP/NewGame/W_skillbutton.SkillIndex` (`self.SkillIndex`) _asw_skillbutton)
          (`/Game/BP/NewGame/W_skillbutton.UpdateButtonOutlook` _asw_skillbutton))))))

(fn `UserConstructionScript`
  (`parent.UserConstructionScript`)
  (bind _returnvalue (`PrimitiveComponent.CreateDynamicMaterialInstance` (`self.Plane`) 0 "/Game/Materials/M_SkillButton.M_SkillButton" "None"))
  (bind _output_get (set `self.MID` _returnvalue))
  (`MaterialInstanceDynamic.SetScalarParameterValue` _output_get "Opacity" 1.0)
  (`MaterialInstanceDynamic.SetScalarParameterValue` _output_get "Intensity" 3.0)
  (`MaterialInstanceDynamic.SetTextureParameterValue` _output_get "Image" (select `int` (`self.SkillIndex`) :`0` "/Game/BP/NewGame/UI/UI_Transparent.UI_Transparent" :`1` "/Game/BP/NewGame/UI/UI_Dash.UI_Dash" :`2` "/Game/BP/NewGame/UI/UI_Shield.UI_Shield" :`3` "/Game/BP/NewGame/UI/UI_Teleport.UI_Teleport" :`4` "/Game/BP/NewGame/UI/UI_HoldEnemy.UI_HoldEnemy" :`5` "/Game/BP/NewGame/UI/UI_FireGround.UI_FireGround" :`6` "/Game/BP/NewGame/UI/UI_Explosion.UI_Explosion" :`7` "/Game/BP/NewGame/UI/UI_BigFireBall.UI_BigFireBall" :`8` "/Game/BP/NewGame/UI/UI_SmallFireBall.UI_SmallFireBall" :!type "Texture Object Reference"))
  (`MaterialInstanceDynamic.SetTextureParameterValue` _output_get "Mask" (select `int` (`self.SkillIndex`) :`0` "/Game/BP/NewGame/UI/UI_Transparent.UI_Transparent" :`1` "/Game/BP/NewGame/UI/1.1" :`2` "/Game/BP/NewGame/UI/2.2" :`3` "/Game/BP/NewGame/UI/7.7" :`4` "/Game/BP/NewGame/UI/5.5" :`5` "/Game/BP/NewGame/UI/6.6" :`6` "/Game/BP/NewGame/UI/8.8" :`7` "/Game/BP/NewGame/UI/4.4" :`8` "/Game/BP/NewGame/UI/UI_SmallFireBall.UI_SmallFireBall" :!type "Texture Object Reference")))