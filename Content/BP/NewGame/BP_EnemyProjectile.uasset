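; Enemy projectile that homes on a spawned invisible or marker target actor and damages the grid-based player on hit.
; It spawns a homing target at BeginPlay with collision off, then TargetSet moves that target, enables collision and sets strong homing acceleration.
; A player overlap or tick-based proximity check triggers one-time damage, a particle burst and cleanup.
; Dissapate removes it only if unlaunched; the scale timelines are never triggered.
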(event `TargetSet`
  (params (NewLocation :type "Vector Structure"))
  (`self.K2_SetActorLocation` (`self.HomingActor`) NewLocation false false)
  (set `self.Launched` true)
  (set `ProjectileMovementComponent.HomingAccelerationMagnitude` 10000.0 (`self.ProjectileMovement`))
  (`self.SetActorEnableCollision` true))

(event `self.ReceiveBeginPlay`
  (bind _returnvalue_location (`KismetMathLibrary.BreakTransform` (`self.GetTransform`)))
  (`self.SetActorEnableCollision` false)
  (bind _returnvalue (`|SpawnActorFromClass` "/Game/BP/Nova/BP_HomingTarget.BP_HomingTarget_C" (`KismetMathLibrary.MakeTransform` _returnvalue_location) "Undefined" "MultiplyWithRoot" null null))
  (bind _output_get (set `self.HomingActor` _returnvalue))
  (set `ProjectileMovementComponent.HomingTargetComponent` (`Actor.RootComponent` _output_get) (`self.ProjectileMovement`))
  (set `self.Initial Scale` (`self.GetActorScale3D`))
  (bind _returnvalue_2 (`GameplayStatics.GetActorOfClass` "/Game/BP/NewGame/BP_GridBased_Player.BP_GridBased_Player_C"))
  (set `self.Player` _returnvalue_2))

(event `Dissapate`
  (if (not (`self.Launched`))
    (`self.SetActorEnableCollision` false :!label _label)
    (`/Engine/EditorBlueprintResources/StandardMacros.IsValid` (`self.HomingActor`)
      (:`Is Valid`
        (`self.K2_DestroyActor`))
      (:`Is Not Valid`
        _))
    (`self.K2_DestroyActor`)))

(event `self.Sphere.OnComponentBeginOverlap`
  (params (OverlappedComponent :type "PrimitiveComponent Object Reference") (OtherActor :type "Actor Object Reference") (OtherComp :type "PrimitiveComponent Object Reference") (OtherBodyIndex :type Integer) (bFromSweep :type Boolean) (SweepResult :type "HitResult Structure (by ref)"))
  (bind _returnvalue (`self.K2_GetActorLocation`))
  (bind _player (`self.Player`))
  (cast `/Game/BP/NewGame/BP_GridBased_Player` OtherActor)
  (`/Engine/EditorBlueprintResources/StandardMacros.DoOnce` false :!label _label_2
    (:`Completed`
      (`GameplayStatics.ApplyDamage` _player 0.15 null self)
      (`GameplayStatics.SpawnEmitterAtLocation` "/Game/VFX/MagicProjectilesVol2/Particles/Muzzles/P_Muzzle_Blackhole01_Purple.P_Muzzle_Blackhole01_Purple" _returnvalue (`KismetMathLibrary.FindLookAtRotation` (`self.K2_GetActorLocation` _player) _returnvalue) (* (`self.GetActorScale3D`) 0.5))
      (goto _label))))

(event `self.ReceiveTick`
  (params (DeltaSeconds :type "Float (single-precision)"))
  (if (and (`self.Launched`) (<= (`KismetMathLibrary.Vector_Distance` (`self.K2_GetActorLocation` (`self.Player`)) (`self.K2_GetActorLocation`)) 20.0))
    (goto _label_2)))

(fn `UserConstructionScript`)