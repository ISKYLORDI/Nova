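; BP_GroundGenerator is a walker that procedurally lays SM_GroundActor tiles from BeginPlay, up to MaxGenerating iterations.
; Each iteration spawns a tile unless a sphere trace finds a hit, with a short delay after each spawn.
; Four line traces steer it to the first clear side (front, right, left, back), or upward if all are blocked.
; When all four traces hit after a move, it stops and runs EdgeDetection on every spawned tile.
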(event `self.ReceiveBeginPlay`
  (bind (_front _back _right _left) (`self.4DirectionTrace` 50.0 50.0))
  (`/Engine/EditorBlueprintResources/StandardMacros.Do N` (`self.MaxGenerating`) :!label _label
    (:`Exit`
      (if (not (`self.TraceOverlappedGround`))
        (bind _returnvalue (`|SpawnActorFromClass` "/Game/BP/NewGame/SM_GroundActor.SM_GroundActor_C" (`self.GetTransform`) "Undefined" "MultiplyWithRoot" null null))
        (`KismetArrayLibrary.Array_Add` (`self.Grounds`) _returnvalue)
        (`KismetSystemLibrary.Delay` 0.02))
      (`self.K2_AddActorWorldOffset` (select `bool` _front :`false` (100.0 0.0 0.0) :`true` (select `bool` _right :`false` (0.0 100.0 0.0) :`true` (select `bool` _left :`false` (0.0 -100.0 0.0) :`true` (select `bool` _back :`false` (-100.0 0.0 0.0) :`true` (0.0 0.0 50.0) :!type "Vector Structure")))))
      (if (and _front _back _right _left)
        (for _array_element (`self.Grounds`)
          (`/Game/BP/NewGame/SM_GroundActor.EdgeDetection` _array_element))
        (else
          (goto _label))))))

(fn `4DirectionTrace`
  (params (FrontStart :type "Float (double-precision)") (SideStart :type "Float (double-precision)"))
  (returns (Front :type Boolean) (Back :type Boolean) (Right :type Boolean) (Left :type Boolean))
  (bind _returnvalue (`self.GetActorForwardVector`))
  (bind _returnvalue_2 (`self.GetActorRightVector`))
  (bind _returnvalue_3 (* SideStart _returnvalue_2))
  (bind _returnvalue_4 (+ (`self.K2_GetActorLocation`) (* _returnvalue FrontStart)))
  (bind _returnvalue_5 (+ (`self.K2_GetActorLocation`) _returnvalue_3))
  (bind (_outhit _returnvalue_6) (`KismetSystemLibrary.LineTraceSingle` _returnvalue_4 (+ _returnvalue_4 (* _returnvalue 99.0)) "TraceTypeQuery2"))
  (bind (_outhit_2 _returnvalue_7) (`KismetSystemLibrary.LineTraceSingle` (+ (`self.K2_GetActorLocation`) (* FrontStart (`self.GetActorForwardVector`) -1.0)) (+ _returnvalue_4 (* _returnvalue -99.0)) "TraceTypeQuery2"))
  (bind (_outhit_3 _returnvalue_8) (`KismetSystemLibrary.LineTraceSingle` _returnvalue_5 (+ _returnvalue_5 (* _returnvalue_2 99.0)) "TraceTypeQuery2"))
  (bind (_outhit_4 _returnvalue_9) (`KismetSystemLibrary.LineTraceSingle` (+ (`self.K2_GetActorLocation`) (* _returnvalue_3 -1.0)) (+ _returnvalue_5 (* _returnvalue_2 -99.0)) "TraceTypeQuery2"))
  (return _returnvalue_6 _returnvalue_7 _returnvalue_8 _returnvalue_9))

(fn `TraceOverlappedGround`
  (returns (Overlapped :type Boolean))
  (bind _returnvalue (`self.K2_GetActorLocation`))
  (bind (_outhit _returnvalue_2) (`KismetSystemLibrary.SphereTraceSingle` _returnvalue _returnvalue 20.0 "TraceTypeQuery1"))
  (if _returnvalue_2
    (return true)
    (else
      (return false))))

(fn `UserConstructionScript`
  (if (`self.Spawn`)
    _))