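; Player camera for BP_GridBased_Player that either follows an attach point or flies freely within MaxDistance of the player.
; While its spawned BP_HomingTarget is attached, the spring arm lerps to it and zooms closer when obstructed; movement input detaches it.
; Right-drag orbits the player's rotate point or turns the free camera, restoring the cursor position.
; The wheel zooms, with line traces blocking moves into geometry and Tick pulling out-of-range cameras back.
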(event `self.ReceiveTick`
  (params (DeltaSeconds :type "Float (single-precision)"))
  (bind _springarm (`self.SpringArm`))
  (bind _attacher (`self.Attacher`))
  (bind _returnvalue (`self.K2_GetActorLocation` (`self.Player`)))
  (bind _returnvalue_2 (`SceneComponent.K2_GetComponentLocation` (`self.TargetSele`)))
  (bind _returnvalue_3 (`SceneComponent.K2_GetComponentLocation` (`self.SpringArm`)))
  (bind _returnvalue_4 (`KismetMathLibrary.Vector_Distance` _returnvalue _returnvalue_2))
  (`KismetSystemLibrary.Delay` 0.01)
  (`|ExecutionSequence`
    (:`then_0`
      (if (<= _returnvalue_4 (`self.MaxDistance`))
        (if (`KismetSystemLibrary.IsValid` (`self.GetAttachParentActor` _attacher))
          (`SceneComponent.K2_SetWorldLocationAndRotation` _springarm (`KismetMathLibrary.VLerp` (`SceneComponent.K2_GetComponentLocation` _springarm) (`self.K2_GetActorLocation` _attacher) 0.2) (`KismetMathLibrary.RLerp` (`SceneComponent.K2_GetComponentRotation` _springarm) (`self.K2_GetActorRotation` _attacher) 0.4 true) false false))
        (else
          (`SceneComponent.K2_AddWorldOffset` (`self.SpringArm`) (* (`KismetMathLibrary.GetDirectionUnitVector` _returnvalue_2 _returnvalue) (/ _returnvalue_4 100.0)) false false)
          (`SceneComponent.K2_AddWorldOffset` (`self.TargetSele`) (* (`KismetMathLibrary.GetDirectionUnitVector` _returnvalue_2 _returnvalue) (/ _returnvalue_4 100.0)) false false))))
    (:`then_1`
      (if (`KismetSystemLibrary.IsValid` (`self.GetAttachParentActor` (`self.Attacher`)))
        (bind (_outhit _returnvalue_5) (`KismetSystemLibrary.SphereTraceSingle` _returnvalue_3 _returnvalue_3 50.0 "TraceTypeQuery2" true))
        (if _returnvalue_5
          (`self.GetClose`))))))

(event `GetClose`
  (bind _returnvalue (`KismetSystemLibrary.IsValid` (`self.GetAttachParentActor` (`self.Attacher`))))
  (bind _returnvalue_2 (* (`KismetMathLibrary.SelectVector` (`KismetMathLibrary.GetDirectionUnitVector` (`self.K2_GetActorLocation` (`self.Attacher`)) (- (`SceneComponent.K2_GetComponentLocation` (`/Game/BP/NewGame/BP_GridBased_Player.CameraRotatePoint` (`self.Player`))) (0.0 0.0 100.0))) (`SceneComponent.GetForwardVector` (`self.Camera`)) _returnvalue) (`self.MovementStrength`) 2.0))
  (if _returnvalue :!label _label
    (if (> (`KismetMathLibrary.Vector_Distance` (`SceneComponent.K2_GetComponentLocation` (`/Game/BP/NewGame/BP_GridBased_Player.CameraRotatePoint` (`self.Player`))) (`SceneComponent.K2_GetComponentLocation` (`self.SpringArm`))) 150.0)
      (bind _returnvalue_3 (`self.Trace` (.x _returnvalue_2) (.y _returnvalue_2) (.z _returnvalue_2) :!label _label_2))
      (if (not _returnvalue_3)
        (`SceneComponent.K2_AddWorldOffset` (`self.TargetSele`) _returnvalue_2 false false)))
    (else
      (goto _label_2))))

(event `InputAxisKey|MouseY` :consume false
  (params (AxisValue :type "Float (single-precision)"))
  (bind _returnvalue (* AxisValue 2.0))
  (bind _springarm (`self.SpringArm`))
  (bind _springarm_2 (`self.SpringArm`))
  (bind _springarm_3 (`self.SpringArm`))
  (bind (_mouseloc_x _mouseloc_y) (`KismetMathLibrary.BreakVector2D` (`self.MouseLoc`)))
  (bind (_returnvalue_roll _returnvalue_pitch _returnvalue_yaw) (`KismetMathLibrary.BreakRotator` (`SceneComponent.K2_GetComponentRotation` _springarm_3)))
  (bind (_returnvalue_roll_2 _returnvalue_pitch_2 _returnvalue_yaw_2) (`KismetMathLibrary.BreakRotator` (`SceneComponent.K2_GetComponentRotation` _springarm)))
  (bind _camerarotatepoint (`/Game/BP/NewGame/BP_GridBased_Player.CameraRotatePoint` (`self.Player`)))
  (bind (_returnvalue_roll_3 _returnvalue_pitch_3 _returnvalue_yaw_3) (`KismetMathLibrary.BreakRotator` (`SceneComponent.K2_GetComponentRotation` _camerarotatepoint)))
  (bind _targetpoint (`/Game/UI_Cursor.TargetPoint` (`/Game/BP/NewGame/GridPlayerController.Mouse` (`/Game/BP/NewGame/BP_GridBased_Player.Player Controller` (`self.Player`)))))
  (if (`self.Pressed`)
    (if (`KismetSystemLibrary.IsValid` (`self.GetAttachParentActor` (`self.Attacher`)))
      (`SceneComponent.K2_SetWorldRotation` _camerarotatepoint (`KismetMathLibrary.MakeRotator` _returnvalue_roll_3 (`KismetMathLibrary.FClamp` (+ _returnvalue_pitch_3 (* _returnvalue -1.0)) 5.0 80.0) _returnvalue_yaw_3) false false)
      (`SceneComponent.K2_SetWorldRotation` _springarm (`KismetMathLibrary.MakeRotator` 0.0 _returnvalue_pitch_2 _returnvalue_yaw_2) false false)
      (else
        (`SceneComponent.K2_SetWorldRotation` _springarm_3 (`KismetMathLibrary.MakeRotator` _returnvalue_roll (`KismetMathLibrary.FClamp` (+ _returnvalue_pitch _returnvalue) -89.0 60.0) _returnvalue_yaw) false false)))
    (`|ExecutionSequence` :!label _label_3
      (:`then_0`
        (if (`KismetSystemLibrary.IsValid` (`self.GetAttachParentActor`))
          (set `SpringArmComponent.bEnableCameraLag` false _springarm_2)
          (`KismetSystemLibrary.RetriggerableDelay` 0.1)
          (set `SpringArmComponent.bEnableCameraLag` true _springarm_2)))
      (:`then_1`
        (`Widget.SetVisibility` _targetpoint "Hidden")
        (`KismetSystemLibrary.RetriggerableDelay` 0.1)
        (`Widget.SetVisibility` _targetpoint "Visible"))
      (:`then_2`
        (if (or (> (`KismetMathLibrary.Abs` (`self.GetInputAxisKeyValue`)) 0.1) (> (`KismetMathLibrary.Abs` (`self.GetInputAxisKeyValue`)) 0.1))
          (`PlayerController.SetMouseLocation` (`GameplayStatics.GetPlayerController` 0) (`KismetMathLibrary.FTrunc` _mouseloc_x) (`KismetMathLibrary.FTrunc` _mouseloc_y)))))
    (else
      (bind _returnvalue_2 (`WidgetLayoutLibrary.GetMousePositionOnViewport` :!label _label_4))
      (set `self.MouseLoc` _returnvalue_2))))

(event `Key|MouseScrollUp`
  (params (Key :type "Key Structure"))
  (:`Pressed`
    (goto _label)))

(event `Key|MouseScrollDown`
  (params (Key :type "Key Structure"))
  (bind _returnvalue (`KismetSystemLibrary.IsValid` (`self.GetAttachParentActor` (`self.Attacher`))))
  (bind _returnvalue_2 (* (`KismetMathLibrary.SelectVector` (`KismetMathLibrary.GetDirectionUnitVector` (`self.K2_GetActorLocation` (`self.Attacher`)) (- (`SceneComponent.K2_GetComponentLocation` (`/Game/BP/NewGame/BP_GridBased_Player.CameraRotatePoint` (`self.Player`))) (0.0 0.0 100.0))) (`SceneComponent.GetForwardVector` (`self.Camera`)) _returnvalue) (`self.MovementStrength`) -2.0))
  (:`Pressed`
    (if _returnvalue
      (if (< (`KismetMathLibrary.Vector_Distance` (`SceneComponent.K2_GetComponentLocation` (`/Game/BP/NewGame/BP_GridBased_Player.CameraRotatePoint` (`self.Player`))) (`SceneComponent.K2_GetComponentLocation` (`self.SpringArm`))) (`self.MaxDistance`))
        (bind _returnvalue_3 (`self.Trace` (.x _returnvalue_2) (.y _returnvalue_2) (.z _returnvalue_2) :!label _label_5))
        (if (not _returnvalue_3)
          (`SceneComponent.K2_AddWorldOffset` (`self.TargetSele`) _returnvalue_2 false false)))
      (else
        (goto _label_5)))))

(event `InputAxisKey|MouseX` :consume false
  (params (AxisValue :type "Float (single-precision)"))
  (if (`self.Pressed`)
    (`SceneComponent.K2_AddWorldRotation` (select `bool` (`KismetSystemLibrary.IsValid` (`self.GetAttachParentActor` (`self.Attacher`))) :`false` (`self.SpringArm`) :`true` (`/Game/BP/NewGame/BP_GridBased_Player.CameraRotatePoint` (`self.Player`)) :!type "SceneComponent Object Reference") (`KismetMathLibrary.MakeRotator` 0.0 0.0 (* AxisValue 2.0)) false false)
    (goto _label_3)
    (else
      (goto _label_4))))

(event `Key|RightMouseButton` :consume false
  (params (Key :type "Key Structure"))
  (:`Pressed`
    (set `self.Pressed` true))
  (:`Released`
    (set `self.Pressed` false)))

(event `InputAxis|MovementForward`
  (params (AxisValue :type "Float (single-precision)"))
  (bind _attacher (`self.Attacher`))
  (bind (_returnvalue_x _returnvalue_y) (`KismetMathLibrary.BreakVector` (* (`KismetMathLibrary.Vector_Normal2D` (`SceneComponent.GetForwardVector` (`self.Camera`))) (* AxisValue (`self.MovementStrength`)))))
  (`KismetSystemLibrary.Delay` 0.01)
  (if (`self.DistanceCheck` (`KismetMathLibrary.MakeVector` _returnvalue_x _returnvalue_y))
    (bind _returnvalue (`self.Trace` _returnvalue_x _returnvalue_y))
    (if (not _returnvalue)
      (`SceneComponent.K2_AddWorldOffset` (`self.SpringArm`) (`KismetMathLibrary.MakeVector` _returnvalue_x _returnvalue_y) true false)
      (if (or (> (`KismetMathLibrary.Abs` (`self.GetInputAxisValue`)) 0.1) (> (`KismetMathLibrary.Abs` (`self.GetInputAxisValue`)) 0.1) (> (`KismetMathLibrary.Abs` (`self.GetInputAxisValue`)) 0.1)) :!label _label_6
        (`/Engine/EditorBlueprintResources/StandardMacros.IsValid` (`self.GetAttachParentActor` _attacher)
          (:`Is Valid`
            (`self.K2_DetachFromActor` _attacher "KeepWorld" "KeepWorld" "KeepWorld")))))))

(event `InputAxis|MovementSide`
  (params (AxisValue :type "Float (single-precision)"))
  (bind (_returnvalue_x _returnvalue_y) (`KismetMathLibrary.BreakVector` (* (`SceneComponent.GetRightVector` (`self.Camera`)) (* AxisValue (`self.MovementStrength`)))))
  (`KismetSystemLibrary.Delay` 0.01)
  (if (`self.DistanceCheck` (`KismetMathLibrary.MakeVector` _returnvalue_x _returnvalue_y))
    (bind _returnvalue (`self.Trace` _returnvalue_x _returnvalue_y))
    (if (not _returnvalue)
      (`SceneComponent.K2_AddWorldOffset` (`self.SpringArm`) (`KismetMathLibrary.MakeVector` _returnvalue_x _returnvalue_y) true false)
      (goto _label_6))))

(event `InputAxis|MovementUp`
  (params (AxisValue :type "Float (single-precision)"))
  (bind _returnvalue (* AxisValue (* (`self.MovementStrength`) 0.8)))
  (`KismetSystemLibrary.Delay` 0.01)
  (if (`self.DistanceCheck` (`KismetMathLibrary.MakeVector` 0.0 0.0 _returnvalue))
    (bind _returnvalue_2 (`self.Trace` 0.0 0.0 _returnvalue))
    (if (not _returnvalue_2)
      (`SceneComponent.K2_AddWorldOffset` (`self.SpringArm`) (`KismetMathLibrary.MakeVector` 0.0 0.0 _returnvalue) true false)
      (goto _label_6))))

(event `self.ReceiveBeginPlay`
  (`PlayerController.SetViewTargetWithBlend` (`GameplayStatics.GetPlayerController` 0) self 0.0 "VTBlend_Linear" 0.0 false)
  (bind _returnvalue (`|SpawnActorFromClass` "/Game/BP/Nova/BP_HomingTarget.BP_HomingTarget_C" (`self.GetTransform`) "Undefined" "MultiplyWithRoot" null null))
  (set `self.Attacher` _returnvalue)
  (bind _returnvalue_2 (`GameplayStatics.GetActorOfClass` "/Game/BP/NewGame/BP_GridBased_Player.BP_GridBased_Player_C"))
  (set `self.Player` _returnvalue_2)
  (`KismetSystemLibrary.Delay` 0.2)
  (`self.EnableInput` (`GameplayStatics.GetPlayerController` 0)))

(fn `DistanceCheck`
  (params (AddDistance :type "Vector Structure"))
  (returns (ReturnValue :type Boolean))
  (bind _returnvalue (+ (`SceneComponent.K2_GetComponentLocation` (`self.SpringArm`)) AddDistance))
  (bind (_outhit _returnvalue_2) (`KismetSystemLibrary.SphereTraceSingle` _returnvalue _returnvalue 100.0 "TraceTypeQuery1"))
  (return (<= (`KismetMathLibrary.Vector_Distance` (`self.K2_GetActorLocation` (`self.Player`)) _returnvalue) (`self.MaxDistance`))))

(fn `TargetSele`
  (returns (ReturnValue :type "SceneComponent Object Reference"))
  (return (select `bool` (`KismetSystemLibrary.IsValid` (`self.GetAttachParentActor` (`self.Attacher`))) :`false` (`self.SpringArm`) :`true` (`/Game/BP/Nova/BP_HomingTarget.DefaultSceneRoot` (`self.Attacher`)) :!type "SceneComponent Object Reference")))

(fn `Trace`
  (params (X :type "Float (double-precision)") (Y :type "Float (double-precision)") (Z :type "Float (double-precision)"))
  (returns (ReturnValue :type Boolean))
  (bind _returnvalue (`SceneComponent.K2_GetComponentLocation` (`self.SpringArm`)))
  (bind (_outhit _returnvalue_2) (`KismetSystemLibrary.LineTraceSingle` _returnvalue (+ _returnvalue (* (`KismetMathLibrary.MakeVector` X Y Z) 5.0)) "TraceTypeQuery2" true))
  (return _returnvalue_2))

(fn `UserConstructionScript`)