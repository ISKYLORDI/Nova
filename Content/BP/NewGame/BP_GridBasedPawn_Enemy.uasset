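; Grid-based enemy pawn that moves on EnemyMove as Random Straight, Chase Straight or Chase Cross, with color set by type.
; Line traces gather reachable cells along straight axes, plus diagonals for Cross, allowing one-level height steps.
; It picks a random cell or the one nearest the player, retrying when another enemy claims it, then calls TakeNextStep.
; An A* pathfinding function exists but is never called.
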(event `self.ReceiveBeginPlay`
  (bind _returnvalue (`GameplayStatics.GetActorOfClass` "/Game/BP/NewGame/BP_AStarPathfinding.BP_AStarPathfinding_C"))
  (set `self.A Star` _returnvalue))

(event `EnemyMove`
  (params (Delay :type "Float (single-precision)"))
  (`KismetSystemLibrary.Delay` Delay)
  (set `self.EndLoc` (0.0 0.0 0.0))
  (`KismetArrayLibrary.Array_Clear` (`self.TargetLocations`))
  (for _index (range 1 (+ (`self.MovePoints`) 1))
    (switch `/Game/BP/NewGame/EN_GridEnemyType` (`self.EnemyType`)
      (:`NewEnumerator0`
        _)
      (:`NewEnumerator1`
        _)
      (:`NewEnumerator2`
        (bind _returnvalue (* (`self.MoveDistance`) _index))
        (`self.DetectTargets` (+ (`self.GetActorForwardVector`) (`self.GetActorRightVector`)) _returnvalue)
        (`self.DetectTargets` (+ (* (`self.GetActorForwardVector`) -1.0) (`self.GetActorRightVector`)) _returnvalue)
        (`self.DetectTargets` (+ (`self.GetActorForwardVector`) (* (`self.GetActorRightVector`) -1.0)) _returnvalue)
        (`self.DetectTargets` (+ (* (`self.GetActorForwardVector`) -1.0) (* (`self.GetActorRightVector`) -1.0)) _returnvalue)))
    (`self.DetectTargets` (`self.GetActorForwardVector`) (* (`self.MoveDistance`) _index))
    (`self.DetectTargets` (`self.GetActorRightVector`) (* (`self.MoveDistance`) _index))
    (`self.DetectTargets` (`self.GetActorForwardVector`) (* (* (`self.MoveDistance`) -1.0) _index))
    (`self.DetectTargets` (`self.GetActorRightVector`) (* (* (`self.MoveDistance`) -1.0) _index))
    (switch `/Game/BP/NewGame/EN_GridEnemyType` (`self.EnemyType`)
      (:`NewEnumerator0`
        (set `self.Occupied` false :!label _label)
        (set `self.EndLoc` (`KismetArrayLibrary.Array_Random` (`self.TargetLocations`)))
        (bind _outactors (`GameplayStatics.GetAllActorsOfClass` "BP_GridBasedPawn_Enemy_C"))
        (for _array_element _outactors
          (if (== (`/Game/BP/NewGame/BP_GridBasedPawn.EndLoc` _array_element) (`self.EndLoc`) :`ErrorTolerance` 1.0)
            (set `self.Occupied` true)))
        (if (`self.Occupied`)
          (goto _label)
          (else
            (`self.TakeNextStep`))))
      (:`NewEnumerator1`
        (`|ExecutionSequence` :!label _label_2
          (:`then_0`
            (goto _label_4 :!via `Reset`))
          (:`then_1`
            (set `self.Occupied` false :!label _label_3)
            (`/Engine/EditorBlueprintResources/StandardMacros.Do N` 5 :!label _label_4
              (:`Exit`
                (bind _targetlocation (`self.ClosestTarget`))
                (set `self.EndLoc` _targetlocation)
                (bind _outactors_2 (`GameplayStatics.GetAllActorsOfClass` "BP_GridBasedPawn_Enemy_C"))
                (for _array_element_2 _outactors_2
                  (if (and (== (`/Game/BP/NewGame/BP_GridBasedPawn.EndLoc` _array_element_2) (`self.EndLoc`) :`ErrorTolerance` 1.0) (!= _array_element_2 self))
                    (set `self.Occupied` true)))
                (if (`self.Occupied`)
                  (`KismetArrayLibrary.Array_RemoveItem` (`self.TargetLocations`) (`self.EndLoc`))
                  (goto _label_3)
                  (elif (!= (`self.EndLoc`) (0.0 0.0 0.0))
                    (`self.TakeNextStep`))))))))
      (:`NewEnumerator2`
        (goto _label_2)))))

(fn `AStarPathfindingFunction`
  (bind _a_star (`self.A Star`))
  (bind _returnvalue (`GameplayStatics.GetActorOfClass` "/Game/BP/NewGame/BP_GridBased_Player.BP_GridBased_Player_C"))
  (`AStarPathfinding.setStartEndCoord` _a_star 1300 2000 100 0 (`self.K2_GetActorLocation`) (`self.K2_GetActorLocation` _returnvalue))
  (`AStarPathfinding.solve` _a_star)
  (bind _returnvalue_2 (`AStarPathfinding.getNextStepDirection` _a_star))
  (`self.K2_SetActorLocation` (+ _returnvalue_2 (`self.K2_GetActorLocation`))))

(fn `ClosestTarget`
  (returns (TargetLocation :type "Vector Structure"))
  (locals (Closest :type "Float (double-precision)" :default 50000.0) (ClosestLocation :type "Vector Structure"))
  (set `local.Closest` 50000.0)
  (bind _outactors (`GameplayStatics.GetAllActorsOfClass` "/Game/BP/NewGame/BP_GridBased_Player.BP_GridBased_Player_C"))
  (for _array_element (`self.TargetLocations`)
    (bind _returnvalue (`KismetMathLibrary.Vector_Distance` _array_element (`self.K2_GetActorLocation` (`|GetArrayItem` _outactors))))
    (if (< _returnvalue (`local.Closest`))
      (set `local.Closest` _returnvalue)
      (set `local.ClosestLocation` _array_element)))
  (return (`local.ClosestLocation`)))

(fn `DetectTargets`
  (params (Direction :type "Vector Structure") (Distance :type "Float (double-precision)"))
  (bind _returnvalue (`self.K2_GetActorLocation`))
  (bind _targetlocations (`self.TargetLocations`))
  (bind _targetlocations_2 (`self.TargetLocations`))
  (bind _returnvalue_2 (+ _returnvalue (* Direction Distance)))
  (bind _returnvalue_3 (+ _returnvalue_2 (0.0 0.0 50.0)))
  (bind (_outhit _returnvalue_4) (`KismetSystemLibrary.LineTraceSingle` _returnvalue _returnvalue_2 "TraceTypeQuery1"))
  (if _returnvalue_4
    (bind (_bblockinghit _binitialoverlap _time _distance _location _impactpoint _normal _impactnormal _physmat _hitactor) (`GameplayStatics.BreakHitResult` _outhit))
    (bind _asbp_grid_based_player (cast `/Game/BP/NewGame/BP_GridBased_Player` _hitactor)
      (:`then`
        (`KismetArrayLibrary.Array_Add` _targetlocations (`self.K2_GetActorLocation` _asbp_grid_based_player)))
      (:`CastFailed`
        (cast `/Game/BP/NewGame/BP_GridBasedPawn_Enemy` _hitactor
          (:`CastFailed`
            (bind (_outhit_2 _returnvalue_5) (`KismetSystemLibrary.LineTraceSingle` _returnvalue_3 (+ _returnvalue_2 (0.0 0.0 0.1)) "TraceTypeQuery1"))
            (if (not _returnvalue_5)
              (`KismetArrayLibrary.Array_Add` _targetlocations _returnvalue_3))))))
    (else
      (bind (_outhit_3 _returnvalue_6) (`KismetSystemLibrary.LineTraceSingle` _returnvalue_2 (+ _returnvalue_2 (0.0 0.0 -51.0)) "TraceTypeQuery1"))
      (if _returnvalue_6
        (`KismetArrayLibrary.Array_Add` _targetlocations_2 _returnvalue_2)
        (else
          (bind (_outhit_4 _returnvalue_7) (`KismetSystemLibrary.LineTraceSingle` _returnvalue_2 (+ _returnvalue_2 (0.0 0.0 -101.0)) "TraceTypeQuery1"))
          (if _returnvalue_7
            (`KismetArrayLibrary.Array_Add` _targetlocations_2 (+ _returnvalue_2 (0.0 0.0 -50.0)))))))))

(fn `UserConstructionScript`
  (`parent.UserConstructionScript`)
  (`MeshComponent.SetVectorParameterValueOnMaterials` (`self.StaticMesh`) "Color" (`KismetMathLibrary.Conv_LinearColorToVector` (select `/Game/BP/NewGame/EN_GridEnemyType` (`self.EnemyType`) :`NewEnumerator0` (struct :`R` 1.0 :`G` 0.380392 :`A` 1.0) :`NewEnumerator1` (struct :`R` 1.0 :`G` 0.380392 :`A` 1.0) :`NewEnumerator2` (struct :`R` 0.521699 :`B` 1.0 :`A` 1.0) :!type "LinearColor Structure")))
  (bind _returnvalue (`GameplayStatics.GetActorOfClass` "/Game/BP/NewGame/BP_AStarPathfinding.BP_AStarPathfinding_C"))
  (set `self.A Star` _returnvalue))